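; Game mode for CoLab gameplay that tracks connected CoLab player controllers and picks their spawn points.
; Login, controller swap and logout events update the Players list, with list-updated notifications deferred to callbacks for a controller's first possession and EndPlay.
; ChoosePlayerStart returns either a random CoLab player start or, when UseEmptiestPlayerStart is set, the one whose nearest CoLab character is farthest away.
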(event EventBeginPlay)

(event EventTick
  (params (DeltaSeconds :type Float%20%28single-precision%29)))

(event EventPostLogin
  (params (NewPlayer :type Player%20Controller%20Object%20Reference))
  ;[1 1 1] Player initial connect to session
  (CallFunction|SetPlayerRegistered NewPlayer true))

(event EventOnSwapPlayerControllers
  (params (OldPC :type Player%20Controller%20Object%20Reference) (NewPC :type Player%20Controller%20Object%20Reference))
  ;[1 1 1] Player change PC during session (swap levels)
  (CallFunction|SetPlayerRegistered OldPC false)
  (CallFunction|SetPlayerRegistered NewPC true))

(event EventOnLogout
  (params (ExitingController :type Controller%20Object%20Reference))
  ;[1 1 1] Player leaves session
  (bind _asplayer_controller (Utilities|Casting|CastToPlayerController ExitingController))
  (CallFunction|SetPlayerRegistered _asplayer_controller false))

(fn ConstructionScript)

(fn SetPlayerRegistered
  (params (Player :type Player%20Controller%20Object%20Reference) (bRegistered :type Boolean))
  (bind _players (Variables|Default|GetPlayers))
  (bind _asbp_pc_co_lab_gameplay (Utilities|Casting|CastToBP_PC_CoLabGameplay Player))
  (LocalVariables|SetL_Player _asbp_pc_co_lab_gameplay)
  (if bRegistered
    (Utilities|Set|Add _players (LocalVariables|GetL_Player))
    (Pawn|BindEventtoOnPossessedPawnChanged (LocalVariables|GetL_Player) (EventDispatchers|CreateEvent :!event OnControllerInitialSpawn))
    (else
      (Utilities|Set|Remove _players (LocalVariables|GetL_Player))
      (Game|BindEventtoOnEndPlay (LocalVariables|GetL_Player) (EventDispatchers|CreateEvent :!event OnControllerEndPlay)))))

(fn FindRandomPlayerStart
  (bind _outactors (Actor|GetAllActorsOfClass "/Game/CoLab/Modes/Gameplay/Actors/BP_CoLabPlayerStart.BP_CoLabPlayerStart_C"))
  (return (Utilities|Array|Get(acopy) _outactors (Math|Random|RandomIntegerinRange 0 (- (Utilities|Array|Length _outactors) 1)))))

(fn ChoosePlayerStart
  (params (Player :type Controller%20Object%20Reference))
  (if (Variables|Default|GetbUseEmptiestPlayerStart)
    (bind _playerstart (Spawning|FindEmptiestPlayerStart))
    (return _playerstart)
    (else
      (bind _playerstart_2 (Spawning|FindRandomPlayerStart))
      (return _playerstart_2))))

(fn FindEmptiestPlayerStart
  (bind _outactors (Actor|GetAllActorsOfClass "/Game/CoLab/Modes/Gameplay/Actors/BP_CoLabPlayerStart.BP_CoLabPlayerStart_C"))
  (LocalVariables|SetL_PlayerStarts _outactors)
  (bind _outactors_2 (Actor|GetAllActorsOfClass "/Game/CoLab/Modes/Gameplay/Characters/Player/BP_CoLabCharacter.BP_CoLabCharacter_C"))
  (LocalVariables|SetL_Players _outactors_2)
  (for _array_element (LocalVariables|GetL_PlayerStarts)
    (LocalVariables|SetL_PlayerStart _array_element)
    (LocalVariables|SetL_MinDistance 0.0)
    (for _array_element_2 (LocalVariables|GetL_Players)
      (Utilities|FlowControl|Sequence
        (:then_0
          (if (< (Transformation|GetSquaredDistanceTo _array_element_2 (LocalVariables|GetL_PlayerStart)) (LocalVariables|GetL_MinDistance))
            (LocalVariables|SetL_MinDistance (Transformation|GetSquaredDistanceTo _array_element_2 (LocalVariables|GetL_PlayerStart)) :!label _label)))
        (:then_1
          (Utilities|FlowControl|DoOnce false
            (:Completed
              (goto _label))))))
    (Utilities|FlowControl|Sequence
      (:then_0
        (Utilities|FlowControl|DoOnce false) ; enters at Reset
      )
      (:then_1
        (Utilities|Map|Add (LocalVariables|GetL_MinPlayerStartDists) (LocalVariables|GetL_PlayerStart) (LocalVariables|GetL_MinDistance)))))
  (LocalVariables|SetL_MaxDistance -1.0)
  (bind _keys (Utilities|Map|Keys (LocalVariables|GetL_MinPlayerStartDists)))
  (for _array_element_3 _keys
    (if (> (.Value (Utilities|Map|Find (LocalVariables|GetL_MinPlayerStartDists) _array_element_3)) (LocalVariables|GetL_MaxDistance))
      (LocalVariables|SetL_MaxDistance (.Value (Utilities|Map|Find (LocalVariables|GetL_MinPlayerStartDists) _array_element_3)))
      (LocalVariables|SetL_FurthestSpawn _array_element_3)))
  (return (LocalVariables|GetL_FurthestSpawn)))

(fn OnControllerEndPlay
  (params (Actor :type Actor%20Object%20Reference) (EndPlayReason :type EEndPlayReason%20Enum :default "Destroyed"))
  (Default|CallOnPlayerListUpdated))

(fn OnControllerInitialSpawn
  (params (OldPawn :type Pawn%20Object%20Reference) (NewPawn :type Pawn%20Object%20Reference))
  (Default|CallOnPlayerListUpdated)
  (bind _asplayer_controller (Utilities|Casting|CastToPlayerController (Pawn|GetController NewPawn)))
  (Pawn|UnbindEventfromOnPossessedPawnChanged _asplayer_controller (EventDispatchers|CreateEvent :!event OnControllerInitialSpawn)))