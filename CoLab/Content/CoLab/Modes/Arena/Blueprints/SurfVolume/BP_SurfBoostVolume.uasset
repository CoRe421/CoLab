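; Arena surf boost volume that grants players inside it a gameplay effect.
; Overrides of the parent's player enter and leave events apply the effect to the PlayerState's ability system component and remove all its stacks on exit.
; The construction script fits the Niagara effect to the box, scaling spawn rate with its volume; BeginPlay resets the fixed bounds.
; A helper graph tracks overlapping players, changing the list only when their state changes.
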(event EventBeginPlay
  (|CallParentFunction)
  (Class|NiagaraComponent|SetSystemFixedBounds (Variables|Default|GetNiagara) (Class|KismetMathLibrary|MakeBoxwithOrigin (Math|Vector|VectorZero) (Components|Box|GetScaledBoxExtent (Variables|Default|GetBox)))))

(event Collision|EventActorBeginOverlap
  (params (OtherActor :type Actor%20Object%20Reference)))

(event EventTick
  (params (DeltaSeconds :type Float%20%28single-precision%29)))

(fn ConstructionScript
  (bind _niagara (Variables|Default|GetNiagara))
  (bind _box (Variables|Default|GetBox))
  (bind _returnvalue (Components|Box|GetScaledBoxExtent _box))
  (|CallParentFunction)
  (Effects|Components|ParticleSystem|SetVectorParameter _niagara "BoxSize" _returnvalue)
  (Effects|Components|ParticleSystem|SetFloatParameter _niagara "SpawnRate" (+ 3.0 (/ (Class|KismetMathLibrary|GetBoxVolume (Class|KismetMathLibrary|MakeBoxwithOrigin (.Origin (Collision|GetComponentBounds 0)) _returnvalue)) 1e+08)))
  (Class|NiagaraComponent|SetSystemFixedBounds _niagara (Class|KismetMathLibrary|MakeBoxwithOrigin (Math|Vector|VectorZero) _returnvalue)))

(fn OnNewPlayerEnter
  (params (Player :type Collab%20Player%20Character%20Object%20Reference))
  (|CallParentFunction Player)
  (bind _output_get (Variables|Default|SetTargetComponent (Class|CollabAbilitySystemComponent|FindAbilitySystemComponent (Variables|/Script/Engine.Pawn|GetPlayerState Player))))
  (Utilities|IsValid _output_get
    (:Is%20Valid
      (GameplayEffects|ApplyGameplayEffectToSelf :self _output_get :GameplayEffectClass (Variables|Default|GetSurgBoostEffect)))))

(fn OnPlayerLeave
  (params (Player :type Collab%20Player%20Character%20Object%20Reference))
  (|CallParentFunction Player)
  (bind _output_get (Variables|Default|SetTargetComponent (Class|CollabAbilitySystemComponent|FindAbilitySystemComponent (Variables|/Script/Engine.Pawn|GetPlayerState Player))))
  (Utilities|IsValid _output_get
    (:Is%20Valid
      (GameplayEffects|RemoveActiveGameplayEffectbySourceEffect _output_get (Variables|Default|GetSurgBoostEffect) 0 -1))))