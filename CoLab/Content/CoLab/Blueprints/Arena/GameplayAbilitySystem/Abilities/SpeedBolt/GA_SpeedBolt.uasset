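; Arena gameplay ability for Speed Bolt, a hold-to-charge shot that trades the caster's time dilation for damage.
; On activation it commits cost and cooldown, tags casting and starts a looping timer that, in scale-to-speed mode, lowers CustomTimeDilation and updates the charge widget.
; Release fires an instant line trace, applying SetByCaller damage from initial speed and dilation lost.
; Ending restores dilation; the static-reduction mode only caches values, without slowing.
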(event Custom|TryFireBolt
  (params (InitialSpeed :type Float%20%28double-precision%29) (SpeedDifferenceRatio :type Float%20%28double-precision%29))
  (bind _data (|WaitTargetData :TaskInstanceName "SpeedBoltTrace" :ConfirmationType "Instant" :Class "/Script/GameplayAbilities.GameplayAbilityTargetActor_SingleLineTrace" :TraceProfile "(Name=\"BlockAll\")" :StartLocation (Class|GameplayAbility|MakeTargetLocationInfofromOwnerActor) :ReticleClass "/Script/GameplayAbilities.GameplayAbilityWorldReticle")
    (:ValidData
      (Utilities|FlowControl|Sequence
        (:then_0
          (bind _output_get (Variables|Default|SetHitActor (Utilities|Array|Get(acopy) (Ability|TargetData|GetActorsfromTargetData _data))))
          (bind _returnvalue (Ability|GameplayEffect|AssignTagSetbyCallerMagnitude (Ability|MakeOutgoingGameplayEffectSpec "/Game/CoLab/Blueprints/Arena/GameplayAbilitySystem/Abilities/SpeedBolt/GE_SpeedBoltDamage.GE_SpeedBoltDamage_C") "(TagName=\"Gameplay.Effect.Damage\")" (* (* InitialSpeed 0.05) (Math|Float|Lerp 1.0 0.0 SpeedDifferenceRatio))))
          (GameplayEffects|ApplyGameplayEffectSpecToTarget _returnvalue (Ability|TargetData|AbilityTargetDatafromActor _output_get)))
        (:then_1
          (Ability|EndAbility :!label _label))))
    (:Cancelled
      (goto _label))))

(event Custom|CustomEvent
  (Development|PrintString "Hello"))

(event Ability|EventActivateAbility
  (bind _returnvalue (Class|CollabRuntimeConfigSubsystem|GetConfigData (Subsystems|GetCollabRuntimeConfigSubsystem) (Variables|Default|GetConfigClass)))
  (bind _aspda_speed_bolt_config (Utilities|Casting|CastToPDA_SpeedBoltConfig _returnvalue)
    (:then
      (Variables|Default|SetCachedConfigData _aspda_speed_bolt_config)
      (bind _asbp_arena_character (Utilities|Casting|CastToBP_ArenaCharacter (Ability|GetAvatarActorfromActorInfo))
        (:then
          (bind _output_get (Variables|Default|SetCachedCharacter _asbp_arena_character))
          (bind _output_get_2 (Variables|Default|SetCachedMovementComponent (Actor|GetComponentbyClass _output_get "/Script/Collab.CollabMovementComponent")))
          (Utilities|IsValid _output_get_2
            (:Is%20Valid
              (bind _returnvalue_2 (Ability|CommitAbilityCost true))
              (if _returnvalue_2
                (bind _returnvalue_3 (Ability|CommitAbilityCooldown true true))
                (if _returnvalue_3
                  (Variables|Default|SetCachedInitialVelocity (Variables|/Script/Engine.MovementComponent|GetVelocity (Variables|Default|GetCachedMovementComponent)))
                  (Ability|GameplayEffect|AddLooseGameplayTags (Variables|Default|GetCachedCharacter) (GameplayTags|MakeGameplayTagContainerfromTag "(TagName=\"Gameplay.State.Casting\")"))
                  (Variables|Default|SetCachedPrevTimeDilation (Variables|/Script/Engine.Actor|GetCustomTimeDilation (Variables|Default|GetCachedCharacter)))
                  (Utilities|FlowControl|Sequence
                    (:then_0
                      ;[1 1 1] On Release
                      (Ability|Tasks|WaitInputRelease false
                        (:OnRelease
                          (Ability|GameplayEffect|RemoveLooseGameplayTags (Variables|Default|GetCachedCharacter) (GameplayTags|MakeLiteralGameplayTagContainer "(GameplayTags=((TagName=\"Gameplay.State.Casting\")))"))
                          (Ability|CommitAbilityCooldown true true)
                          (Utilities|Time|ClearandInvalidateTimerbyHandle (Variables|Default|GetBoltGrowthTickHandle))
                          (Class|BPIPCCollab|RemoveWidgetfromStack(Message) (Pawn|GetLocalViewingPlayerController (Variables|Default|GetCachedCharacter)) "(TagName=\"UI.Layer.Game\")" (Variables|Default|GetCachedUI) true)
                          (CallFunction|TryFireBolt (Math|Vector|VectorLength (Variables|Default|GetCachedInitialVelocity)) (/ (Variables|/Script/Engine.Actor|GetCustomTimeDilation (Variables|Default|GetCachedCharacter)) (Variables|Default|GetCachedPrevTimeDilation))))))
                    (:then_1
                      (if (Variables|/Game/CoLab/Blueprints/Arena/GameplayAbilitySystem/Abilities/SpeedBolt/Config/PDA_SpeedBoltConfig.PDA_SpeedBoltConfig_C|GetbScaleCastToSpeed (Variables|Default|GetCachedConfigData))
                        (Variables|Default|SetCachedScaledTickPercent (Variables|/Game/CoLab/Blueprints/Arena/GameplayAbilitySystem/Abilities/SpeedBolt/Config/PDA_SpeedBoltConfig.PDA_SpeedBoltConfig_C|GetScaledCastTickPercent (Variables|Default|GetCachedConfigData)))
                        (else
                          (Variables|Default|SetCachedMaxVelocityRatio (Math|Vector|MakeVector (/ (.X (Math|Vector|BreakVector (Variables|Default|GetCachedInitialVelocity))) (Math|Vector|GetMaxElement (Variables|Default|GetCachedInitialVelocity))) (/ (.Y (Math|Vector|BreakVector (Variables|Default|GetCachedInitialVelocity))) (Math|Vector|GetMaxElement (Variables|Default|GetCachedInitialVelocity))) (/ (.Z (Math|Vector|BreakVector (Variables|Default|GetCachedInitialVelocity))) (Math|Vector|GetMaxElement (Variables|Default|GetCachedInitialVelocity)))))
                          (Variables|Default|SetCachedStaticTickSpeedReduction (Variables|/Game/CoLab/Blueprints/Arena/GameplayAbilitySystem/Abilities/SpeedBolt/Config/PDA_SpeedBoltConfig.PDA_SpeedBoltConfig_C|GetStaticSpeedTickReduction (Variables|Default|GetCachedConfigData)))))
                      (Variables|Default|SetCurrentBoltGrowthTime 0.0)
                      (Variables|Default|SetCachedBoltGrowthRate (Variables|/Game/CoLab/Blueprints/Arena/GameplayAbilitySystem/Abilities/SpeedBolt/Config/PDA_SpeedBoltConfig.PDA_SpeedBoltConfig_C|GetSpeedBoltGrowthRate (Variables|Default|GetCachedConfigData)))
                      (bind _widget (Class|BPIPCCollab|PushWidgettoStack(Message) (Pawn|GetLocalViewingPlayerController (Variables|Default|GetCachedCharacter)) "(TagName=\"UI.Layer.Game\")" "/Game/CoLab/Blueprints/Arena/GameplayAbilitySystem/Abilities/SpeedBolt/UI/WB_SpeedBoltUI.WB_SpeedBoltUI_C" true))
                      (bind _aswb_speed_bolt_ui (Utilities|Casting|CastToWB_SpeedBoltUI _widget)
                        (:then
                          (bind _output_get_3 (Variables|Default|SetCachedUI _aswb_speed_bolt_ui))
                          (Default|SetChargePercent _output_get_3 0.0))
                        (:CastFailed
                          _))
                      (bind _returnvalue_4 (Utilities|Time|SetTimerbyEvent (EventDispatchers|CreateEvent :!event TickBoltGrowth) (Variables|Default|GetCachedBoltGrowthRate) true))
                      (Variables|Default|SetBoltGrowthTickHandle _returnvalue_4)))
                  (else
                    (Ability|EndAbility)))
                (else
                  (Ability|EndAbility))))
            (:Is%20Not%20Valid
              (Ability|EndAbility))))
        (:CastFailed
          (Ability|EndAbility))))
    (:CastFailed
      (Ability|EndAbility))))

(event Ability|EventOnEndAbility
  (params (bWasCancelled :type Boolean)))

(event EventOnEndAbility
  (params (bWasCancelled :type Boolean))
  (Variables|/Script/Engine.Actor|SetCustomTimeDilation (Variables|Default|GetCachedCharacter) (Variables|Default|GetCachedPrevTimeDilation)))

(fn TickBoltGrowth
  (bind _cachedui (Variables|Default|GetCachedUI))
  (Variables|Default|SetCurrentBoltGrowthTime (+ (Variables|Default|GetCachedBoltGrowthRate) (Variables|Default|GetCurrentBoltGrowthTime)))
  (if (Variables|/Game/CoLab/Blueprints/Arena/GameplayAbilitySystem/Abilities/SpeedBolt/Config/PDA_SpeedBoltConfig.PDA_SpeedBoltConfig_C|GetbScaleCastToSpeed (Variables|Default|GetCachedConfigData))
    (LocalVariables|SetL_NewTimeDilation (- (Variables|/Script/Engine.Actor|GetCustomTimeDilation (Variables|Default|GetCachedCharacter)) (Variables|Default|GetCachedScaledTickPercent)))
    (LocalVariables|SetL_NewTimeDilation (Math|Float|Max(Float) (LocalVariables|GetL_NewTimeDilation) 0.001))
    (Utilities|IsValid _cachedui
      (:Is%20Valid
        (Default|SetChargePercent _cachedui (Math|Float|Lerp 1.0 0.0 (/ (LocalVariables|GetL_NewTimeDilation) (Variables|Default|GetCachedPrevTimeDilation)))))
      (:Is%20Not%20Valid
        _))
    (Variables|/Script/Engine.Actor|SetCustomTimeDilation (Variables|Default|GetCachedCharacter) (LocalVariables|GetL_NewTimeDilation))
    (if (Math|Float|NearlyEqual(Float) (LocalVariables|GetL_NewTimeDilation) 0.0 1e-06)
      (Utilities|Time|ClearandInvalidateTimerbyHandle (Variables|Default|GetBoltGrowthTickHandle)))))