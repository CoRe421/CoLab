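; Surf path actor for the SurfRace mode that defines a spline ending at a target point.
; The construction script calls ResetPathToTargetPoint, which moves the last SurfPath spline point to TargetPoint in local space.
; When TargetPoint is near zero, it first resets to InitialPointLocation and inserts a spline point halfway to it at index 1.
; The event graph holds no active gameplay logic.
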(event EventBeginPlay)

(event Collision|EventActorBeginOverlap
  (params (OtherActor :type Actor%20Object%20Reference)))

(event EventTick
  (params (DeltaSeconds :type Float%20%28single-precision%29)))

(fn ConstructionScript
  (CallFunction|ResetPathtoTargetPoint))

(fn ResetPathtoTargetPoint
  (bind _surfpath (Variables|Default|GetSurfPath))
  (if (Math|Vector|VectorIsNearlyZero (Variables|Default|GetTargetPoint))
    (bind _output_get (Variables|Default|SetTargetPoint (Variables|Default|GetInitialPointLocation)))
    (Spline|AddSplinePointatIndex (Variables|Default|GetSurfPath) (/ _output_get 2.0) 1 "Local" true))
  (Spline|SetLocationatSplinePoint _surfpath (- (Spline|GetNumberOfSplinePoints _surfpath) 1) (Variables|Default|GetTargetPoint) "Local" true))