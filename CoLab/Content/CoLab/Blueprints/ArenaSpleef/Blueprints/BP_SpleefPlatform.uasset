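; Spleef arena platform that builds a SizeX by SizeY grid of box meshes whose touched pieces drop away as physics bodies.
; The construction script rebuilds on size change or ForceReconstruction, using SMRoot for the first cell, added components for others, and instanced platform meshes beneath each.
; OnTouched enables replication and reapplies component settings as simulated, leaving collision only with WorldStatic.
; A distance-based component cleanup function exists, but its tick binding is disconnected.
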(event EventBeginPlay)

(event Collision|EventActorBeginOverlap
  (params (OtherActor :type Actor%20Object%20Reference)))

(event EventTick
  (params (DeltaSeconds :type Float%20%28single-precision%29)))

(event EventOnTouched
  (params (TouchedComponents :type Array%20of%20Primitive%20Component%20Object%20References))
  (Networking|SetReplicates true)
  (for _array_element TouchedComponents
    (CallFunction|ApplyComponentSettings _array_element true)))

(fn ConstructionScript
  (bind _ism_platform (Variables|Default|GetISM_Platform))
  (Utilities|FlowControl|Sequence
    (:then_0
      (if (Math|Boolean|ORBoolean (!= (Variables|Default|GetSizeX) (Variables|Internal|GetPrevSizeX)) (!= (Variables|Default|GetSizeY) (Variables|Internal|GetPrevSizeY)) (Variables|Default|GetbForceReconstruction))
        (Utilities|FlowControl|Sequence
          (:then_0
            (bind _output_get (LocalVariables|SetL_ChildrenComponents (Components|GetChildrenComponents (Variables|Default|GetSM_Root) true)))
            (for _array_element _output_get
              _)
            (bind _returnvalue (Utilities|LoadAssetBlocking (Variables|Default|GetBoxStaticMesh)))
            (bind _asstatic_mesh (Utilities|Casting|CastToStaticMesh _returnvalue))
            (bind _output_get_2 (LocalVariables|SetL_LoadedStaticMesh _asstatic_mesh))
            (Components|StaticMesh|SetStaticMesh (Variables|Default|GetSM_Root) _output_get_2)
            ;[1 1 1] Cache root static mesh bounds
            (LocalVariables|SetL_MeshExtent (.BoxExtent (Math|BoxSphereBounds|BreakBoxSphereBounds (StaticMesh|GetBounds _output_get_2))))
            (bind _returnvalue_2 (Utilities|LoadAssetBlocking (Variables|Default|GetPlatformStaticMesh)))
            (bind _asstatic_mesh_2 (Utilities|Casting|CastToStaticMesh _returnvalue_2)
              (:then
                (bind _output_get_3 (LocalVariables|SetL_LoadedPlatformMesh _asstatic_mesh_2))
                (Components|StaticMesh|SetStaticMesh _ism_platform _output_get_3)
                (Components|InstancedStaticMesh|ClearInstances _ism_platform))
              (:CastFailed
                _))
            (for _index (range 0 (- (Variables|Default|GetSizeX) 1))
              (LocalVariables|SetL_CurrentX _index)
              (for _index_2 (range 0 (- (Variables|Default|GetSizeY) 1))
                (LocalVariables|SetL_CurrentY _index_2)
                (Utilities|FlowControl|Sequence
                  (:then_0
                    ;[1 1 1] Only fires on 0,0
                    (Utilities|FlowControl|DoOnce false
                      (:Completed
                        (LocalVariables|SetL_CurrentComponent (Variables|Default|GetSM_Root))
                        (LocalVariables|SetL_NewTransform (Math|Transform|MakeTransform "0, 0, 0")))))
                  (:then_1
                    ;[1 1 1] Prevents firing on 0,0
                    (Utilities|FlowControl|DoOnce true :!label _label
                      (:Completed
                        (bind _output_get_4 (LocalVariables|SetL_NewTransform (Math|Transform|MakeTransform (Math|Vector|MakeVector (* (LocalVariables|GetL_CurrentX) (.X (Math|Vector|BreakVector (LocalVariables|GetL_MeshExtent))) 2.0) (* (LocalVariables|GetL_CurrentY) (.Y (Math|Vector|BreakVector (LocalVariables|GetL_MeshExtent))) 2.0) (.Z (Math|Vector|BreakVector "0, 0, 0"))))))
                        (bind _returnvalue_3 (AddComponent|AddCollabStaticMeshComponent false _output_get_4))
                        (bind _output_get_5 (LocalVariables|SetL_CurrentComponent _returnvalue_3))
                        (Components|StaticMesh|SetStaticMesh _output_get_5 (LocalVariables|GetL_LoadedStaticMesh)))))
                  (:then_2
                    (goto _label Reset)))
                (CallFunction|ApplyComponentSettings (LocalVariables|GetL_CurrentComponent) false)
                (CallFunction|TryAddPlatformforMesh (LocalVariables|GetL_NewTransform) (LocalVariables|GetL_MeshExtent)))))
          (:then_1
            (Variables|Default|SetbForceReconstruction false)))))
    (:then_1
      (Variables|Internal|SetPrevSizeX (Variables|Default|GetSizeX))
      (Variables|Internal|SetPrevSizeY (Variables|Default|GetSizeY)))))

(fn ApplyComponentSettings
  (params (StaticMeshComponent :type Primitive%20Component%20Object%20Reference) (bSimulated :type Boolean))
  (Class|CollabReplicatedComponentInterface|SetMaxDrawDistance(Message) StaticMeshComponent (Math|Float|SelectFloat 4e+03 1.5e+04 bSimulated))
  (Class|ActorComponent|SetIsReplicated StaticMeshComponent true)
  (Physics|SetSimulatePhysics StaticMeshComponent bSimulated)
  (Transformation|SetMobility StaticMeshComponent "Movable")
  (if bSimulated
    (Transformation|SetAbsolute StaticMeshComponent true false false))
  (Collision|SetCollisionObjectType StaticMeshComponent "ECC_PhysicsBody")
  (Collision|SetCollisionResponsetoAllChannels StaticMeshComponent (select bSimulated "ECR_Ignore" "ECR_Block"))
  (Collision|SetCollisionResponsetoChannel StaticMeshComponent "ECC_PhysicsBody" "ECR_Ignore")
  (Collision|SetCollisionEnabled StaticMeshComponent "QueryAndPhysics")
  (Collision|SetCollisionResponsetoChannel StaticMeshComponent "ECC_WorldStatic" "ECR_Block"))

(fn TryAddPlatformforMesh
  (params (MeshTransform :type Transform%20%28by%20ref%29) (MeshExtent :type Vector))
  (bind (_location _rotation _scale) (Math|Transform|BreakTransform MeshTransform))
  (bind _ism_platform (Variables|Default|GetISM_Platform))
  (bind (_x _y _z) (Math|Vector|BreakVector _location))
  (bind _staticmesh (Variables|/Script/Engine.StaticMeshComponent|GetStaticMesh _ism_platform))
  (Utilities|IsValid _staticmesh
    (:Is%20Valid
      (Components|InstancedStaticMesh|AddInstance (Variables|Default|GetISM_Platform) (Math|Transform|MakeTransform (Math|Vector|MakeVector _x _y (Utilities|Operators|Subtract _z (.Z (Math|Vector|BreakVector MeshExtent)) (.Z (Math|Vector|BreakVector (.BoxExtent (Math|BoxSphereBounds|BreakBoxSphereBounds (StaticMesh|GetBounds _staticmesh))))))) _rotation _scale) false))))

(fn OnComponentTick
  (params (Component :type Collab%20Static%20Mesh%20Component%20Object%20Reference) (DeltaTime :type Float%20%28single-precision%29))
  (Utilities|IsValid Component
    (:Is%20Valid
      (if (> (Math|Vector|Distance(Vector) (Transformation|GetActorLocation) (Transformation|GetWorldLocation Component)) (Variables|Default|GetMaxComponentDistance))
        (Class|CollabReplicatedComponentInterface|DestroyComponent Component)))))