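; Game mode for Arena that ends a match when a player reaches the configured winning score.
; It loads the ruleset from the collab runtime config subsystem and binds to game state score updates.
; A win is passed to the game state, and the game restarts after a short delay.
; Spawned arena characters get a palette color indexed by player ID or a character-code sum of their name.
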(event Custom|TriggerPlayerWin
  (params (Player :type Unique%20Net%20Id%20Repl%20Structure))
  (Development|PrintString (Utilities|String|Append "Player " (Utilities|String|ToString(Integer) (Variables|/Script/Engine.PlayerState|GetPlayerId (Game|GetPlayerStatefromUniqueNetId Player))) " wins!"))
  (Default|HandlePlayerWin (Variables|Default|GetCachedGameState) Player)
  (Variables|Default|SetbGameEnding true)
  (Utilities|FlowControl|Delay 5.0)
  (Class|GameMode|RestartGame))

(event EventBeginPlay
  (|CallParentFunction)
  (CallFunction|InitializeArenaRuleset)
  (bind _asbp_gs_arena (Utilities|Casting|CastToBP_GS_Arena (Game|GetGameState)))
  ;[1 0.1354 0.1354] Check if this works with player states
  (bind _output_get (Variables|Default|SetCachedGameState _asbp_gs_arena))
  (EventDispatchers|BindEventtoOnPlayerScoreUpdated _output_get (EventDispatchers|CreateEvent :!event CheckforPlayerWin)))

(event EventTick
  (params (DeltaSeconds :type Float%20%28single-precision%29))
  (|CallParentFunction DeltaSeconds) ; This node is disabled and will not be called.\nDrag off pins to build functionality.
)

(fn ConstructionScript
  (|CallParentFunction))

(fn CheckforPlayerWin
  (params (PlayerNetID :type Unique%20Net%20Id%20Repl%20Structure) (PlayerScore :type Integer%20%28by%20ref%29))
  (if (>= PlayerScore (Variables|/Game/CoLab/Modes/Arena/GameFramework/Config/PDA_ArenaConfig.PDA_ArenaConfig_C|GetPlayerWinScoreThreshold (Variables|Default|GetArenaConfigRuleset)))
    (CallFunction|TriggerPlayerWin PlayerNetID)
    (return)))

(fn InitializeArenaRuleset
  (Variables|Default|GetArenaConfigRuleset
    (:then)
    (:else
      (bind _returnvalue (Class|CollabRuntimeConfigSubsystem|GetConfigData (Subsystems|GetCollabRuntimeConfigSubsystem) (LocalVariables|GetL_RulesetConfig)))
      (bind _aspda_arena_config (Utilities|Casting|CastToPDA_ArenaConfig _returnvalue))
      (Variables|Default|SetArenaConfigRuleset _aspda_arena_config))))

(fn SpawnDefaultPawnatTransform
  (params (NewPlayer :type Controller%20Object%20Reference) (SpawnTransform :type Transform%20%28by%20ref%29))
  (bind _playerstate (Variables|/Script/Engine.Controller|GetPlayerState NewPlayer))
  (bind _returnvalue (|CallParentFunction NewPlayer SpawnTransform))
  (bind _output_get (LocalVariables|SetL_SpawnedPawn _returnvalue))
  (bind _asbp_arena_character (Utilities|Casting|CastToBP_ArenaCharacter _output_get)
    (:then
      (if (Variables|Default|GetbUseHashedNamesForColors)
        (Utilities|FlowControl|Sequence
          (:then_0
            (bind _output_get_2 (LocalVariables|SetL_PlayerNameString (Utilities|String|GetCharacterArrayfromString (PlayerState|GetPlayerName _playerstate))))
            (for _array_element _output_get_2
              (LocalVariables|SetL_PlayerColorID (+ (Utilities|String|GetCharacterasNumber _array_element) (LocalVariables|GetL_PlayerColorID)))))
          (:then_1
            (Development|PrintString (Utilities|String|Append "Selecting color for player: " (Utilities|String|ToString(Integer) (LocalVariables|GetL_PlayerColorID))) true true "(R=0.079685,G=0.000000,B=1.000000,A=1.000000)" :!label _label)
            (Default|SetDefaultPlayerColor _asbp_arena_character (Utilities|Array|Get(acopy) (Variables|Default|GetPlayerColors) (Math|Integer|%(Integer) (LocalVariables|GetL_PlayerColorID) (Utilities|Array|Length (Variables|Default|GetPlayerColors)))))
            (return (LocalVariables|GetL_SpawnedPawn))))
        (else
          (LocalVariables|SetL_PlayerColorID (Variables|/Script/Engine.PlayerState|GetPlayerId _playerstate))
          (goto _label))))
    (:CastFailed
      (return (LocalVariables|GetL_SpawnedPawn)))))