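; GA_ArenaDeath is the Arena mode's gameplay ability for player death, noted as running only on the server.
; Once committed, it plays the character's multicast death animation, first disabling input and detaching the camera if locally controlled.
; It then reports the death to the game state through BPI_GS_Arena when the event's instigator is valid and not the victim.
; After a short delay it hides the avatar and ends.
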(event Ability|EventActivateAbility
  ;[1 1 1] This is only run on the server, because effect is only applied in C++ on the server
  (bind _returnvalue (Ability|CommitAbility))
  (if _returnvalue
    (CallFunction|HandlePlayerDeath)
    (CallFunction|RegisterPlayerDeath)
    (Utilities|FlowControl|Delay 1.0)
    (Rendering|SetActorHiddenInGame (Ability|GetAvatarActorfromActorInfo) true)
    (Ability|EndAbility)
    (else
      (Ability|EndAbility))))

(event Ability|EventOnEndAbility
  (params (bWasCancelled :type Boolean)))

(fn HandlePlayerDeath
  (bind _asbp_arena_character (Utilities|Casting|CastToBP_ArenaCharacter (Ability|GetAvatarActorfromActorInfo)))
  (bind _output_get (LocalVariables|SetL_Player _asbp_arena_character))
  (if (Pawn|IsLocallyControlled _output_get)
    (Utilities|FlowControl|Sequence
      (:then_0
        (Input|DisableInput (LocalVariables|GetL_Player) (Pawn|GetLocalViewingPlayerController (LocalVariables|GetL_Player)))
        (Default|DetachCamera (LocalVariables|GetL_Player)))
      (:then_1
        (Default|MULPlayDeathAnimation (LocalVariables|GetL_Player) :!label _label)))
    (else
      (goto _label))))

(fn RegisterPlayerDeath
  (bind _currenteventdata (Variables|Default|GetCurrentEventData))
  (bind (_eventtag _instigator _target) (Utilities|Struct|BreakGameplayEventData _currenteventdata))
  (bind _output_get (LocalVariables|SetL_Instigator _instigator))
  (Utilities|IsValid _output_get
    (:Is%20Valid
      (if (!= (LocalVariables|GetL_Instigator) (Variables|/Script/Engine.Pawn|GetPlayerState (.AsPawn (Utilities|Casting|CastToPawn _target))))
        (bind _asbpi_gs_arena (Utilities|Casting|CastToBPI_GS_Arena (Game|GetGameState)))
        (Default|OnPlayerDeath _asbpi_gs_arena (LocalVariables|GetL_Instigator) _target)))))