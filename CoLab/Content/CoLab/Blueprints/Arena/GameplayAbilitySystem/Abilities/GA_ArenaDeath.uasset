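; Gameplay ability for arena character death, intended to run only on the server.
; After committing, it triggers the death animation on BP_ArenaCharacter via MULPlayDeathAnimation, first disabling input and detaching the camera if that character is locally controlled.
; After a one-second delay it hides the avatar rather than destroying it, then ends the ability.
; Physics, destroy and gameplay cue nodes are left unconnected.
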(event Ability|EventActivateAbility
  ;[1 1 1] This is only run on the server, because effect is only applied in C++ on the server
  (bind _returnvalue (Ability|CommitAbility))
  (if _returnvalue
    (CallFunction|HandlePlayerDeath)
    (Utilities|FlowControl|Delay 1.0)
    (Rendering|SetActorHiddenInGame (Ability|GetAvatarActorfromActorInfo) true)
    (Ability|EndAbility)
    (else
      (Ability|EndAbility))))

(event Ability|EventOnEndAbility
  (params (bWasCancelled :type Boolean)))

(fn HandlePlayerDeath
  (bind _asbp_arena_character (Utilities|Casting|CastToBP_ArenaCharacter (Ability|GetAvatarActorfromActorInfo)))
  (bind _output_get (LocalVariables|SetL_Player _asbp_arena_character))
  (if (Pawn|IsLocallyControlled _output_get)
    (Utilities|FlowControl|Sequence
      (:then_0
        (Input|DisableInput (LocalVariables|GetL_Player) (Pawn|GetLocalViewingPlayerController (LocalVariables|GetL_Player)))
        (Default|DetachCamera (LocalVariables|GetL_Player)))
      (:then_1
        (Default|MULPlayDeathAnimation (LocalVariables|GetL_Player) :!label _label)))
    (else
      (goto _label))))