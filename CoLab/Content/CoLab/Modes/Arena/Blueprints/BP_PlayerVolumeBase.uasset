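; Base Arena-mode volume that detects player characters entering and leaving its box, exposing empty enter and leave hooks for children.
; An overlap macro tracks players inside so each hook fires only on real changes.
; Enabling applies collision and visibility on the server; visibility requires being enabled.
; A server-set lifetime timer, cleared on disable, supports a finish notification, and construction tints the cube through a dynamic material.
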(event OnComponentBeginOverlap(Box)
  (params (OverlappedComponent :type Primitive%20Component%20Object%20Reference) (OtherActor :type Actor%20Object%20Reference) (OtherComp :type Primitive%20Component%20Object%20Reference) (OtherBodyIndex :type Integer) (bFromSweep :type Boolean) (SweepResult :type Hit%20Result%20Structure%20%28by%20ref%29))
  (bind _ascollab_player_character (Utilities|Casting|CastToCollabPlayerCharacter OtherActor))
  (Utilities|CheckorAddOverlappingPlayer _ascollab_player_character true
    (:Overlapping
      (CallFunction|OnNewPlayerEnter _ascollab_player_character))))

(event OnComponentEndOverlap(Box)
  (params (OverlappedComponent :type Primitive%20Component%20Object%20Reference) (OtherActor :type Actor%20Object%20Reference) (OtherComp :type Primitive%20Component%20Object%20Reference) (OtherBodyIndex :type Integer))
  (bind _ascollab_player_character (Utilities|Casting|CastToCollabPlayerCharacter OtherActor))
  (Utilities|CheckorAddOverlappingPlayer _ascollab_player_character false
    (:Overlapping
      (CallFunction|OnPlayerLeave _ascollab_player_character))))

(event EventBeginPlay
  (Utilities|FlowControl|Sequence
    (:then_0
      (if (Variables|Default|GetbStartEnabled)
        (CallFunction|SetVolumeEnabled true)
        (else
          ;[1 1 1] Makes sure this hasn't been overriden to be enabled before this has fired
          (if (not (Variables|Default|GetbIsEnabled))
            (CallFunction|SetVolumeEnabled false)))))
    (:then_1
      (CallFunction|SetVisible (Variables|Default|GetbStartVisible)))))

(event Collision|EventActorBeginOverlap
  (params (OtherActor :type Actor%20Object%20Reference)))

(event EventTick
  (params (DeltaSeconds :type Float%20%28single-precision%29)))

(fn ConstructionScript
  (bind _returnvalue (Rendering|Material|CreateDynamicMaterialInstance "/Game/CoLab/Modes/Arena/Assets/M_TransparentColor.M_TransparentColor" "None" "None" :!class /Script/Engine.KismetMaterialLibrary))
  (Rendering|Material|SetVectorParameterValue _returnvalue "Color" (Variables|Default|GetBoxColor) :!class /Script/Engine.MaterialInstanceDynamic)
  (Rendering|Material|SetMaterial (Variables|Default|GetCube) 0 _returnvalue))

(fn SetVolumeEnabled
  (params (bEnabled :type Boolean))
  (Variables|Default|SetbIsEnabled bEnabled)
  ;[1 1 1] Only change on server
  (Networking|SwitchHasAuthority
    (:Authority
      (CallFunction|SetVisible (Variables|Default|GetbIsEnabled))
      (Collision|SetCollisionEnabled (Variables|Default|GetBox) (select (Variables|Default|GetbIsEnabled) "QueryAndPhysics" "NoCollision"))
      (if (not (Variables|Default|GetbIsEnabled))
        (CallFunction|DisableLifetime)))))

(fn SetLifetime
  (params (Lifetime :type Float%20%28double-precision%29))
  ;[1 1 1] Only set lifetime on server
  (Networking|SwitchHasAuthority
    (:Authority
      (if (and (> Lifetime 0.0) (not (Utilities|Time|IsValidTimerHandle (Variables|Default|GetActiveLifetimeTimer))))
        (bind _returnvalue (Utilities|Time|SetTimerbyEvent (EventDispatchers|CreateEvent :!event OnLifetimeFinished) Lifetime))
        (Variables|Default|SetActiveLifetimeTimer _returnvalue)))))

(fn OnLifetimeFinished
  (CallFunction|DisableLifetime)
  (Default|CallOnLifetimeFinish self))

(fn DisableLifetime
  (Utilities|Time|ClearandInvalidateTimerbyHandle (Variables|Default|GetActiveLifetimeTimer)))

(fn OnNewPlayerEnter
  (params (Player :type Collab%20Player%20Character%20Object%20Reference)))

(fn OnPlayerLeave
  (params (Player :type Collab%20Player%20Character%20Object%20Reference)))

(fn SetVisible
  (params (bVisible :type Boolean))
  (if bVisible
    ;[1 1 1] Can only be set to visible if enabled
    (if (Variables|Default|GetbIsEnabled)
      (Rendering|SetActorHiddenInGame self false))
    (else
      (Rendering|SetActorHiddenInGame true))))