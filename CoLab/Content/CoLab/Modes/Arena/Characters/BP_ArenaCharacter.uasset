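; BP_ArenaCharacter is the networked first-person player character for the CoLab Arena mode.
; A timer scales a looping 2D sound's volume with speed, and the runtime Arena config, cached on authority, selects the sound.
; RepNotifies apply camera pitch, player color, time dilation, speed sound and ignored-collision actors.
; Death animation rolls the mesh, while weapon firing, local death handling and health/mana bindings are stubbed or disconnected.
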(event Custom|SR_FireWeapon
  (params (Weapon :type Co%20Lab%20Weapon%20Interface%20Interface)))

(event Custom|CL_InitializeSpeedSound
  (Utilities|IsValid (Variables|Default|GetSpeedSoundComponent)
    (:Is%20Valid
      (Audio|Components|Audio|Stop (Variables|Default|GetSpeedSoundComponent))
      (Components|DestroyComponent (Variables|Default|GetSpeedSoundComponent)))
    (:Is%20Not%20Valid
      _))
  (bind _returnvalue (Audio|CreateSound2D (Variables|Default|GetSpeedSound) 0.1 1.0 0.0 0 false false))
  (bind _output_get (Variables|Default|SetSpeedSoundComponent _returnvalue))
  (Class|AudioComponent|SetUISound _output_get true)
  ;[1 1 1] Don't need this because looping is handled at a soundwave level
  (EventDispatchers|AssignOnAudioFinished _output_get (delegate Custom|OnSpeedSoundFinished))
  (bind _returnvalue_2 (Utilities|Time|SetTimerbyEvent (delegate Custom|OnSpeedSoundTick) (Variables|Default|GetSpeedSoundTickRate) true))
  (Variables|Default|SetSpeedSoundTickTimerHandle _returnvalue_2)
  (Audio|Components|Audio|Play (Variables|Default|GetSpeedSoundComponent) 0.0))

(event Custom|CL_ControllerPlayerDeath
  ;[1 1 1] Will only fire on local client with a valid PlayerController
  (if (Pawn|IsLocallyControlled)
    _))

(event Custom|OnSpeedSoundFinished)

(event Custom|MUL_PlayDeathAnimation
  (Variables|Default|SetPreDeathRotation (Variables|/Script/Engine.SceneComponent|GetRelativeRotation (Variables|Default|GetMesh1P)))
  (bind _rotationpercent (Timeline|DeathTimeline PlayFromStart)
    (:Update
      (Transformation|SetRelativeRotation (Variables|Default|GetMesh1P) (Math|Rotator|Lerp(Rotator) (Math|Rotator|MakeRotator 0.0 (.Pitch (Math|Rotator|BreakRotator (Variables|Default|GetPreDeathRotation))) (.Yaw (Math|Rotator|BreakRotator (Variables|Default|GetPreDeathRotation)))) (Math|Rotator|MakeRotator 9e+01 (.Pitch (Math|Rotator|BreakRotator (Variables|Default|GetPreDeathRotation))) (.Yaw (Math|Rotator|BreakRotator (Variables|Default|GetPreDeathRotation)))) _rotationpercent) false false))))

(event Custom|SVR_SetPlayerCameraPitch
  (params (PlayerCameraPitch :type Float%20%28double-precision%29))
  (Variables|Default|SetPlayerCameraPitch PlayerCameraPitch))

(event Custom|OnSpeedSoundTick
  (bind _cachedcastedmovementcomponent (Variables|Default|GetCachedCastedMovementComponent))
  (bind _minspeedsoundspeed (Variables|Default|GetMinSpeedSoundSpeed))
  (Utilities|IsValid _cachedcastedmovementcomponent
    (:Is%20Valid
      (Audio|Components|Audio|SetVolumeMultiplier (Variables|Default|GetSpeedSoundComponent) (Math|Float|Clamp(Float) (Utilities|Operators|Divide (- (Math|Vector|VectorLength (Variables|/Script/Engine.MovementComponent|GetVelocity _cachedcastedmovementcomponent)) _minspeedsoundspeed) (- (Variables|Default|GetMaxSpeedSoundSpeed) _minspeedsoundspeed) 3.0) 0.0 0.75) :!class /Script/Engine.AudioComponent))))

(event Custom|OnArenaConfigPropertyChanged
  (params (PropertyName :type Name))
  (bind _cachedarenaconfig (Variables|Default|GetCachedArenaConfig))
  (Variables|Default|SetSpeedSound (select (and (Utilities|IsValid _cachedarenaconfig) (Variables|/Game/CoLab/Modes/Arena/GameFramework/Config/PDA_ArenaConfig.PDA_ArenaConfig_C|GetbItalian _cachedarenaconfig)) "/Game/CoLab/Modes/Arena/Assets/Sounds/Mario/mlrpg3_luigi_shivering1_Loop.mlrpg3_luigi_shivering1_Loop" "/Game/CoLab/Modes/Arena/Assets/Sounds/BrawlhallaSounds/4_WEP_Explosion_71_Loop.4_WEP_Explosion_71_Loop")))

(event Custom|TryCacheConfigData
  (bind _returnvalue (Class|CollabRuntimeConfigSubsystem|GetConfigData (Subsystems|GetCollabRuntimeConfigSubsystem) "/Game/CoLab/Modes/Arena/GameFramework/Config/PDA_ArenaConfig.PDA_ArenaConfig_C"))
  (bind _output_get (Variables|Default|SetCachedArenaConfig _returnvalue))
  (Utilities|IsValid _output_get
    (:Is%20Valid
      (EventDispatchers|BindEventtoOnConfigPropertyChanged _output_get (EventDispatchers|CreateEvent :!event Custom|OnArenaConfigPropertyChanged))
      (CallFunction|OnArenaConfigPropertyChanged "None"))))

(event Input|EnhancedActionEvents|EnhancedInputActionIA_CollabLookMouse
  (params (ActionValue :type Vector%202D%20Structure) (ElapsedSeconds :type Float%20%28double-precision%29) (TriggeredSeconds :type Float%20%28double-precision%29) (InputAction :type Input%20Action%20Object%20Reference :default "/Collab/Input/Actions/IA_CollabLookMouse.IA_CollabLookMouse"))
  (CallFunction|SVRSetPlayerCameraPitch (.Pitch (Math|Rotator|BreakRotator (Transformation|GetWorldRotation (Variables|Default|GetFirstPersonCameraComponent))))))

(event EventBeginPlay
  (Utilities|FlowControl|Sequence
    (:then_0
      (bind _ascollab_movement_component (Utilities|Casting|CastToCollabMovementComponent (Variables|Character|GetCharacterMovement)))
      (Variables|Default|SetCachedCastedMovementComponent _ascollab_movement_component)
      (CallFunction|CLInitializeSpeedSound))
    (:then_1
      (Networking|SwitchHasAuthority
        (:Authority
          (CallFunction|TryCacheConfigData))))
    (:then_3
      (CallFunction|UpdateOverlappedActorsonSpawn))))

(event EventOnDestroyCharacter
  (CallFunction|OnCharacterDeath)
  (Development|PrintString "Hello1"))

(event EventTick
  (params (DeltaSeconds :type Float%20%28single-precision%29)))

(event EventSetChargePercent
  (params (NewPercent :type Float%20%28double-precision%29))
  (Variables|Default|SetCurrentPlayerColor (Math|Color|Lerp(LinearColor) (Variables|Default|GetDefaultPlayerColor) "(R=0.614396,G=0.000000,B=1.000000,A=1.000000)" NewPercent)))

(event Input|KeyboardEvents|Q
  (params (Key :type Key%20Structure :default "None")))

(event Input|KeyboardEvents|F5
  (params (Key :type Key%20Structure :default "None")))

(event Input|KeyboardEvents|CapsLock
  (params (Key :type Key%20Structure :default "None")))

(fn ConstructionScript
  (Utilities|FlowControl|Sequence
    (:then_0
      (bind _returnvalue (Rendering|Material|CreateDynamicMaterialInstance (Variables|Default|GetPlayerMeshParentMaterial) "None" "None" :!class /Script/Engine.KismetMaterialLibrary))
      (Variables|Default|SetMeshMaterialInstance _returnvalue)
      (CallFunction|SetDefaultPlayerColor (Variables|Default|GetDefaultPlayerColor))
      (Rendering|Material|SetMaterial (Variables|Default|GetMesh3P) 0 (Variables|Default|GetMeshMaterialInstance)))
    (:then_1
      (Variables|Default|SetRep_TimeDilation (Variables|Default|GetCustomTimeDilation)))))

(fn TryFire
  (params (Value :type Input%20Action%20Value%20Structure%20%28by%20ref%29))
  (bind _output_get (LocalVariables|SetL_WeaponComponents (Class|Actor|GetComponentsbyInterface "/Script/CoLab.CoLabWeaponInterface")))
  (for _array_element _output_get
    (bind _asco_lab_weapon_interface (Utilities|Casting|CastToCoLabWeaponInterface _array_element))
    (CallFunction|SRFireWeapon _asco_lab_weapon_interface)))

(fn OnHealthChanged
  (params (NewHealth :type Float%20%28single-precision%29) (MaxHealth :type Float%20%28single-precision%29))
  (bind _aswb_character_attributes (Utilities|Casting|CastToWB_CharacterAttributes (UserInterface|GetWidget (Variables|Default|GetAttributeWidgetComponent))))
  (Default|SetHealth _aswb_character_attributes NewHealth MaxHealth))

(fn SetupAbilitySystemComponentBindings
  (|CallParentFunction))

(fn OnManaChanged
  (params (NewMana :type Float%20%28single-precision%29) (OldMana :type Float%20%28single-precision%29))
  (bind _aswb_character_attributes (Utilities|Casting|CastToWB_CharacterAttributes (UserInterface|GetWidget (Variables|Default|GetAttributeWidgetComponent))))
  (Default|SetMana _aswb_character_attributes NewMana OldMana))

(fn OnCharacterDeath
  (Utilities|FlowControl|Sequence
    (:then_0
      (CallFunction|CLControllerPlayerDeath))))

(fn DetachCamera
  (Transformation|DetachFromComponent (Variables|Default|GetFirstPersonCameraComponent) "KeepRelative" "KeepRelative" "KeepRelative" true))

(fn OnRepPlayerCameraPitch
  (bind _firstpersoncameracomponent (Variables|Default|GetFirstPersonCameraComponent))
  (bind _returnvalue (Transformation|GetWorldRotation _firstpersoncameracomponent))
  (bind (_roll _pitch _yaw) (Math|Rotator|BreakRotator _returnvalue))
  (Transformation|SetWorldRotation _firstpersoncameracomponent (Math|Rotator|MakeRotator _roll (Variables|Default|GetPlayerCameraPitch) _yaw) false false))

(fn SetIgnoreActorCollisions
  (params (Actor :type Actor%20Object%20Reference) (bShouldIgnore :type Boolean))
  (bind _repcollisionignoredactors (Variables|Default|GetRepCollisionIgnoredActors))
  (bind _localcollisionignoredactors (Variables|Default|GetLocalCollisionIgnoredActors))
  (Collision|IgnoreActorwhenMoving (Variables|Default|GetCapsuleComponent) Actor bShouldIgnore)
  (if bShouldIgnore
    (Utilities|Array|AddUnique _localcollisionignoredactors Actor)
    (Utilities|Array|AddUnique _repcollisionignoredactors Actor)
    (else
      (Utilities|Array|RemoveItem _localcollisionignoredactors Actor)
      (Utilities|Array|RemoveItem _repcollisionignoredactors Actor))))

(fn OnRepRepCollisionIgnoredActors
  (bind _capsulecomponent (Variables|Default|GetCapsuleComponent))
  (Collision|ClearMoveIgnoreActors (Variables|Default|GetCapsuleComponent))
  (for _array_element (Variables|Default|GetRepCollisionIgnoredActors)
    (Collision|IgnoreActorwhenMoving _capsulecomponent _array_element true))
  (for _array_element_2 (Variables|Default|GetLocalCollisionIgnoredActors)
    (Collision|IgnoreActorwhenMoving _capsulecomponent _array_element_2 true)))

(fn GetInputDirectionforTargetSpeed
  (params (TargetSpeed :type Float%20%28double-precision%29) (Velocity :type Vector))
  (bind (_x _y) (Math|Vector|BreakVector Velocity))
  (bind _returnvalue (Math|Vector|MakeVector _x _y 0.0))
  (bind _returnvalue_2 (Math|Vector|DotProduct _returnvalue _returnvalue))
  (bind _returnvalue_3 (* _returnvalue TargetSpeed))
  (bind _returnvalue_4 (+ "" _returnvalue_3))
  (bind _returnvalue_5 (/ _returnvalue_4 _returnvalue_2))
  (bind (_x_2 _y_2) (Math|Vector|BreakVector _returnvalue_5))
  (return (Math|Vector|MakeVector _x_2 _y_2 0.0)))

(fn OnRepCurrentPlayerColor
  (CallFunction|ApplyPlayerColor))

(fn SetReplicatedTimeDilation
  (params (NewTimeDilation :type Float%20%28double-precision%29))
  (Variables|Default|SetRep_TimeDilation NewTimeDilation))

(fn OnRepRepTimeDilation
  (Variables|Default|SetCustomTimeDilation (Variables|Default|GetRep_TimeDilation)))

(fn SetDefaultPlayerColor
  (params (DefaultPlayerColor :type Linear%20Color%20Structure))
  (Variables|Default|SetDefaultPlayerColor DefaultPlayerColor))

(fn ApplyPlayerColor
  (Rendering|Material|SetVectorParameterValue (Variables|Default|GetMeshMaterialInstance) (Variables|Default|GetMaterialColorParameter) (Variables|Default|GetCurrentPlayerColor) :!class /Script/Engine.MaterialInstanceDynamic))

(fn OnRepDefaultPlayerColor
  (Variables|Default|SetCurrentPlayerColor (Variables|Default|GetDefaultPlayerColor)))

(fn UpdateOverlappedActorsonSpawn
  (bind _capsulecomponent (Variables|Default|GetCapsuleComponent))
  (bind _outactors (Collision|ComponentOverlapActors _capsulecomponent (Transformation|GetWorldTransform _capsulecomponent) (Utilities|Array|MakeArray) 0 (Utilities|Array|MakeArray)))
  (bind _output_get (LocalVariables|SetL_OverlappedActors _outactors))
  (for _array_element _output_get
    (Class|BPIOverlaponSpawn|AddSpawnedOverlappedActor(Message) _array_element self)))

(fn OnRepSpeedSound
  (CallFunction|CLInitializeSpeedSound))

(fn GetProjectileSpawnComponent
  (return (Variables|Default|GetProjectileSpawnLocation)))

(fn GetProjectileSpawnLocation
  (bind _projectilespawnlocation (Variables|Default|GetProjectileSpawnLocation))
  (bind _returnvalue (Transformation|GetWorldTransform _projectilespawnlocation))
  (bind (_location _rotation) (Math|Transform|BreakTransform _returnvalue))
  (return _location _rotation))