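; Arena mode game state that tracks per-player scores, the active ruleset config and the winning player.
; On authority it awards kill points from the ruleset and syncs score entries with the player list.
; RepNotifies propagate score, config and winner changes, with the winner relayed through each Arena player controller.
; Score and config changes refresh player-list widgets found by interface.
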(event Custom|SVR_UpdateCachedRuleset
  (bind _returnvalue (Class|CollabRuntimeConfigSubsystem|GetConfigData (Subsystems|GetCollabRuntimeConfigSubsystem) "/Game/CoLab/Modes/Arena/GameFramework/Config/PDA_ArenaConfig.PDA_ArenaConfig_C"))
  (bind _output_get (Variables|Default|SetCachedRulesetConfig _returnvalue))
  (EventDispatchers|BindEventtoOnConfigPropertyChanged _output_get (delegate Custom|OnConfigPropertyChanged)))

(event Custom|HandlePlayerWin
  (params (WinningPlayer :type Unique%20Net%20Id%20Repl%20Structure))
  (Variables|Default|SetWinningPlayer (Game|GetPlayerStatefromUniqueNetId WinningPlayer)))

(event Custom|OnConfigPropertyChanged
  (params (PropertyName :type Name))
  (CallFunction|UpdateTabMenus))

(event Custom|OnPlayerScoreUpdate
  (params (PlayerNetID :type Unique%20Net%20Id%20Repl%20Structure) (PlayerScore :type Integer%20%28by%20ref%29))
  (CallFunction|UpdateTabMenus))

(event EventBeginPlay
  (|CallParentFunction)
  (Utilities|FlowControl|Sequence
    (:then_0
      (EventDispatchers|BindEventtoOnPlayerListUpdated (EventDispatchers|CreateEvent :!event PlayerListUpdated)))
    (:then_1
      (Networking|SwitchHasAuthority
        (:Authority
          (bind _asbpi_gm_arena (Utilities|Casting|CastToBPI_GM_Arena (Game|GetGameMode)))
          (Variables|Default|SetCachedGameMode _asbpi_gm_arena)
          (CallFunction|SVRUpdateCachedRuleset)
          (EventDispatchers|BindEventtoOnPlayerScoreUpdated (delegate Custom|OnPlayerScoreUpdate)))
        (:Remote
          (CallFunction|SVRUpdateCachedRuleset))))))

(event EventTick
  (params (DeltaSeconds :type Float%20%28single-precision%29))
  (|CallParentFunction DeltaSeconds) ; This node is disabled and will not be called.\nDrag off pins to build functionality.
)

(event EventOnPlayerDeath
  (params (Instigator :type Actor%20Object%20Reference) (Target :type Actor%20Object%20Reference))
  (Networking|SwitchHasAuthority
    (:Authority
      (bind _asplayer_state (Utilities|Casting|CastToPlayerState Instigator))
      (CallFunction|AddPlayerScore (PlayerState|GetUniqueID _asplayer_state) (Variables|/Game/CoLab/Modes/Arena/GameFramework/Config/PDA_ArenaConfig.PDA_ArenaConfig_C|GetPlayerKillScoreValue (Variables|Default|GetCachedRulesetConfig))))))

(fn ConstructionScript
  (|CallParentFunction))

(fn AddPlayerScore
  (params (PlayerNetID :type Unique%20Net%20Id%20Repl%20Structure) (ScoreToAdd :type Integer%20%28by%20ref%29))
  (bind (_playerscore _bfound) (CallFunction|TryFindPlayerScore PlayerNetID))
  (CallFunction|SetPlayerScore PlayerNetID (Math|Integer|SelectInt (+ (.Score (Utilities|Struct|BreakS_PlayerScore _playerscore)) ScoreToAdd) ScoreToAdd _bfound)))

(fn UpdateTabMenus
  (bind _foundwidgets (Class|WidgetBlueprintLibrary|GetAllWidgetswithInterface "/Collab/UI/Common/TabMenu/BPI_CollabPlayerListItem.BPI_CollabPlayerListItem_C" false))
  (for _array_element _foundwidgets
    (Class|BPICollabPlayerListItem|UpdateWidget(Message) _array_element)))

(fn UpdateRulesetProperties
  (params (PropertyName :type Name))
  (CallFunction|SVRUpdateCachedRuleset))

(fn TryFindPlayerScore
  (params (PlayerNetID :type Unique%20Net%20Id%20Repl%20Structure))
  (for _array_element (Variables|Default|GetPlayerScores)
    (if (== (Game|GetPlayerStatefromUniqueNetId (.PlayerNetID (Utilities|Struct|BreakS_PlayerScore _array_element))) (Game|GetPlayerStatefromUniqueNetId PlayerNetID))
      (return _array_element true)))
  (return "" false))

(fn SetPlayerScore
  (params (PlayerNetID :type Unique%20Net%20Id%20Repl%20Structure) (NewScore :type Integer))
  (Networking|SwitchHasAuthority
    (:Authority
      (for _index (range 0 (Utilities|Array|LastIndex (Variables|Default|GetPlayerScores)))
        (if (== (Game|GetPlayerStatefromUniqueNetId (.PlayerNetID (Utilities|Struct|BreakS_PlayerScore (Utilities|Array|Get(acopy) (Variables|Default|GetPlayerScores) _index)))) (Game|GetPlayerStatefromUniqueNetId PlayerNetID))
          (if (!= (.Score (Utilities|Struct|BreakS_PlayerScore (Utilities|Array|Get(acopy) (Variables|Default|GetPlayerScores) _index))) NewScore)
            (Utilities|Struct|SetmembersinS_PlayerScore (Utilities|Array|Get(acopy) (Variables|Default|GetPlayerScores) _index) NewScore)
            (Default|CallOnPlayerScoreUpdated PlayerNetID NewScore)
            (return)
            (else
              (return)))))
      ;[1 1 1] If player wasn't found, will add new player to array here
      (Utilities|Array|Add (Variables|Default|GetPlayerScores) (Utilities|Struct|MakeS_PlayerScore PlayerNetID NewScore))
      (return))))

(fn PlayerListUpdated
  (Networking|SwitchHasAuthority
    (:Authority
      (CallFunction|UpdateLocalPlayerScores))))

(fn UpdateLocalPlayerScores
  (for _array_element (Variables|Default|GetRepPlayerArray)
    (Utilities|Set|Add (LocalVariables|GetL_FoundPlayers) (PlayerState|GetUniqueID _array_element))
    (bind _bfound (CallFunction|TryFindPlayerScore (PlayerState|GetUniqueID _array_element)))
    (if (not _bfound)
      (CallFunction|SetPlayerScore (PlayerState|GetUniqueID _array_element))))
  (LocalVariables|SetL_CurrentIndex 0)
  (while (< (LocalVariables|GetL_CurrentIndex) (Utilities|Array|Length (Variables|Default|GetPlayerScores)))
    (if (Utilities|Set|Contains (LocalVariables|GetL_FoundPlayers) (.PlayerNetID (Utilities|Struct|BreakS_PlayerScore (Utilities|Array|Get(acopy) (Variables|Default|GetPlayerScores) (LocalVariables|GetL_CurrentIndex)))))
      (Math|Integer|IncrementInt (LocalVariables|GetL_CurrentIndex))
      (else
        (Utilities|Array|RemoveIndex (Variables|Default|GetPlayerScores) (LocalVariables|GetL_CurrentIndex))))))

(fn OnRepPlayerScores
  (CallFunction|OnPlayerScoreUpdate))

(fn OnRepWinningPlayer
  (bind _winningplayer (Variables|Default|GetWinningPlayer))
  (for _array_element (Variables|Default|GetRepPlayerArray)
    (bind _asbp_pc_arena (Utilities|Casting|CastToBP_PC_Arena (Game|GetPlayerController _array_element)))
    (Default|MULHandlePlayerWin _asbp_pc_arena (PlayerState|GetPlayerName _winningplayer) (== _array_element _winningplayer))))

(fn OnRepCachedRulesetConfig
  (bind _cachedrulesetconfig (Variables|Default|GetCachedRulesetConfig))
  (CallFunction|UpdateTabMenus)
  (Utilities|IsValid _cachedrulesetconfig
    (:Is%20Valid
      ;[1 1 1] Doesn't get broadcast properly on the server so need to force update this via other delegate, but this works for clients
      (EventDispatchers|BindEventtoOnPropertyReplicated _cachedrulesetconfig (EventDispatchers|CreateEvent :!event UpdateTabMenus)))))

(fn GetMaxPlayerScore
  (bind _cachedrulesetconfig (Variables|Default|GetCachedRulesetConfig)
    (:then
      (return (Variables|/Game/CoLab/Modes/Arena/GameFramework/Config/PDA_ArenaConfig.PDA_ArenaConfig_C|GetPlayerWinScoreThreshold _cachedrulesetconfig)))
    (:else)))

(fn GetPlayerScore
  (params (PlayerNetID :type Unique%20Net%20Id%20Repl%20Structure))
  (bind (_playerscore _bfound) (CallFunction|TryFindPlayerScore PlayerNetID))
  (if _bfound
    (return (.Score (Utilities|Struct|BreakS_PlayerScore _playerscore)))
    (else
      (return -1))))