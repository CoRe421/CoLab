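; Arena-mode collision volume that stops overlapping players moving along the axes flagged by BlockX, BlockY and BlockZ.
; On entry and every Tick, it zeroes those velocity components on the MovementComponent, or on a physics-simulating root.
; Tick also teleports each player by the velocity change times delta time to undo movement, which a note says causes slow upward drift.
; Debug prints remain, and ActorVelocities survives from unused experiments.
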(event EventBeginPlay)

(event Collision|EventActorBeginOverlap
  (params (OtherActor :type Actor%20Object%20Reference)))

(event EventTick
  (params (DeltaSeconds :type Float%20%28single-precision%29))
  (bind _result (Utilities|Set|ToArray (Variables|Default|GetOverlappedPlayers)))
  (for _array_element _result
    (bind _velocity_change (CallFunction|ResetActorVelocity _array_element))
    (Transformation|SetActorLocation _array_element (+ (Transformation|GetActorLocation _array_element) (* _velocity_change DeltaSeconds)) false true)))

(fn ConstructionScript
  (|CallParentFunction))

(fn ResetActorVelocity
  (params (Actor :type Actor%20Object%20Reference))
  (bind _rootcomponent (Variables|/Script/Engine.Actor|GetRootComponent Actor))
  (bind _output_get (LocalVariables|SetL_MovementComponent (Actor|GetComponentbyClass Actor "/Script/Engine.MovementComponent")))
  (Utilities|IsValid _output_get
    (:Is%20Valid
      (bind _output_get_2 (LocalVariables|SetL_PrevVelocity (Variables|/Script/Engine.MovementComponent|GetVelocity (LocalVariables|GetL_MovementComponent))))
      (bind _output_get_3 (LocalVariables|SetL_NewVelocity (CallFunction|ApplyVelocityReset _output_get_2 Actor)))
      (Variables|/Script/Engine.MovementComponent|SetVelocity (LocalVariables|GetL_MovementComponent) _output_get_3)
      ;[1 1 1] For some reason the delta for Z is slightly stronger than gravity so player will slowly rise upwards
      (return (- (LocalVariables|GetL_NewVelocity) (LocalVariables|GetL_PrevVelocity))))
    (:Is%20Not%20Valid
      (if (Class|SceneComponent|IsAnySimulatingPhysics _rootcomponent)
        (bind _asprimitive_component (Utilities|Casting|CastToPrimitiveComponent _rootcomponent))
        (bind _returnvalue (Physics|GetPhysicsLinearVelocity _asprimitive_component "None"))
        (bind _output_get_4 (LocalVariables|SetL_PrevVelocity _returnvalue))
        (bind _output_get_5 (LocalVariables|SetL_NewVelocity (CallFunction|ApplyVelocityReset _output_get_4 Actor)))
        (Class|PrimitiveComponent|SetAllPhysicsLinearVelocity _asprimitive_component _output_get_5 false)
        (return (- (LocalVariables|GetL_NewVelocity) (LocalVariables|GetL_PrevVelocity)))))))

(fn ApplyVelocityReset
  (params (Velocity :type Vector) (Actor :type Actor%20Object%20Reference))
  (bind (_x _y _z) (Math|Vector|BreakVector Velocity))
  (bind _returnvalue (Math|Vector|VectorZero))
  (bind _bblockx_ (Variables|Default|GetbBlockX+))
  (bind _bblockx__2 (Variables|Default|GetbBlockX-))
  (bind _bblocky_ (Variables|Default|GetbBlockY-))
  (bind _bblocky__2 (Variables|Default|GetbBlockY+))
  (bind _bblockz_ (Variables|Default|GetbBlockZ-))
  (bind _bblockz__2 (Variables|Default|GetbBlockZ+))
  (bind (_x_2 _y_2 _z_2) (Math|Vector|BreakVector _returnvalue))
  (bind _returnvalue_2 (<= _z 0.0))
  (bind _returnvalue_3 (<= _x 0.0))
  (bind _returnvalue_4 (<= _y 0.0))
  (bind _returnvalue_5 (Math|Float|Min(Float) _x _x_2))
  (bind _returnvalue_6 (Math|Float|Max(Float) _y _y_2))
  (bind _returnvalue_7 (Math|Float|Min(Float) _y _y_2))
  (bind _returnvalue_8 (Math|Float|Max(Float) _z _z_2))
  (bind _returnvalue_9 (Math|Float|Min(Float) _z _z_2))
  (bind _returnvalue_10 (Math|Float|Max(Float) _x _x_2))
  (bind _returnvalue_11 (Math|Float|SelectFloat _returnvalue_9 _z _bblockz__2))
  (bind _returnvalue_12 (Math|Float|SelectFloat _returnvalue_8 _z _bblockz_))
  (bind _returnvalue_13 (Math|Float|SelectFloat _returnvalue_10 _x _bblockx__2))
  (bind _returnvalue_14 (Math|Float|SelectFloat _returnvalue_5 _x _bblockx_))
  (bind _returnvalue_15 (Math|Float|SelectFloat _returnvalue_6 _y _bblocky_))
  (bind _returnvalue_16 (Math|Float|SelectFloat _returnvalue_7 _y _bblocky__2))
  (bind _returnvalue_17 (Math|Float|SelectFloat _returnvalue_12 _returnvalue_11 _returnvalue_2))
  (bind _returnvalue_18 (Math|Float|SelectFloat _returnvalue_13 _returnvalue_14 _returnvalue_3))
  (bind _returnvalue_19 (Math|Float|SelectFloat _returnvalue_15 _returnvalue_16 _returnvalue_4))
  (bind _returnvalue_20 (Math|Vector|MakeVector _returnvalue_18 _returnvalue_19 _returnvalue_17))
  (Development|PrintString (Utilities|String|ToString(Integer) _returnvalue_20) true true "(R=0.000000,G=1.000000,B=0.951383,A=1.000000)" 0.0)
  (return _returnvalue_20))

(fn OnNewPlayerEnter
  (params (Player :type Collab%20Player%20Character%20Object%20Reference))
  (|CallParentFunction Player)
  (CallFunction|ResetActorVelocity Player))

(fn OnPlayerLeave
  (params (Player :type Collab%20Player%20Character%20Object%20Reference))
  (|CallParentFunction Player)
  (Utilities|Map|Remove (Variables|Default|GetActorVelocities) Player))