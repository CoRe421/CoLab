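; Arena mode player controller that relays combat, scoring and win feedback to the arena HUD and local audio.
; It binds to the pawn health component's damage delegate and forwards hits through a client event that shows damage UI and plays a sound.
; Kills and points-volume scores play a client-side score sound, with the cached arena config able to swap in "Italian" sound variants.
; On death it strips the casting gameplay tag.
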(event Custom|MUL_HandlePlayerWin
  (params (PlayerName :type String) (bCurrentPlayerWon :type Boolean))
  (bind _aswb_arena_hud (Utilities|Casting|CastToWB_ArenaHUD (Variables|Default|GetGameplayHUD)))
  (Default|TriggerPlayerWinText _aswb_arena_hud (Utilities|String|SelectText "You win!" (Utilities|Text|FormatText "{Player} wins!" PlayerName) bCurrentPlayerWon)))

(event Custom|CL_PlayScoreSound
  (bind _cachedarenaconfig (Variables|Default|GetCachedArenaConfig))
  (if (Pawn|IsLocallyControlled (Pawn|GetControlledPawn))
    (Audio|PlaySound2D (select (and (Utilities|IsValid _cachedarenaconfig) (Variables|/Game/CoLab/Modes/Arena/GameFramework/Config/PDA_ArenaConfig.PDA_ArenaConfig_C|GetbItalian _cachedarenaconfig)) "/Game/CoLab/Modes/Arena/Assets/Sounds/Mario/mlrpg3_mario_oh_yeah_2.mlrpg3_mario_oh_yeah_2" (Variables|Default|GetPlayerScoreSound)) 1.0 1.0 0.0 0 0)))

(event Custom|OnDamaged
  (params (Damage :type Float%20%28single-precision%29))
  ;[1 1 1] Needs to multicast because client doesn't bind this properly because 'controlled pawn' isn't valid at this time, but even if it WAS the damaged delegate is only broacast on server because damage is only on the server. Could theoretically broadcast from health changing, but think it's safer and makes more sense to just trigger from specifically the damage attribute that has an instigator/etc
  (CallFunction|CLonDamaged Damage))

(event Custom|CL_OnDamaged
  (params (Damage :type Float%20%28double-precision%29))
  (bind _cachedarenaconfig (Variables|Default|GetCachedArenaConfig))
  ;[1 1 1] Needs to multicast because client doesn't bind this properly because 'controlled pawn' isn't valid at this time, but even if it WAS the damaged delegate is only broacast on server because damage is only on the server. Could theoretically broadcast from health changing, but think it's safer and makes more sense to just trigger from specifically the damage attribute that has an instigator/etc
  ;;[1 1 1] NOT reliable because purely cosmetic
  (CallFunction|TriggerTookDamageUI Damage)
  (Audio|PlaySound2D (select (and (Utilities|IsValid _cachedarenaconfig) (Variables|/Game/CoLab/Modes/Arena/GameFramework/Config/PDA_ArenaConfig.PDA_ArenaConfig_C|GetbItalian _cachedarenaconfig)) "/Game/CoLab/Modes/Arena/Assets/Sounds/Mario/mlrpg3_luigi_help.mlrpg3_luigi_help" "/Game/CoLab/Modes/Arena/Assets/Sounds/SW_TookDamage3.SW_TookDamage3") 1.0 1.0 0.0 0 self))

(event EventBeginPlay
  (|CallParentFunction)
  (bind _returnvalue (Class|CollabRuntimeConfigSubsystem|GetConfigData (Subsystems|GetCollabRuntimeConfigSubsystem) "/Game/CoLab/Modes/Arena/GameFramework/Config/PDA_ArenaConfig.PDA_ArenaConfig_C"))
  (Variables|Default|SetCachedArenaConfig _returnvalue))

(event EventTick
  (params (DeltaSeconds :type Float%20%28single-precision%29)))

(event EventDestroyed)

(event EventOnPlayerKill
  (CallFunction|CLPlayScoreSound))

(event EventOnPlayerDeath
  (params (PlayerActor :type Actor%20Object%20Reference))
  (Ability|GameplayEffect|RemoveLooseGameplayTags PlayerActor (GameplayTags|MakeLiteralGameplayTagContainer "(GameplayTags=((TagName=\"Gameplay.State.Casting\")))"))
  (|CallParentFunction PlayerActor))

(event EventOnPointsVolumeScore
  (CallFunction|CLPlayScoreSound))

(event EventSetupPlayerBindings
  (bind _returnvalue (Pawn|GetControlledPawn))
  (bind _returnvalue_2 (Actor|GetComponentbyClass _returnvalue "/Script/Collab.CollabHealthComponent"))
  (|CallParentFunction)
  (Utilities|FlowControl|Sequence
    (:then_0
      (Utilities|IsValid _returnvalue_2
        (:Is%20Valid
          ;[1 1 1] Needs to multicast because client doesn't bind this properly because 'controlled pawn' isn't valid at this time, but even if it WAS the damaged delegate is only broacast on server because damage is only on the server. Could theoretically broadcast from health changing, but think it's safer and makes more sense to just trigger from specifically the damage attribute that has an instigator/etc
          (EventDispatchers|AssignOnDamaged _returnvalue_2 (delegate Custom|OnDamaged)))))))

(fn ConstructionScript
  (|CallParentFunction))

(fn TriggerDealtDamageUI
  (bind _aswb_arena_hud (Utilities|Casting|CastToWB_ArenaHUD (Variables|Default|GetGameplayHUD)))
  (Default|TriggerDealtDamage _aswb_arena_hud))

(fn TriggerTookDamageUI
  (params (Damage :type Float%20%28single-precision%29))
  (bind _aswb_arena_hud (Utilities|Casting|CastToWB_ArenaHUD (Variables|Default|GetGameplayHUD)))
  (Default|TriggerTookDamage _aswb_arena_hud Damage))