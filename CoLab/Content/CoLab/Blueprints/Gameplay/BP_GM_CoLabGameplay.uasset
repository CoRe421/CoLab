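; Game mode for CoLab gameplay that tracks connected players and provides pawn spawning for them.
; Login, seamless controller swap and logout events add or remove CoLab gameplay player controllers in a Players list.
; SpawnPlayer destroys any current pawn, then spawns and possesses a BP_CoLabCharacter at a randomly chosen BP_CoLabPlayerStart.
; Nothing in this Blueprint calls SpawnPlayer itself.
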(event EventBeginPlay)

(event EventTick
  (params (DeltaSeconds :type Float%20%28single-precision%29)))

(event EventPostLogin
  (params (NewPlayer :type Player%20Controller%20Object%20Reference))
  ;[1 1 1] Player initial connect to session
  (CallFunction|RegisterPlayer NewPlayer))

(event EventOnSwapPlayerControllers
  (params (OldPC :type Player%20Controller%20Object%20Reference) (NewPC :type Player%20Controller%20Object%20Reference))
  ;[1 1 1] Player change PC during session (swap levels)
  (CallFunction|UnregisterPlayer OldPC)
  (CallFunction|RegisterPlayer NewPC))

(event EventOnLogout
  (params (ExitingController :type Controller%20Object%20Reference))
  ;[1 1 1] Player leaves session
  (bind _asplayer_controller (Utilities|Casting|CastToPlayerController ExitingController))
  (CallFunction|UnregisterPlayer _asplayer_controller))

(fn ConstructionScript)

(fn RegisterPlayer
  (params (Player :type Player%20Controller%20Object%20Reference))
  (bind _asbp_pc_co_lab_gameplay (Utilities|Casting|CastToBP_PC_CoLabGameplay Player))
  (Utilities|Array|Add (Variables|Default|GetPlayers) _asbp_pc_co_lab_gameplay))

(fn UnregisterPlayer
  (params (Player :type Player%20Controller%20Object%20Reference))
  (bind _asbp_pc_co_lab_gameplay (Utilities|Casting|CastToBP_PC_CoLabGameplay Player))
  (Utilities|Array|RemoveItem (Variables|Default|GetPlayers) _asbp_pc_co_lab_gameplay))

(fn FindRandomPlayerStart
  (bind _outactors (Actor|GetAllActorsOfClass "/Game/CoLab/Blueprints/Gameplay/Actors/BP_CoLabPlayerStart.BP_CoLabPlayerStart_C"))
  (return (Utilities|Array|Get(acopy) _outactors (Math|Random|RandomIntegerinRange 0 (- (Utilities|Array|Length _outactors) 1)))))

(fn SpawnPlayer
  (params (PlayerController :type BP%20PC%20Co%20Lab%20Gameplay%20Object%20Reference))
  (bind _output_get (LocalVariables|SetL_CurrentPawn (Pawn|GetControlledPawn PlayerController)))
  (Utilities|IsValid _output_get
    (:Is%20Valid
      (Actor|DestroyActor (LocalVariables|GetL_CurrentPawn))
      (LocalVariables|SetL_CurrentPawn 0))
    (:Is%20Not%20Valid
      _))
  (bind _playerstart (Spawning|FindRandomPlayerStart))
  (bind _pawnclass (CallFunction|GetPawnforPlayer PlayerController))
  (bind _playerpawn (Spawning|SpawnPlayerPawnatStart _playerstart _pawnclass))
  (Pawn|Possess PlayerController _playerpawn))

(fn GetDefaultPawnClassforController
  (params (InController :type Controller%20Object%20Reference))
  (bind _returnvalue (|CallParentFunction InController))
  (return _returnvalue))

(fn SpawnPlayerPawnatStart
  (params (PlayerStart :type BP%20Co%20Lab%20Player%20Start%20Object%20Reference) (PawnClass :type Pawn%20Class%20Reference))
  (bind _returnvalue (Game|SpawnActorfromClass PawnClass (Transformation|GetActorTransform PlayerStart) "Undefined" "MultiplyWithRoot" 0 0))
  (return _returnvalue))

(fn GetPawnforPlayer
  (params (PlayerController :type BP%20PC%20Co%20Lab%20Gameplay%20Object%20Reference))
  (return "/Game/CoLab/Blueprints/Gameplay/Characters/Player/BP_CoLabCharacter.BP_CoLabCharacter_C"))