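; Server-side manager for Arena point volumes that keeps a configured number active at random.
; On BeginPlay it pools assigned or level-found volumes that are not self-managed, using the PDA_SurfPointVolumes runtime config.
; When a player scores or an optional lifespan expires, it enables another random volume before releasing the old one, avoiding an immediate repeat.
; Config changes reset and re-roll the active set.
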(event Custom|OnConfigPropertyChanged
  (params (PropertyName :type Name))
  (CallFunction|RestartVolumes))

(event EventBeginPlay
  (bind _assignedpointvolumes (Variables|Default|GetAssignedPointVolumes))
  (bind _returnvalue (Utilities|Set|IsEmpty _assignedpointvolumes))
  ;[1 1 1] Only run on server
  (Networking|SwitchHasAuthority
    (:Authority
      (bind _returnvalue_2 (Class|CollabRuntimeConfigSubsystem|GetConfigData (Subsystems|GetCollabRuntimeConfigSubsystem) "/Game/CoLab/Modes/Arena/Blueprints/PointsVolume/PDA_SurfPointVolumes.PDA_SurfPointVolumes_C"))
      (Utilities|IsValid _returnvalue_2
        (:Is%20Valid
          (bind _output_get (Variables|Default|SetCachedVolumeConfig _returnvalue_2))
          (EventDispatchers|AssignOnConfigPropertyChanged _output_get (delegate Custom|OnConfigPropertyChanged))
          (if _returnvalue
            (bind _outactors (Actor|GetAllActorsOfClass "/Game/CoLab/Modes/Arena/Blueprints/PointsVolume/BP_PointsVolume.BP_PointsVolume_C"))
            (else
              (bind _result (Utilities|Set|ToArray _assignedpointvolumes))))
          (for _array_element (select _returnvalue _outactors _result)
            (if (not (Variables|/Game/CoLab/Modes/Arena/Blueprints/PointsVolume/BP_PointsVolume.BP_PointsVolume_C|GetbSelfManaged _array_element))
              (Default|SetVolumeEnabled _array_element false)
              (Utilities|Set|Add (Variables|Default|GetAvailablePointVolumes) _array_element)
              (Utilities|Set|Add (Variables|Default|GetAllPointVolumes) _array_element)))
          (CallFunction|RestartVolumes))))))

(event Collision|EventActorBeginOverlap
  (params (OtherActor :type Actor%20Object%20Reference)))

(event EventTick
  (params (DeltaSeconds :type Float%20%28single-precision%29)))

(fn ConstructionScript)

(fn SetVolumeEnabled
  (params (Volume :type BP%20Points%20Volume%20Object%20Reference) (bEnabled :type Boolean))
  (Utilities|IsValid Volume
    (:Is%20Valid
      (Default|SetVolumeEnabled Volume bEnabled)
      (if bEnabled
        (Utilities|Set|Remove (Variables|Default|GetAvailablePointVolumes) Volume)
        (EventDispatchers|BindEventtoOnPlayerScore Volume (EventDispatchers|CreateEvent :!event OnPlayerScored))
        (CallFunction|TryStartTimerforVolume Volume)
        (else
          (EventDispatchers|UnbindallEventsfromOnPlayerScore Volume)
          (EventDispatchers|UnbindallEventsfromOnLifetimeFinish Volume)
          (Utilities|Set|Add (Variables|Default|GetAvailablePointVolumes) Volume)
          (Default|DisableLifetime Volume))))))

(fn EndTimerforVolume
  (Utilities|Time|ClearandInvalidateTimerbyHandle (Variables|Default|GetPointVolumeTimer))
  (CallFunction|TryStartTimerforVolume))

(fn TryStartTimerforVolume
  (params (Volume :type BP%20Points%20Volume%20Object%20Reference))
  (if (> (Variables|/Game/CoLab/Modes/Arena/Blueprints/PointsVolume/PDA_SurfPointVolumes.PDA_SurfPointVolumes_C|GetActiveVolumeLifespan (Variables|Default|GetCachedVolumeConfig)) 0.0)
    (EventDispatchers|BindEventtoOnLifetimeFinish Volume (EventDispatchers|CreateEvent :!event OnVolumeTimerFinished))
    (Default|SetLifetime Volume (Variables|/Game/CoLab/Modes/Arena/Blueprints/PointsVolume/PDA_SurfPointVolumes.PDA_SurfPointVolumes_C|GetActiveVolumeLifespan (Variables|Default|GetCachedVolumeConfig)))))

(fn EnableRandomVolume
  (bind _availablepointvolumes (Variables|Default|GetAvailablePointVolumes))
  (if (Utilities|Set|IsNotEmpty _availablepointvolumes)
    (bind _result (Utilities|Set|ToArray _availablepointvolumes))
    (bind _output_get (LocalVariables|SetL_ChosenVolume (.OutItem (Utilities|Array|Random _result))))
    (CallFunction|SetVolumeEnabled _output_get true)))

(fn OnVolumeTimerFinished
  (params (Volume :type BP%20Player%20Volume%20Base%20Object%20Reference))
  (bind _asbp_points_volume (Utilities|Casting|CastToBP_PointsVolume Volume))
  (CallFunction|SwitchVolumes _asbp_points_volume))

(fn SwitchVolumes
  (params (OldVolume :type BP%20Points%20Volume%20Object%20Reference))
  (CallFunction|EnableRandomVolume)
  ;[1 1 1] Happens afterwards because don't want it to be part of available volume pool
  (CallFunction|SetVolumeEnabled OldVolume false))

(fn OnPlayerScored
  (params (Volume :type BP%20Points%20Volume%20Object%20Reference))
  (CallFunction|SwitchVolumes Volume))

(fn RestartVolumes
  (bind _cachedvolumeconfig (Variables|Default|GetCachedVolumeConfig))
  (bind _numactivevolumes (Variables|/Game/CoLab/Modes/Arena/Blueprints/PointsVolume/PDA_SurfPointVolumes.PDA_SurfPointVolumes_C|GetNumActiveVolumes _cachedvolumeconfig))
  (Utilities|FlowControl|Sequence
    (:then_0
      ;[1 1 1] This gets all active volumes
      (bind _result (Utilities|Set|Difference (Variables|Default|GetAllPointVolumes) (Variables|Default|GetAvailablePointVolumes)))
      (bind _result_2 (Utilities|Set|ToArray _result))
      (for _array_element _result_2
        (CallFunction|SetVolumeEnabled _array_element false)))
    (:then_1
      (if (> (Utilities|Set|Length (Variables|Default|GetAvailablePointVolumes)) _numactivevolumes)
        (for _index (range 1 _numactivevolumes)
          (CallFunction|EnableRandomVolume))))))