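; Base Arena scoring volume that awards the configured zone score through BP_GS_Arena when a player character overlaps its box, then broadcasts a score event.
; Starts disabled unless already enabled; the server toggles visibility and collision, and disabling clears the lifetime timer.
; An optional server-side lifetime timer pairs with a finish handler that notifies listeners without disabling the volume itself.
; The construction script tints the cube with a dynamic material using BoxColor.
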(event OnComponentBeginOverlap(Box)
  (params (OverlappedComponent :type Primitive%20Component%20Object%20Reference) (OtherActor :type Actor%20Object%20Reference) (OtherComp :type Primitive%20Component%20Object%20Reference) (OtherBodyIndex :type Integer) (bFromSweep :type Boolean) (SweepResult :type Hit%20Result%20Structure%20%28by%20ref%29))
  (bind _cachedgamestate (Variables|Default|GetCachedGameState))
  (bind _cachedarenaconfig (Variables|Default|GetCachedArenaConfig))
  (bind _ascollab_player_character (Utilities|Casting|CastToCollabPlayerCharacter OtherActor))
  (if (Math|Boolean|ANDBoolean (Utilities|IsValid _cachedgamestate) (Utilities|IsValid (Variables|/Script/Engine.Pawn|GetPlayerState _ascollab_player_character)) (Utilities|IsValid _cachedarenaconfig))
    (Default|AddPlayerScore _cachedgamestate (PlayerState|GetUniqueID (Variables|/Script/Engine.Pawn|GetPlayerState _ascollab_player_character)) (Variables|/Game/CoLab/Blueprints/Arena/GameFramework/Config/PDA_ArenaConfig.PDA_ArenaConfig_C|GetPlayerZoneScoreValue _cachedarenaconfig))
    (Default|CallOnPlayerScore self)))

(event EventBeginPlay
  (Utilities|FlowControl|Sequence
    (:then_0
      (bind _asbp_gs_arena (Utilities|Casting|CastToBP_GS_Arena (Game|GetGameState))
        (:then
          (Variables|Default|SetCachedGameState _asbp_gs_arena))
        (:CastFailed
          _))
      (bind _returnvalue (Class|CollabRuntimeConfigSubsystem|GetConfigData (Subsystems|GetCollabRuntimeConfigSubsystem) "/Game/CoLab/Blueprints/Arena/GameFramework/Config/PDA_ArenaConfig.PDA_ArenaConfig_C"))
      (Variables|Default|SetCachedArenaConfig _returnvalue))
    (:then_1
      ;[1 1 1] Prevents from self-disabling if has already been enabled
      (if (not (Variables|Default|GetbSetEnabled))
        (CallFunction|SetVolumeEnabled false)))))

(event Collision|EventActorBeginOverlap
  (params (OtherActor :type Actor%20Object%20Reference)))

(event EventTick
  (params (DeltaSeconds :type Float%20%28single-precision%29)))

(fn ConstructionScript
  (bind _returnvalue (Rendering|Material|CreateDynamicMaterialInstance "/Game/CoLab/Blueprints/Arena/Assets/M_TransparentColor.M_TransparentColor" "None" "None" :!class /Script/Engine.KismetMaterialLibrary))
  (Rendering|Material|SetVectorParameterValue _returnvalue "Color" (Variables|Default|GetBoxColor) :!class /Script/Engine.MaterialInstanceDynamic)
  (Rendering|Material|SetMaterial (Variables|Default|GetCube) 0 _returnvalue))

(fn SetVolumeEnabled
  (params (bEnabled :type Boolean))
  (Variables|Default|SetbSetEnabled bEnabled)
  ;[1 1 1] Only change on server
  (Networking|SwitchHasAuthority
    (:Authority
      (Rendering|SetActorHiddenInGame self (not (Variables|Default|GetbSetEnabled)))
      (Collision|SetCollisionEnabled (Variables|Default|GetBox) (select (Variables|Default|GetbSetEnabled) "QueryAndPhysics" "NoCollision"))
      (if (not (Variables|Default|GetbSetEnabled))
        (CallFunction|DisableLifetime)))))

(fn SetLifetime
  (params (Lifetime :type Float%20%28double-precision%29))
  ;[1 1 1] Only set lifetime on server
  (Networking|SwitchHasAuthority
    (:Authority
      (if (and (> Lifetime 0.0) (not (Utilities|Time|IsValidTimerHandle (Variables|Default|GetActiveLifetimeTimer))))
        (bind _returnvalue (Utilities|Time|SetTimerbyEvent (EventDispatchers|CreateEvent :!event OnLifetimeFinished) Lifetime))
        (Variables|Default|SetActiveLifetimeTimer _returnvalue)))))

(fn OnLifetimeFinished
  (CallFunction|DisableLifetime)
  (Default|CallOnLifetimeFinish self))

(fn DisableLifetime
  (Utilities|Time|ClearandInvalidateTimerbyHandle (Variables|Default|GetActiveLifetimeTimer)))