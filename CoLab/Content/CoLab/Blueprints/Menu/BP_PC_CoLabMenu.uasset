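; Player controller for the CoLab menu that sets up the menu UI and mouse input for the local player.
; On BeginPlay it creates the layout widget through the collab layout interface, if none exists yet, and adds it to the viewport.
; It then pushes the menu widget onto the layout's menu layer and keeps it as the session menu.
; The cursor is shown and input is locked to UI only.
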(event Custom|InitMenuUI
  (CallFunction|TryInitLayout)
  (bind _widget (Default|PushWidgettoLayerStack (Variables|Default|GetLayout) "(TagName=\"UI.Layer.Menu\")" (Variables|Default|GetMenuWidget)))
  (Variables|Default|SetSessionMenu _widget))

(event Custom|TryInitLayout
  (if (not (Utilities|IsValidInterface (Variables|Default|GetLayout)))
    (bind _returnvalue (UserInterface|CreateWidget (Variables|Default|GetLayoutWidgetClass) self))
    (bind _asbpi_collab_layout (Utilities|Casting|CastToBPI_CollabLayout _returnvalue))
    (Variables|Default|SetLayout _asbpi_collab_layout)
    (UserInterface|Viewport|AddtoViewport _returnvalue 0)))

(event EventBeginPlay
  (if (Pawn|IsLocalController)
    (CallFunction|InitMenuUI)
    (Variables|/Script/Engine.PlayerController|SetbShowMouseCursor self true)
    (Input|SetInputModeUIOnly self 0 "LockAlways" false)))

(event EventTick
  (params (DeltaSeconds :type Float%20%28single-precision%29)))

(fn ConstructionScript)