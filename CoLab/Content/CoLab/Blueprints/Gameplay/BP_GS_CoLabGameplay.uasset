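; Game state for CoLab gameplay that keeps player list widgets in sync with the connected players.
; On BeginPlay the server binds to the CoLab game mode's player-list update event to copy PlayerArray into RepPlayerArray.
; The RepNotify on that array finds every WB_PlayerList widget and passes it the replicated list.
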(event EventBeginPlay
  (if (Networking|IsServer)
    (bind _asbp_gm_co_lab_gameplay (Utilities|Casting|CastToBP_GM_CoLabGameplay (Game|GetGameMode)))
    (EventDispatchers|BindEventtoOnPlayerListUpdated _asbp_gm_co_lab_gameplay (EventDispatchers|CreateEvent :!event OnPlayersUpdated))))

(event EventTick
  (params (DeltaSeconds :type Float%20%28single-precision%29)))

(fn ConstructionScript)

(fn OnPlayersUpdated
  (Variables|Default|SetRepPlayerArray (Variables|Default|GetPlayerArray)))

(fn OnRepRepPlayerArray
  (bind _foundwidgets (Widget|GetAllWidgetsOfClass "/Game/CoLab/Blueprints/Gameplay/UI/WB_PlayerList.WB_PlayerList_C" false))
  (for _array_element _foundwidgets
    (Default|SetPlayers _array_element (Variables|Default|GetRepPlayerArray))))