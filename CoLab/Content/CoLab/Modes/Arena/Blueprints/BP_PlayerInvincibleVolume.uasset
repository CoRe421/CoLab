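; Arena-mode volume that makes players invincible while they are inside it by granting a loose, non-replicated invincibility gameplay tag.
; It overrides the parent's player enter and leave hooks to add and remove the tag.
; If the player's Ability System Component is not ready on entry, it waits for the init event, then resolves the character from the ASC owner, directly or via PlayerState, and re-runs entry.
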(event EventBeginPlay
  (|CallParentFunction) ; This node is disabled and will not be called.\nDrag off pins to build functionality.
)

(event Collision|EventActorBeginOverlap
  (params (OtherActor :type Actor%20Object%20Reference))
  (|CallParentFunction OtherActor) ; This node is disabled and will not be called.\nDrag off pins to build functionality.
)

(event EventTick
  (params (DeltaSeconds :type Float%20%28single-precision%29))
  (|CallParentFunction DeltaSeconds) ; This node is disabled and will not be called.\nDrag off pins to build functionality.
)

(fn ConstructionScript
  (|CallParentFunction))

(fn OnNewPlayerEnter
  (params (Player :type Collab%20Player%20Character%20Object%20Reference))
  (|CallParentFunction Player)
  (bind _output_get (LocalVariables|SetL_FoundASC (Ability|GetAbilitySystemComponent Player)))
  (Utilities|IsValid _output_get
    (:Is%20Valid
      (bind _returnvalue (Ability|GameplayEffect|AddLooseGameplayTags Player (GameplayTags|MakeGameplayTagContainerfromTag (Variables|Default|GetInvincibleTag))))
      (Development|PrintString (Utilities|String|ToString(Boolean) _returnvalue)))
    (:Is%20Not%20Valid
      (EventDispatchers|BindEventtoOnAbilitySystemInit Player (EventDispatchers|CreateEvent :!event OnOverlappingPlayerASCInit)))))

(fn OnPlayerLeave
  (params (Player :type Collab%20Player%20Character%20Object%20Reference))
  (|CallParentFunction Player)
  (EventDispatchers|UnbindallEventsfromOnAbilitySystemInit Player)
  (Ability|GameplayEffect|RemoveLooseGameplayTags Player (GameplayTags|MakeGameplayTagContainerfromTag (Variables|Default|GetInvincibleTag))))

(fn OnOverlappingPlayerASCInit
  (params (ASC :type Collab%20Ability%20System%20Component%20Object%20Reference))
  (Utilities|FlowControl|Sequence
    (:then_0
      (LocalVariables|SetL_TargetActor (Components|GetOwner ASC)))
    (:then_1
      (bind _asplayer_state (Utilities|Casting|CastToPlayerState (LocalVariables|GetL_TargetActor)))
      (Utilities|IsValid (Game|GetPlayerController _asplayer_state)
        (:Is%20Valid
          (LocalVariables|SetL_TargetActor (Pawn|GetControlledPawn (Game|GetPlayerController _asplayer_state)))))))
  (bind _ascollab_player_character (Utilities|Casting|CastToCollabPlayerCharacter (LocalVariables|GetL_TargetActor)))
  (EventDispatchers|UnbindallEventsfromOnAbilitySystemInit _ascollab_player_character)
  (CallFunction|OnNewPlayerEnter _ascollab_player_character)
  (return))