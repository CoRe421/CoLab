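; Arena speed volume that boosts players inside it along their current direction of travel.
; On entry and on a looping timer, it adds a velocity-change impulse from normalized velocity, masked by SpeedAxes and scaled by SpeedForceStrength.
; Each player gets a 2D loop sound at a random start time, removed on exit; the arena config's Italian flag swaps sound and pitch.
; The construction script fits Niagara effect size and spawn rate to the box.
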(event EventBeginPlay
  (|CallParentFunction)
  (bind _returnvalue (Utilities|Time|SetTimerbyEvent (EventDispatchers|CreateEvent :!event SpeedTick) (Variables|Default|GetSpeedTickRate) true))
  (Variables|Default|SetSpeedTickHandle _returnvalue)
  (Class|NiagaraComponent|SetSystemFixedBounds (Variables|Default|GetNiagara) (Class|KismetMathLibrary|MakeBoxwithOrigin (Math|Vector|VectorZero) (Components|Box|GetScaledBoxExtent (Variables|Default|GetBox))))
  (bind _returnvalue_2 (Class|CollabRuntimeConfigSubsystem|GetConfigData (Subsystems|GetCollabRuntimeConfigSubsystem) "/Game/CoLab/Modes/Arena/GameFramework/Config/PDA_ArenaConfig.PDA_ArenaConfig_C"))
  (Variables|Default|SetCachedArenaConfig _returnvalue_2))

(event Collision|EventActorBeginOverlap
  (params (OtherActor :type Actor%20Object%20Reference))
  (|CallParentFunction OtherActor) ; This node is disabled and will not be called.\nDrag off pins to build functionality.
)

(event EventTick
  (params (DeltaSeconds :type Float%20%28single-precision%29))
  (|CallParentFunction DeltaSeconds))

(fn ConstructionScript
  (bind _niagara (Variables|Default|GetNiagara))
  (bind _box (Variables|Default|GetBox))
  (bind _returnvalue (Components|Box|GetScaledBoxExtent _box))
  (|CallParentFunction)
  (Effects|Components|ParticleSystem|SetVectorParameter _niagara "BoxSize" _returnvalue)
  (Effects|Components|ParticleSystem|SetFloatParameter _niagara "SpawnRate" (+ 3.0 (/ (Class|KismetMathLibrary|GetBoxVolume (Class|KismetMathLibrary|MakeBoxwithOrigin (.Origin (Collision|GetComponentBounds 0)) _returnvalue)) 1e+08)))
  (Class|NiagaraComponent|SetSystemFixedBounds _niagara (Class|KismetMathLibrary|MakeBoxwithOrigin (Math|Vector|VectorZero) _returnvalue)))

(fn OnNewPlayerEnter
  (params (Player :type Collab%20Player%20Character%20Object%20Reference))
  (bind _cachedarenaconfig (Variables|Default|GetCachedArenaConfig))
  (bind _speedsound (Variables|Default|GetSpeedSound))
  (bind _returnvalue (Utilities|IsValid _cachedarenaconfig))
  (bind _bitalian (Variables|/Game/CoLab/Modes/Arena/GameFramework/Config/PDA_ArenaConfig.PDA_ArenaConfig_C|GetbItalian _cachedarenaconfig))
  (bind _returnvalue_2 (and _returnvalue _bitalian))
  (bind _returnvalue_3 (select _returnvalue_2 "/Game/CoLab/Modes/Arena/Assets/Sounds/Mario/mlrpg3_luigi_gibberish_6_Loop.mlrpg3_luigi_gibberish_6_Loop" _speedsound))
  (|CallParentFunction Player)
  (bind _returnvalue_4 (Audio|CreateSound2D _returnvalue_3 (Variables|Default|GetSpeedSoundVolume) (Math|Float|SelectFloat 1.0 1.5 _returnvalue_2) (Math|Random|RandomFloatinRange 0.0 (Variables|/Script/Engine.SoundBase|GetDuration _returnvalue_3)) "/Game/CoLab/Modes/Arena/Blueprints/SpeedVolume/C_SpeedVolume.C_SpeedVolume" false false))
  (Class|AudioComponent|SetUISound _returnvalue_4 true)
  (Audio|Components|Audio|Play _returnvalue_4 0.0)
  (Utilities|Map|Add (Variables|Default|GetPlayerSpeedSounds) Player _returnvalue_4)
  (CallFunction|ApplyBoosttoPlayer Player))

(fn OnPlayerLeave
  (params (Player :type Collab%20Player%20Character%20Object%20Reference))
  (|CallParentFunction Player)
  (bind _output_get (LocalVariables|SetL_FoundSpeedSound (.Value (Utilities|Map|Find (Variables|Default|GetPlayerSpeedSounds) Player))))
  (Utilities|IsValid _output_get
    (:Is%20Valid
      (Audio|Components|Audio|Stop _output_get)
      (Components|DestroyComponent _output_get)
      (Utilities|Map|Remove (Variables|Default|GetPlayerSpeedSounds) Player))))

(fn GetMovementComponent
  (params (Player :type Pawn%20Object%20Reference))
  (bind _ascollab_movement_component (Utilities|Casting|CastToCollabMovementComponent (Pawn|GetMovementComponent Player))
    (:then
      _)
    (:CastFailed
      _))
  (return _ascollab_movement_component))

(fn ApplyBoosttoPlayer
  (params (Player :type Collab%20Player%20Character%20Object%20Reference))
  (bind _movementcomponent (CallFunction|GetMovementComponent Player))
  (bind _output_get (LocalVariables|SetL_MovementComponent _movementcomponent))
  (Utilities|IsValid _output_get
    (:Is%20Valid
      (Physics|AddImpulse _output_get (* (* (Variables|Default|GetSpeedAxes) (Math|Vector|Normalize (Variables|/Script/Engine.MovementComponent|GetVelocity _output_get))) (Variables|Default|GetSpeedForceStrength)) true))))

(fn SpeedTick
  (bind _result (Utilities|Set|ToArray (Variables|Default|GetOverlappedPlayers)))
  (for _array_element _result
    (CallFunction|ApplyBoosttoPlayer _array_element)))