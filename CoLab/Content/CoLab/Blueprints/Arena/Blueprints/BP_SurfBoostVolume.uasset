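; Arena trigger volume that grants a surf boost Gameplay Effect to player characters while they are inside it.
; Box begin and end overlaps apply and remove the effect on the Ability System Component found through the player's PlayerState.
; A helper macro tracks overlapped players, so only real enter or exit changes trigger either action.
; The construction script tints the Cube with a configurable color through a dynamic transparent material.
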(event OnComponentBeginOverlap(Box)
  (params (OverlappedComponent :type Primitive%20Component%20Object%20Reference) (OtherActor :type Actor%20Object%20Reference) (OtherComp :type Primitive%20Component%20Object%20Reference) (OtherBodyIndex :type Integer) (bFromSweep :type Boolean) (SweepResult :type Hit%20Result%20Structure%20%28by%20ref%29))
  (bind _ascollab_player_character (Utilities|Casting|CastToCollabPlayerCharacter OtherActor))
  (Utilities|CheckorAddOverlappingPlayer _ascollab_player_character true
    (:Overlapping
      (bind _output_get (Variables|Default|SetTargetComponent (Class|CollabAbilitySystemComponent|FindAbilitySystemComponent (Variables|/Script/Engine.Pawn|GetPlayerState _ascollab_player_character))))
      (Utilities|IsValid _output_get
        (:Is%20Valid
          (GameplayEffects|ApplyGameplayEffectToSelf :self _output_get :GameplayEffectClass (Variables|Default|GetSurgBoostEffect)))))))

(event OnComponentEndOverlap(Box)
  (params (OverlappedComponent :type Primitive%20Component%20Object%20Reference) (OtherActor :type Actor%20Object%20Reference) (OtherComp :type Primitive%20Component%20Object%20Reference) (OtherBodyIndex :type Integer))
  (bind _ascollab_player_character (Utilities|Casting|CastToCollabPlayerCharacter OtherActor))
  (Utilities|CheckorAddOverlappingPlayer _ascollab_player_character false
    (:Overlapping
      (bind _output_get (Variables|Default|SetTargetComponent (Class|CollabAbilitySystemComponent|FindAbilitySystemComponent (Variables|/Script/Engine.Pawn|GetPlayerState _ascollab_player_character))))
      (Utilities|IsValid _output_get
        (:Is%20Valid
          (GameplayEffects|RemoveActiveGameplayEffectbySourceEffect _output_get (Variables|Default|GetSurgBoostEffect) 0 -1))))))

(event EventBeginPlay)

(event Collision|EventActorBeginOverlap
  (params (OtherActor :type Actor%20Object%20Reference)))

(event EventTick
  (params (DeltaSeconds :type Float%20%28single-precision%29)))

(fn ConstructionScript
  (bind _returnvalue (Rendering|Material|CreateDynamicMaterialInstance "/Game/CoLab/Blueprints/Arena/Assets/M_TransparentColor.M_TransparentColor" "None" "None" :!class /Script/Engine.KismetMaterialLibrary))
  (Rendering|Material|SetVectorParameterValue _returnvalue "Color" (Variables|Default|GetBoxColor) :!class /Script/Engine.MaterialInstanceDynamic)
  (Rendering|Material|SetMaterial (Variables|Default|GetCube) 0 _returnvalue))