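; Arena Spleef trigger volume that removes listed actor classes or static meshes entering its box.
; An overlapping actor of a listed class is destroyed; otherwise the overlapped component and its children are searched for a listed mesh.
; The first match is destroyed through the Collab replicated component interface, or otherwise hidden with physics, collision and tick disabled, since another actor's component cannot be destroyed directly.
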(event OnComponentBeginOverlap(Box)
  (params (OverlappedComponent :type Primitive%20Component%20Object%20Reference) (OtherActor :type Actor%20Object%20Reference) (OtherComp :type Primitive%20Component%20Object%20Reference) (OtherBodyIndex :type Integer) (bFromSweep :type Boolean) (SweepResult :type Hit%20Result%20Structure%20%28by%20ref%29))
  (bind _bdestroyed (CallFunction|TryDestroyOverlappedActor OtherActor))
  (if (not _bdestroyed)
    (CallFunction|TryDestroyOverlappedComponent OtherComp)))

(event EventBeginPlay)

(event Collision|EventActorBeginOverlap
  (params (OtherActor :type Actor%20Object%20Reference)))

(event EventTick
  (params (DeltaSeconds :type Float%20%28single-precision%29)))

(fn ConstructionScript)

(fn TryDestroyOverlappedActor
  (params (OverlappedActor :type Actor%20Object%20Reference))
  (for _array_element (Variables|Default|GetDestroyActorClasses)
    (if (Class|GameplayStatics|ObjectIsA OverlappedActor _array_element)
      (Actor|DestroyActor OverlappedActor)
      (return true)))
  (return false))

(fn TryDestroyOverlappedComponent
  (params (OverlappedComponent :type Scene%20Component%20Object%20Reference))
  (bind _output_get (LocalVariables|SetL_ChildrenComponents (Components|GetChildrenComponents OverlappedComponent true)))
  (Utilities|Array|Add _output_get OverlappedComponent)
  (for _array_element _output_get
    (Utilities|IsValid _array_element
      (:Is%20Valid
        (bind _asstatic_mesh_component (Utilities|Casting|CastToStaticMeshComponent _array_element))
        (bind _output_get_2 (LocalVariables|SetL_Component _asstatic_mesh_component))
        (if (Utilities|Set|Contains (Variables|Default|GetDestroyMeshObjects) (Variables|/Script/Engine.StaticMeshComponent|GetStaticMesh _output_get_2))
          (bind _ascollab_replicated_component_interface (Utilities|Casting|CastToCollabReplicatedComponentInterface _output_get_2)
            (:then
              (Class|CollabReplicatedComponentInterface|DestroyComponent _ascollab_replicated_component_interface))
            (:CastFailed
              ;[1 1 1] Can't destroy another actor's component so essentially try to remove it from the game or any calculations
              (Development|SetHiddeninGame (LocalVariables|GetL_Component) true true)
              (Physics|SetSimulatePhysics (LocalVariables|GetL_Component) false)
              (Collision|SetCollisionEnabled (LocalVariables|GetL_Component) "NoCollision")
              (Components|Tick|SetComponentTickEnabled (LocalVariables|GetL_Component) false)))
          (return true)))))
  (return false))