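; Player character Blueprint for CoLab, with health and mana widget updates, death notification, weapon firing and a CapsLock reverse-camera toggle.
; Health and mana handlers push values into the attribute widget component, and death reaches the locally controlled gameplay PlayerController through a client event.
; TryFire passes weapon-interface components to a server fire event with an empty body.
; Ability attribute binding and startup initialization logic is disconnected, leaving only the parent binding call.
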(event Custom|SR_FireWeapon
  (params (Weapon :type Co%20Lab%20Weapon%20Interface%20Interface)))

(event Custom|CL_ControllerPlayerDeath
  ;[1 1 1] Will only fire on local client with a valid PlayerController
  (if (Pawn|IsLocallyControlled)
    (bind _asbp_pc_co_lab_gameplay (Utilities|Casting|CastToBP_PC_CoLabGameplay (Pawn|GetController)))
    (Default|OnPlayerDeath _asbp_pc_co_lab_gameplay)))

(event EventBeginPlay
  (Utilities|FlowControl|Sequence))

(event EventOnDestroyCharacter
  (CallFunction|OnCharacterDeath))

(event Input|KeyboardEvents|Q
  (params (Key :type Key%20Structure :default "None")))

(event Input|KeyboardEvents|F5
  (params (Key :type Key%20Structure :default "None")))

(event Input|KeyboardEvents|CapsLock
  (params (Key :type Key%20Structure :default "None"))
  (:Pressed
    (Utilities|FlowControl|FlipFlop
      (:A
        (Components|Activation|SetActive (Variables|Default|GetReverseCamera) true false)
        (Components|Activation|SetActive (Variables|Default|GetFirstPersonCameraComponent) false false))
      (:B
        (Components|Activation|SetActive (Variables|Default|GetFirstPersonCameraComponent) true false)
        (Components|Activation|SetActive (Variables|Default|GetReverseCamera) false false)))))

(fn ConstructionScript)

(fn TryFire
  (params (Value :type Input%20Action%20Value%20Structure%20%28by%20ref%29))
  (bind _output_get (LocalVariables|SetL_WeaponComponents (Class|Actor|GetComponentsbyInterface "/Script/CoLab.CoLabWeaponInterface")))
  (for _array_element _output_get
    (bind _asco_lab_weapon_interface (Utilities|Casting|CastToCoLabWeaponInterface _array_element))
    (CallFunction|SRFireWeapon _asco_lab_weapon_interface)))

(fn OnHealthChanged
  (params (NewHealth :type Float%20%28single-precision%29) (MaxHealth :type Float%20%28single-precision%29))
  (bind _aswb_character_attributes (Utilities|Casting|CastToWB_CharacterAttributes (UserInterface|GetWidget (Variables|Default|GetAttributeWidgetComponent))))
  (Default|SetHealth _aswb_character_attributes NewHealth MaxHealth))

(fn SetupAbilitySystemComponentBindings
  (|CallParentFunction))

(fn InitializeStartupValues
  ;[1 1 1] Runs startup value logic, ASC must be initialized and actor must be fully constructed for widget component to be created - CR
)

(fn OnManaChanged
  (params (NewMana :type Float%20%28single-precision%29) (OldMana :type Float%20%28single-precision%29))
  (bind _aswb_character_attributes (Utilities|Casting|CastToWB_CharacterAttributes (UserInterface|GetWidget (Variables|Default|GetAttributeWidgetComponent))))
  (Default|SetMana _aswb_character_attributes NewMana OldMana))

(fn InitOverlay
  (bind _returnvalue (UserInterface|CreateWidget "/Game/CoLab/Blueprints/Gameplay/UI/WB_CharacterAttributes.WB_CharacterAttributes_C"))
  (bind _output_get (Variables|Default|SetAttributeWidget _returnvalue))
  (UserInterface|SetWidget (Variables|Default|GetAttributeWidgetComponent) _output_get)
  (if (Pawn|IsLocallyControlled)
    _))

(fn InitializeCharacter)

(fn OnCharacterDeath
  (Utilities|FlowControl|Sequence
    (:then_0
      (CallFunction|CLControllerPlayerDeath))))