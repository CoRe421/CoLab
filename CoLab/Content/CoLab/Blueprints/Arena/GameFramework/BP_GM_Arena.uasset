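; Game mode for the Arena that detects when a player reaches the winning score and restarts the game.
; On BeginPlay it blocking-loads a ruleset data asset if none is valid, then binds to the Arena game state's score update event.
; A score check against the ruleset's threshold triggers the win, which prints the winner, calls the game state's win handler and restarts after a short delay.
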(event Custom|TriggerPlayerWin
  (params (Player :type Unique%20Net%20Id%20Repl%20Structure))
  (Development|PrintString (Utilities|String|Append "Player " (Utilities|String|ToString(Integer) (Variables|/Script/Engine.PlayerState|GetPlayerId (Game|GetPlayerStatefromUniqueNetId Player))) " wins!"))
  (Default|MULHandlePlayerWin (Variables|Default|GetCachedGameState) Player)
  (Utilities|FlowControl|Delay 5.0)
  (Class|GameMode|RestartGame))

(event EventBeginPlay
  (|CallParentFunction)
  (CallFunction|InitializeArenaRuleset)
  (bind _asbp_gs_arena (Utilities|Casting|CastToBP_GS_Arena (Game|GetGameState)))
  ;[1 0.1354 0.1354] Check if this works with player states
  (bind _output_get (Variables|Default|SetCachedGameState _asbp_gs_arena))
  (EventDispatchers|BindEventtoOnPlayerScoreUpdated _output_get (EventDispatchers|CreateEvent :!event CheckforPlayerWin)))

(event EventTick
  (params (DeltaSeconds :type Float%20%28single-precision%29))
  (|CallParentFunction DeltaSeconds) ; This node is disabled and will not be called.\nDrag off pins to build functionality.
)

(fn ConstructionScript
  (|CallParentFunction))

(fn CheckforPlayerWin
  (params (Player :type Integer%20%28by%20ref%29) (PlayerScore :type Integer%20%28by%20ref%29))
  (if (>= PlayerScore (Default|GetPlayerWinScoreThreshold (Variables|Default|GetArenaRuleset)))
    (CallFunction|TriggerPlayerWin)
    (return)))

(fn InitializeArenaRuleset
  (Variables|Default|GetArenaRuleset
    (:then)
    (:else
      (bind _returnvalue (Utilities|LoadAssetBlocking (LocalVariables|GetL_RulesetObject)))
      (bind _aspda_arena_ruleset (Utilities|Casting|CastToPDA_ArenaRuleset _returnvalue))
      (Variables|Default|SetArenaRuleset _aspda_arena_ruleset))))

(fn GetArenaRuleset
  (return (Variables|Default|GetArenaRuleset)))