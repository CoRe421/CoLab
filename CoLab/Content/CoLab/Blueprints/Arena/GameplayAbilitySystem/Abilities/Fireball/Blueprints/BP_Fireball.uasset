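; Fireball projectile actor for a Gameplay Ability System ability, reporting its outcome to its owner through gameplay events.
; A mesh hit on anything but the owner spawns an explosion and destroys the actor on both authority and remote.
; On authority, a hit first sends the hit event with target and impact location.
; If it is destroyed without hitting, authority sends a despawn event instead, tracked by the Triggered flag.
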(event OnComponentHit(StaticMesh)
  (params (HitComponent :type Primitive%20Component%20Object%20Reference) (OtherActor :type Actor%20Object%20Reference) (OtherComp :type Primitive%20Component%20Object%20Reference) (NormalImpulse :type Vector :default "0, 0, 0") (Hit :type Hit%20Result%20Structure%20%28by%20ref%29))
  (bind _location (Collision|BreakHitResult Hit))
  (bind _returnvalue (Math|Transform|MakeTransform _location))
  (bind _gameplayabilitytargetinglocationinfo (Utilities|Struct|MakeGameplayAbilityTargetingLocationInfo "LiteralTransform" _returnvalue))
  (if (!= OtherActor (Components|GetOwner))
    (Effects|SpawnEmitteratLocation "/Game/StarterContent/Particles/P_Explosion.P_Explosion" (Transformation|GetActorLocation) "0, 0, 0" "2.000000,2.000000,2.000000")
    (Networking|SwitchHasAuthority
      (:Authority
        (Variables|Default|SetbTriggered true)
        (Ability|SendGameplayEventtoActor (Components|GetOwner) "(TagName=\"Gameplay.Event.Hit.Fireball\")" (Utilities|Struct|MakeGameplayEventData "(TagName=\"\")" self OtherActor 0 0 "()" "(GameplayTags=)" "(GameplayTags=)" 0.0 (Class|AbilitySystemBlueprintLibrary|AbilityTargetDatafromLocations _gameplayabilitytargetinglocationinfo _gameplayabilitytargetinglocationinfo)))
        (Actor|DestroyActor))
      (:Remote
        (Actor|DestroyActor)))))

(event EventBeginPlay)

(event Collision|EventActorBeginOverlap
  (params (OtherActor :type Actor%20Object%20Reference)))

(event EventTick
  (params (DeltaSeconds :type Float%20%28single-precision%29)))

(event EventDestroyed
  (Networking|SwitchHasAuthority
    (:Authority
      (if (not (Variables|Default|GetbTriggered))
        (Ability|SendGameplayEventtoActor (Components|GetOwner) "(TagName=\"Gameplay.Event.Despawn.Fireball\")" (Utilities|Struct|MakeGameplayEventData "(TagName=\"\")" self))))))

(fn ConstructionScript)