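; Surf Race block port actor, a directional marker made of a sphere and an arrow.
; The construction script calls ResetActorSize to apply the sphere's world scale and the arrow's size, dividing arrow length by arrow size to offset its scaling.
; FlipDirection negates the actor's current rotator, which is not a general 180-degree turn.
; The event graph holds no active logic.
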(event EventBeginPlay)

(event Collision|EventActorBeginOverlap
  (params (OtherActor :type Actor%20Object%20Reference)))

(event EventTick
  (params (DeltaSeconds :type Float%20%28single-precision%29)))

(fn ConstructionScript
  (CallFunction|ResetActorSize))

(fn ResetActorSize
  (bind _arrow (Variables|Default|GetArrow))
  (Transformation|SetWorldScale3D (Variables|Default|GetSphere) (Variables|Default|GetSphereScale))
  (Variables|/Script/Engine.ArrowComponent|SetArrowSize _arrow (Variables|Default|GetArrowSize))
  (Variables|/Script/Engine.ArrowComponent|SetArrowLength _arrow (/ (Variables|Default|GetArrowLength) (Variables|Default|GetArrowSize))))

(fn FlipDirection
  (Transformation|SetActorRotation (Class|KismetMathLibrary|NegateRotator (Transformation|GetActorRotation))))