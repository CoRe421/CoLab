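; Gameplay HUD Blueprint marked as not to be used, with a note that its logic lives in the player controller.
; Its events do nothing, but it still exposes functions to push and remove widgets on tag-identified layer stacks.
; Both forward to a WB_GameplayLayout overlay, which TryCreateOverlay lazily creates for player controller 0, adds to the viewport and caches.
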(event EventBeginPlay
  ;[1 1 1] DONT USE HUD - Logic is in player controller
)

(event Collision|EventActorBeginOverlap
  (params (OtherActor :type Actor%20Object%20Reference)))

(event EventTick
  (params (DeltaSeconds :type Float%20%28single-precision%29)))

(fn ConstructionScript)

(fn PushWidgettoLayerStack
  (params (LayerTag :type Gameplay%20Tag%20Structure) (WidgetClass :type Common%20Activatable%20Widget%20Class%20Reference))
  (bind _overlay (CallFunction|TryCreateOverlay))
  (bind _widget (Default|PushWidgettoLayerStack _overlay LayerTag WidgetClass))
  (return _widget))

(fn RemoveWidgetfromLayerStack
  (params (LayerTag :type Gameplay%20Tag%20Structure) (Widget :type Common%20Activatable%20Widget%20Object%20Reference))
  (bind _overlay (CallFunction|TryCreateOverlay))
  (Default|RemoveWidgetfromLayerStack _overlay LayerTag Widget))

(fn TryCreateOverlay
  (Variables|Default|GetGameplayOverlay
    (:then
      _)
    (:else
      (bind _returnvalue (UserInterface|CreateWidget "/Game/CoLab/Modes/Gameplay/UI/WB_GameplayLayout.WB_GameplayLayout_C" (Game|GetPlayerController 0)))
      (bind _output_get (Variables|Default|SetGameplayOverlay _returnvalue))
      (UserInterface|Viewport|AddtoViewport _output_get 0)))
  (return (Variables|Default|GetGameplayOverlay)))