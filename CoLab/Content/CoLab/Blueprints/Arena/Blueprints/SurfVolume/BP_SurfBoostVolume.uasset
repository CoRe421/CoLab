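; Arena surf boost volume that applies a gameplay effect to players inside its box and removes it when they leave.
; Overlap events track players in a list to ignore duplicate enters and exits, then use the PlayerState's ability system component.
; The construction script tints the preview cube via a dynamic material and fits Niagara particles to the box, scaling spawn rate with volume.
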(event OnComponentBeginOverlap(Box)
  (params (OverlappedComponent :type Primitive%20Component%20Object%20Reference) (OtherActor :type Actor%20Object%20Reference) (OtherComp :type Primitive%20Component%20Object%20Reference) (OtherBodyIndex :type Integer) (bFromSweep :type Boolean) (SweepResult :type Hit%20Result%20Structure%20%28by%20ref%29))
  (bind _ascollab_player_character (Utilities|Casting|CastToCollabPlayerCharacter OtherActor))
  (Utilities|CheckorAddOverlappingPlayer _ascollab_player_character true
    (:Overlapping
      (bind _output_get (Variables|Default|SetTargetComponent (Class|CollabAbilitySystemComponent|FindAbilitySystemComponent (Variables|/Script/Engine.Pawn|GetPlayerState _ascollab_player_character))))
      (Utilities|IsValid _output_get
        (:Is%20Valid
          (GameplayEffects|ApplyGameplayEffectToSelf :self _output_get :GameplayEffectClass (Variables|Default|GetSurgBoostEffect)))))))

(event OnComponentEndOverlap(Box)
  (params (OverlappedComponent :type Primitive%20Component%20Object%20Reference) (OtherActor :type Actor%20Object%20Reference) (OtherComp :type Primitive%20Component%20Object%20Reference) (OtherBodyIndex :type Integer))
  (bind _ascollab_player_character (Utilities|Casting|CastToCollabPlayerCharacter OtherActor))
  (Utilities|CheckorAddOverlappingPlayer _ascollab_player_character false
    (:Overlapping
      (bind _output_get (Variables|Default|SetTargetComponent (Class|CollabAbilitySystemComponent|FindAbilitySystemComponent (Variables|/Script/Engine.Pawn|GetPlayerState _ascollab_player_character))))
      (Utilities|IsValid _output_get
        (:Is%20Valid
          (GameplayEffects|RemoveActiveGameplayEffectbySourceEffect _output_get (Variables|Default|GetSurgBoostEffect) 0 -1))))))

(event EventBeginPlay
  (Class|NiagaraComponent|SetSystemFixedBounds (Variables|Default|GetNiagara) (Class|KismetMathLibrary|MakeBoxwithOrigin (Math|Vector|VectorZero) (Components|Box|GetScaledBoxExtent (Variables|Default|GetBox)))))

(event Collision|EventActorBeginOverlap
  (params (OtherActor :type Actor%20Object%20Reference)))

(event EventTick
  (params (DeltaSeconds :type Float%20%28single-precision%29)))

(fn ConstructionScript
  (bind _niagara (Variables|Default|GetNiagara))
  (bind _box (Variables|Default|GetBox))
  (bind _returnvalue (Components|Box|GetScaledBoxExtent _box))
  (bind _returnvalue_2 (Rendering|Material|CreateDynamicMaterialInstance "/Game/CoLab/Blueprints/Arena/Assets/M_TransparentColor.M_TransparentColor" "None" "None" :!class /Script/Engine.KismetMaterialLibrary))
  (Rendering|Material|SetVectorParameterValue _returnvalue_2 "Color" (Variables|Default|GetBoxColor) :!class /Script/Engine.MaterialInstanceDynamic)
  (Rendering|Material|SetMaterial (Variables|Default|GetCube) 0 _returnvalue_2)
  (Effects|Components|ParticleSystem|SetVectorParameter _niagara "BoxSize" _returnvalue)
  (Effects|Components|ParticleSystem|SetFloatParameter _niagara "SpawnRate" (+ 3.0 (/ (Class|KismetMathLibrary|GetBoxVolume (Class|KismetMathLibrary|MakeBoxwithOrigin (.Origin (Collision|GetComponentBounds _box)) _returnvalue)) 1e+08)))
  (Class|NiagaraComponent|SetSystemFixedBounds _niagara (Class|KismetMathLibrary|MakeBoxwithOrigin (Math|Vector|VectorZero) _returnvalue)))