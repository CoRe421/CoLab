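; Surf Race component that marks an input/output port on a surf block, scaled on construction by its ArrowScale value.
; InvertRotation reverses the port's facing by negating relative pitch and adding a half turn of yaw.
; MoveToCameraLocation gets the owner's block component through BPI_SurfBlock, traces against it from the editor camera, and on a hit snaps the port to that point with the camera's rotation.
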(event EventBeginPlay)

(event EventTick
  (params (DeltaSeconds :type Float%20%28single-precision%29)))

(fn OnComponentConstruction
  (Transformation|SetWorldScale3D (Variables|Default|GetArrowScale)))

(fn InvertRotation
  (bind _relativerotation (Variables|Default|GetRelativeRotation))
  (bind (_roll _pitch _yaw) (Math|Rotator|BreakRotator _relativerotation))
  (Transformation|SetRelativeRotation (Math|Rotator|MakeRotator _roll (* _pitch -1.0) (+ _yaw 1.8e+02)) false false))

(fn MovetoCameraLocation
  (bind _asbpi_surf_block (Utilities|Casting|CastToBPI_SurfBlock (Components|GetOwner)))
  (bind _blockcomponent (Default|GetBlockComponent _asbpi_surf_block))
  (bind (_bhit _hitlocation _cameratransform) (CallFunction|GetLineTracefromEditorCamera _blockcomponent))
  (if _bhit
    (Transformation|SetWorldLocation _hitlocation false false)
    (Transformation|SetWorldRotation (.Rotation (Math|Transform|BreakTransform _cameratransform)) false false)))