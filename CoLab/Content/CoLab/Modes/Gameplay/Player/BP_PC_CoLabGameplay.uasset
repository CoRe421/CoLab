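; Player controller for CoLab gameplay that handles spawning, respawning and the local player's UI.
; On BeginPlay the local client asks the server to spawn it through the game mode, with client UI init creating a layered layout and HUD, also run on possess.
; Death hides the HUD and requests respawn after a delay.
; Pause and tab menus use the menu layer, with a set of transitioning widget stacks blocking pushes mid-transition.
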(event Custom|SR_RequestSpawnPlayer
  (Default|SpawnPlayer (Variables|Default|GetCachedGameMode) self))

(event Custom|SR_CacheGameMode
  (bind _asbp_gm_co_lab_gameplay (Utilities|Casting|CastToBP_GM_CoLabGameplay (Game|GetGameMode)))
  (Variables|Default|SetCachedGameMode _asbp_gm_co_lab_gameplay))

(event Custom|OnPlayerDeath
  (CallFunction|HideUI)
  ;[1 1 1] Temp - find better way to do this perhaps
  ;
  ; Solves race condition where player lifetime hasn't been reached yet before attempted respawn
  (Utilities|FlowControl|Delay 2.0)
  (CallFunction|SRRequestSpawnPlayer))

(event Custom|TryInitGameplayLayout
  (if (Pawn|IsLocalController)
    (Variables|Default|GetGameplayLayout
      (:then)
      (:else
        (bind _returnvalue (UserInterface|CreateWidget "/Game/CoLab/Modes/Gameplay/UI/WB_GameplayLayout.WB_GameplayLayout_C" self))
        (bind _output_get (Variables|Default|SetGameplayLayout _returnvalue))
        (UserInterface|Viewport|AddtoViewport _output_get 0)))))

(event Custom|CL_InitPlayerUI
  (CallFunction|TryInitGameplayLayout)
  (Variables|Default|GetGameplayLayout
    (:then
      (Utilities|FlowControl|Sequence
        (:then_0
          (Variables|Default|GetGameplayHUD
            (:then
              _)
            (:else
              (bind _widget (Default|PushWidgettoLayerStack (Variables|Default|GetGameplayLayout) "(TagName=\"UI.Layer.Game\")" "/Game/CoLab/Modes/Gameplay/UI/WB_GameplayHUD.WB_GameplayHUD_C"))
              (bind _aswb_gameplay_hud (Utilities|Casting|CastToWB_GameplayHUD _widget))
              (bind _output_get (Variables|Default|SetGameplayHUD _aswb_gameplay_hud))))
          (Widget|SetVisibility _output_get "Visible"))
        (:then_1
          (Input|SetInputModeGameOnly self false))))
    (:else)))

(event Custom|SR_InitPlayer
  (CallFunction|CLInitPlayerUI))

(event Input|EnhancedActionEvents|EnhancedInputActionIA_PauseMenu
  (params (ActionValue :type Boolean) (ElapsedSeconds :type Float%20%28double-precision%29) (TriggeredSeconds :type Float%20%28double-precision%29) (InputAction :type Input%20Action%20Object%20Reference :default "/Game/CoLab/Modes/Gameplay/Input/Actions/IA_PauseMenu.IA_PauseMenu"))
  (CallFunction|TryInitGameplayLayout)
  (if (Utilities|Set|IsEmpty (Variables|Default|GetTransitioningStacks))
    (bind _gameplaylayout (Variables|Default|GetGameplayLayout)
      (:then
        (bind _widgetstack (Default|PushWidgettoLayerStack _gameplaylayout "(TagName=\"UI.Layer.Menu\")" "/Game/CoLab/Modes/Gameplay/UI/WB_PauseMenu.WB_PauseMenu_C"))
        (CallFunction|BindtoStackTransition _widgetstack))
      (:else))))

(event Input|EnhancedActionEvents|EnhancedInputActionIA_TabMenu
  (params (ActionValue :type Boolean) (ElapsedSeconds :type Float%20%28double-precision%29) (TriggeredSeconds :type Float%20%28double-precision%29) (InputAction :type Input%20Action%20Object%20Reference :default "/Game/CoLab/Modes/Gameplay/Input/Actions/IA_TabMenu.IA_TabMenu"))
  (CallFunction|TryInitGameplayLayout)
  (Variables|Default|GetGameplayLayout
    (:then
      (if ActionValue
        (if (Utilities|Set|IsEmpty (Variables|Default|GetTransitioningStacks))
          (bind (_widget _widgetstack) (Default|PushWidgettoLayerStack (Variables|Default|GetGameplayLayout) "(TagName=\"UI.Layer.Menu\")" "/Game/CoLab/Modes/Gameplay/UI/WB_TabMenu.WB_TabMenu_C"))
          (Variables|Default|SetCachedTabMenu _widget)
          (CallFunction|BindtoStackTransition _widgetstack))
        (else
          (Variables|Default|GetCachedTabMenu
            (:then
              (bind _widgetstack_2 (Default|RemoveWidgetfromLayerStack (Variables|Default|GetGameplayLayout) "(TagName=\"UI.Layer.Menu\")" (Variables|Default|GetCachedTabMenu)))
              (Variables|Default|SetCachedTabMenu 0)
              (CallFunction|BindtoStackTransition _widgetstack_2))
            (:else)))))
    (:else)))

(event EventBeginPlay
  ;[1 1 1] Makes setup logic only fire on the client
  (if (Pawn|IsLocalController)
    (Development|PrintString (Utilities|GetDisplayName self))
    (CallFunction|SRCacheGameMode)
    (CallFunction|SRRequestSpawnPlayer)
    (CallFunction|SRInitPlayer)))

(fn ConstructionScript)

(fn ReceivePossess
  (params (PossessedPawn :type Pawn%20Object%20Reference))
  (CallFunction|CLInitPlayerUI))

(fn ReceiveUnPossess
  (params (UnpossessedPawn :type Pawn%20Object%20Reference))
  ;[1 1 1] DONT use this, it gets called on player restart but possess isn't called reliably, instead put logic on pawn/player destruction
)

(fn HideUI
  (bind _gameplayhud (Variables|Default|GetGameplayHUD)
    (:then
      (Widget|SetVisibility _gameplayhud "Hidden"))
    (:else)))

(fn OnStackTransitioningChanged
  (params (WidgetStack :type Collab%20Activatable%20Widget%20Stack%20Object%20Reference) (bIsTransitioning :type Boolean))
  (if (not bIsTransitioning)
    (LocalVariables|SetL_Stack WidgetStack)
    (Utilities|Set|Remove (Variables|Default|GetTransitioningStacks) (LocalVariables|GetL_Stack))
    (EventDispatchers|UnbindEventfromOnStackTransitioningChanged (LocalVariables|GetL_Stack) (EventDispatchers|CreateEvent :!event OnStackTransitioningChanged))))

(fn BindtoStackTransition
  (params (WidgetStack :type Collab%20Activatable%20Widget%20Stack%20Object%20Reference))
  (bind _output_get (LocalVariables|SetL_Stack WidgetStack))
  (if (not (Utilities|Set|Contains (Variables|Default|GetTransitioningStacks) _output_get))
    (Utilities|Set|Add (Variables|Default|GetTransitioningStacks) (LocalVariables|GetL_Stack))
    (EventDispatchers|BindEventtoOnStackTransitioningChanged (LocalVariables|GetL_Stack) (EventDispatchers|CreateEvent :!event OnStackTransitioningChanged))))