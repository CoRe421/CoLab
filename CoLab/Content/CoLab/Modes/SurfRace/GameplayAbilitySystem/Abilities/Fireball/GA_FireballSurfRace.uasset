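; Surf Race variant of the fireball gameplay ability that extends the parent's explosion handling to notify actors caught in the blast.
; On explosion, sphere overlaps using the fireball's radial force radius gather nearby actors and components.
; Components are grouped by owner and passed to each actor through OnTouchedMessage, then the parent explosion logic runs.
; A ForceNetUpdate loop over hit actors is left unconnected.
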(event Ability|EventActivateAbility
  (|CallParentFunction) ; This node is disabled and will not be called.\nDrag off pins to build functionality.
)

(event Ability|EventOnEndAbility
  (params (bWasCancelled :type Boolean))
  (|CallParentFunction bWasCancelled) ; This node is disabled and will not be called.\nDrag off pins to build functionality.
)

(fn HandleFireballExplosion
  (params (ExplosionLocation :type Gameplay%20Ability%20Targeting%20Location%20Info%20Structure))
  (bind _fireball (Variables|Default|GetFireball))
  (bind _literaltransform (Utilities|Struct|BreakGameplayAbilityTargetingLocationInfo ExplosionLocation))
  (bind _radialforce (Variables|/Game/CoLab/Modes/Arena/GameplayAbilitySystem/Abilities/Fireball/Blueprints/BP_Fireball.BP_Fireball_C|GetRadialForce _fireball))
  (bind _location (Math|Transform|BreakTransform _literaltransform))
  (bind _radius (Variables|/Script/Engine.RadialForceComponent|GetRadius _radialforce))
  (Utilities|FlowControl|Sequence
    (:then_0
      (Utilities|IsValid (Variables|Default|GetFireball)
        (:Is%20Valid
          (bind _outactors (Collision|SphereOverlapActors _location _radius (Utilities|Array|MakeArray) 0))
          (LocalVariables|SetL_ImpulseHitActors _outactors)
          (bind _outcomponents (Collision|SphereOverlapComponents _location _radius (Utilities|Array|MakeArray)))
          (LocalVariables|SetL_ImpulseHitComponents _outcomponents)
          (for _array_element (LocalVariables|GetL_ImpulseHitActors)
            (LocalVariables|SetL_HitActor _array_element)
            (Utilities|Array|Clear (LocalVariables|GetL_ActorHitComponents))
            (for _array_element_2 (LocalVariables|GetL_ImpulseHitComponents)
              (if (== (Components|GetOwner _array_element_2) (LocalVariables|GetL_HitActor))
                (Utilities|Array|Add (LocalVariables|GetL_ActorHitComponents) _array_element_2)))
            (Class|BPISpleefActor|OnTouched(Message) (LocalVariables|GetL_HitActor) (LocalVariables|GetL_ActorHitComponents))))))
    (:then_1
      (|CallParentFunction ExplosionLocation))))