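; Fireball projectile actor for the Arena mode's Gameplay Ability System, with collision sized to its mesh bounds.
; Hitting anything but its owner fires an explosion GameplayCue scaled by blast radius, sends the owner a hit event with location target data, then destroys it.
; If destroyed without a hit, the server sends a despawn event instead.
; Setters configure RadialForce radius and strength, plus gravity, which the server also multicasts.
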(event OnComponentHit(SphereCollision)
  (params (HitComponent :type Primitive%20Component%20Object%20Reference) (OtherActor :type Actor%20Object%20Reference) (OtherComp :type Primitive%20Component%20Object%20Reference) (NormalImpulse :type Vector :default "0, 0, 0") (Hit :type Hit%20Result%20Structure%20%28by%20ref%29))
  (bind _location (Collision|BreakHitResult Hit))
  (bind _returnvalue (Math|Transform|MakeTransform _location))
  (bind _gameplayabilitytargetinglocationinfo (Utilities|Struct|MakeGameplayAbilityTargetingLocationInfo "LiteralTransform" _returnvalue))
  (if (!= OtherActor (Components|GetOwner))
    (GameplayCue|ExecuteGameplayCueOnActor(Burst) (Components|GetOwner) "(TagName=\"GameplayCue.AOE.FireballEffect\")" (Ability|GameplayCue|MakeGameplayCueParameters :RawMagnitude (CallFunction|GetExplosionRadius) :Location _location))
    (Variables|Default|SetbTriggered true)
    (Ability|SendGameplayEventtoActor (Components|GetOwner) "(TagName=\"Gameplay.Event.Hit.Fireball\")" (Utilities|Struct|MakeGameplayEventData "(TagName=\"\")" self OtherActor 0 0 "()" "(GameplayTags=)" "(GameplayTags=)" 0.0 (Class|AbilitySystemBlueprintLibrary|AbilityTargetDatafromLocations _gameplayabilitytargetinglocationinfo _gameplayabilitytargetinglocationinfo)))
    (Actor|DestroyActor)))

(event Custom|OnActorHit_Event
  (params (SelfActor :type Actor%20Object%20Reference) (OtherActor :type Actor%20Object%20Reference) (NormalImpulse :type Vector) (Hit :type Hit%20Result%20Structure%20%28by%20ref%29))
  (Development|PrintString "Hello"))

(event Custom|MUL_SetProjectileGravity
  (params (NewProjectileGravity :type Float%20%28single-precision%29))
  (Variables|/Script/Engine.ProjectileMovementComponent|SetProjectileGravityScale (Variables|Default|GetProjectileMovement) NewProjectileGravity))

(event EventBeginPlay)

(event Collision|EventActorBeginOverlap
  (params (OtherActor :type Actor%20Object%20Reference)))

(event EventTick
  (params (DeltaSeconds :type Float%20%28single-precision%29)))

(event EventDestroyed
  (if (Class|CollabFunctionLibrary|IsActoronServer)
    (if (not (Variables|Default|GetbTriggered))
      (Ability|SendGameplayEventtoActor (Components|GetOwner) "(TagName=\"Gameplay.Event.Despawn.Fireball\")" (Utilities|Struct|MakeGameplayEventData "(TagName=\"\")" self)))))

(fn ConstructionScript
  (|CallParentFunction)
  (CallFunction|SetCollisionRadius (.SphereRadius (Collision|GetComponentBounds (Variables|Default|GetStaticMesh)))))

(fn SetExplosionRadius
  (params (ExplosionRadius :type Float%20%28single-precision%29))
  (Variables|/Script/Engine.RadialForceComponent|SetRadius (Variables|Default|GetRadialForce) ExplosionRadius))

(fn SetExplosionStrength
  (params (ImpulseStrength :type Float%20%28single-precision%29))
  (Variables|/Script/Engine.RadialForceComponent|SetImpulseStrength (Variables|Default|GetRadialForce) ImpulseStrength))

(fn SetGravityScale
  (params (NewGravityScale :type Float%20%28single-precision%29))
  (Variables|/Script/Engine.ProjectileMovementComponent|SetProjectileGravityScale (Variables|Default|GetProjectileMovement) NewGravityScale)
  (if (Class|CollabFunctionLibrary|IsActoronServer)
    (CallFunction|MULSetProjectileGravity NewGravityScale)))

(fn GetExplosionRadius
  (return (Variables|/Script/Engine.RadialForceComponent|GetRadius (Variables|Default|GetRadialForce))))