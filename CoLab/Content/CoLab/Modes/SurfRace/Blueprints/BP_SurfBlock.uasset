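; Modular level block for SurfRace that groups level actors inside a box sized in whole SurfBlockUnitLength units.
; Overlap and editor update events refresh ManagedActors, attaching overlapped actors except other blocks and their children.
; ResizeBlockToManagedActors refits the box to those actors in an undoable transaction, offsetting attached actors to compensate for the moved origin.
; SpawnIOPortAtCamera adds an IO port component where an editor-camera trace hits the box.
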(event OnComponentBeginOverlap(BlockExtent)
  (params (OverlappedComponent :type Primitive%20Component%20Object%20Reference) (OtherActor :type Actor%20Object%20Reference) (OtherComp :type Primitive%20Component%20Object%20Reference) (OtherBodyIndex :type Integer) (bFromSweep :type Boolean) (SweepResult :type Hit%20Result%20Structure%20%28by%20ref%29))
  (CallFunction|UpdateBoundsandManagedActors))

(event OnComponentEndOverlap(BlockExtent)
  (params (OverlappedComponent :type Primitive%20Component%20Object%20Reference) (OtherActor :type Actor%20Object%20Reference) (OtherComp :type Primitive%20Component%20Object%20Reference) (OtherBodyIndex :type Integer))
  (CallFunction|UpdateBoundsandManagedActors))

(event EventBeginPlay)

(event Collision|EventActorBeginOverlap
  (params (OtherActor :type Actor%20Object%20Reference)))

(event EventTick
  (params (DeltaSeconds :type Float%20%28single-precision%29)))

(event EventUpdateOverlaps
  (CallFunction|UpdateBoundsandManagedActors))

(fn ConstructionScript
  (|CallParentFunction)
  (CallFunction|ResizeBlockExtent))

(fn ResizeBlocktoManagedActors
  (Development|Editor|CreateCopyforUndoBuffer self)
  (Class|KismetSystemLibrary|BeginTransaction "Resize Block" "" self)
  (CallFunction|UpdateBoundsandManagedActors)
  (for _array_element (Variables|Default|GetManagedActors)
    (LocalVariables|SetL_ActorOrigin (.Origin (Collision|GetActorBounds _array_element false true)))
    (LocalVariables|SetL_ActorExtent (.BoxExtent (Collision|GetActorBounds _array_element false true)))
    (Utilities|FlowControl|Sequence
      (:then_0
        (Utilities|FlowControl|DoOnce false
          (:Completed
            (LocalVariables|SetL_Min (LocalVariables|GetL_ActorOrigin))
            (LocalVariables|SetL_Max (LocalVariables|GetL_ActorOrigin)))))
      (:then_1
        (LocalVariables|SetL_Min (Math|Vector|MakeVector (Math|Float|Min(Float) (.X (Math|Vector|BreakVector (LocalVariables|GetL_Min))) (+ (.X (Math|Vector|BreakVector (LocalVariables|GetL_ActorOrigin))) (Math|Float|SelectFloat (.X (Math|Vector|BreakVector (LocalVariables|GetL_ActorExtent))) (* (.X (Math|Vector|BreakVector (LocalVariables|GetL_ActorExtent))) -1.0) (< (.X (Math|Vector|BreakVector (LocalVariables|GetL_ActorExtent))) (* (.X (Math|Vector|BreakVector (LocalVariables|GetL_ActorExtent))) -1.0))))) (Math|Float|Min(Float) (.Y (Math|Vector|BreakVector (LocalVariables|GetL_Min))) (+ (.Y (Math|Vector|BreakVector (LocalVariables|GetL_ActorOrigin))) (Math|Float|SelectFloat (.Y (Math|Vector|BreakVector (LocalVariables|GetL_ActorExtent))) (* (.Y (Math|Vector|BreakVector (LocalVariables|GetL_ActorExtent))) -1.0) (< (.Y (Math|Vector|BreakVector (LocalVariables|GetL_ActorExtent))) (* (.Y (Math|Vector|BreakVector (LocalVariables|GetL_ActorExtent))) -1.0))))) (Math|Float|Min(Float) (.Z (Math|Vector|BreakVector (LocalVariables|GetL_Min))) (+ (.Z (Math|Vector|BreakVector (LocalVariables|GetL_ActorOrigin))) (Math|Float|SelectFloat (.Z (Math|Vector|BreakVector (LocalVariables|GetL_ActorExtent))) (* (.Z (Math|Vector|BreakVector (LocalVariables|GetL_ActorExtent))) -1.0) (< (.Z (Math|Vector|BreakVector (LocalVariables|GetL_ActorExtent))) (* (.Z (Math|Vector|BreakVector (LocalVariables|GetL_ActorExtent))) -1.0))))))))
      (:then_2
        (LocalVariables|SetL_Max (Math|Vector|MakeVector (Math|Float|Max(Float) (.X (Math|Vector|BreakVector (LocalVariables|GetL_Max))) (+ (.X (Math|Vector|BreakVector (LocalVariables|GetL_ActorOrigin))) (Math|Float|SelectFloat (.X (Math|Vector|BreakVector (LocalVariables|GetL_ActorExtent))) (* (.X (Math|Vector|BreakVector (LocalVariables|GetL_ActorExtent))) -1.0) (> (.X (Math|Vector|BreakVector (LocalVariables|GetL_ActorExtent))) (* (.X (Math|Vector|BreakVector (LocalVariables|GetL_ActorExtent))) -1.0))))) (Math|Float|Max(Float) (.Y (Math|Vector|BreakVector (LocalVariables|GetL_Max))) (+ (.Y (Math|Vector|BreakVector (LocalVariables|GetL_ActorOrigin))) (Math|Float|SelectFloat (.Y (Math|Vector|BreakVector (LocalVariables|GetL_ActorExtent))) (* (.Y (Math|Vector|BreakVector (LocalVariables|GetL_ActorExtent))) -1.0) (> (.Y (Math|Vector|BreakVector (LocalVariables|GetL_ActorExtent))) (* (.Y (Math|Vector|BreakVector (LocalVariables|GetL_ActorExtent))) -1.0))))) (Math|Float|Max(Float) (.Z (Math|Vector|BreakVector (LocalVariables|GetL_Max))) (+ (.Z (Math|Vector|BreakVector (LocalVariables|GetL_ActorOrigin))) (Math|Float|SelectFloat (.Z (Math|Vector|BreakVector (LocalVariables|GetL_ActorExtent))) (* (.Z (Math|Vector|BreakVector (LocalVariables|GetL_ActorExtent))) -1.0) (> (.Z (Math|Vector|BreakVector (LocalVariables|GetL_ActorExtent))) (* (.Z (Math|Vector|BreakVector (LocalVariables|GetL_ActorExtent))) -1.0))))))))))
  (LocalVariables|SetL_LocationDelta (- (Transformation|GetActorLocation) (LocalVariables|GetL_Min)))
  (Transformation|SetActorLocation (LocalVariables|GetL_Min) false false)
  (Variables|Default|SetBlockExtender (* (Math|Vector|MakeVector (Math|Conversions|ToFloat(Integer) (Math|Float|Ceil (.X (Math|Vector|BreakVector (/ (- (LocalVariables|GetL_Max) (Transformation|GetActorLocation)) (Variables|Default|GetSurfBlockUnitLength)))))) (Math|Conversions|ToFloat(Integer) (Math|Float|Ceil (.Y (Math|Vector|BreakVector (/ (- (LocalVariables|GetL_Max) (Transformation|GetActorLocation)) (Variables|Default|GetSurfBlockUnitLength)))))) (Math|Conversions|ToFloat(Integer) (Math|Float|Ceil (.Z (Math|Vector|BreakVector (/ (- (LocalVariables|GetL_Max) (Transformation|GetActorLocation)) (Variables|Default|GetSurfBlockUnitLength))))))) (Variables|Default|GetSurfBlockUnitLength)))
  (CallFunction|ResizeBlockExtent)
  (CallFunction|AddOffsettoAttachedActors (LocalVariables|GetL_LocationDelta))
  (Class|KismetSystemLibrary|EndTransaction))

(fn ResizeBlockExtent
  (bind (_worldsize _halfsize) (CallFunction|GetWorldBlockSize))
  (bind _arrow (Variables|Default|GetArrow))
  (bind _blockextent (Variables|Default|GetBlockExtent))
  (if (Math|Vector|VectorIsNearlyZero (Variables|Default|GetBlockExtender))
    (Variables|Default|SetBlockExtender _worldsize)
    (elif (Utilities|Operators|EqualEqual (Variables|Default|GetBlockExtender) _worldsize 0.0)
      _
      (else
        (Variables|Default|SetBlockSize (Math|Conversions|ToVector(Float) (Class|KismetMathLibrary|FTruncVector (/ (Variables|Default|GetBlockExtender) (Variables|Default|GetSurfBlockUnitLength))))))))
  (Transformation|SetRelativeLocation _blockextent _halfsize false false)
  (Components|Box|SetBoxExtent _blockextent _halfsize true)
  (LocalVariables|SetL_bSizeUpadted (Utilities|Operators|NotEqual(!=) (Variables|Default|GetOldBlockSize) (Variables|Default|GetBlockSize) 0.5))
  (Utilities|FlowControl|Sequence
    (:then_0
      (Variables|/Script/Engine.ArrowComponent|SetArrowSize _arrow (.X (Math|Vector|BreakVector (Variables|Default|GetBlockSize))))
      (Variables|/Script/Engine.ArrowComponent|SetArrowLength _arrow (/ (* (.X (Math|Vector|BreakVector (Variables|Default|GetBlockSize))) (Variables|Default|GetSurfBlockUnitLength)) (Variables|/Script/Engine.ArrowComponent|GetArrowSize _arrow))))
    (:then_1
      (Variables|Default|SetOldBlockSize (Variables|Default|GetBlockSize))
      (return (LocalVariables|GetL_bSizeUpadted)))))

(fn GetWorldBlockSize
  (bind _blocksize (Variables|Default|GetBlockSize))
  (bind _surfblockunitlength (Variables|Default|GetSurfBlockUnitLength))
  (bind _returnvalue (* _blocksize _surfblockunitlength))
  (return _returnvalue (/ _returnvalue 2.0)))

(fn UpdateBoundsandManagedActors
  (bind _managedactors (Variables|Default|GetManagedActors))
  (bind _overlappedactors (CallFunction|GetCurrentOverlappedActors))
  (bind _output_get (LocalVariables|SetL_OverlappedActors _overlappedactors))
  (if (not (and (== (Utilities|Array|Length _output_get) (Utilities|Array|Length _managedactors)) (Utilities|Array|Identical _output_get _managedactors)))
    ;[1 1 1] Only works when called from "OnPostPropertyChanged"
    (for _array_element (Variables|Default|GetManagedActors)
      (Transformation|DetachFromActor _array_element "KeepWorld" "KeepWorld" "KeepWorld"))
    (Utilities|Array|Clear (Variables|Default|GetManagedActors))
    (for _array_element_2 (LocalVariables|GetL_OverlappedActors)
      (Utilities|Casting|CastToBP_SurfBlock _array_element_2
        (:CastFailed
          (Utilities|Casting|CastToBP_SurfBlock (Actor|GetAttachParentActor _array_element_2)
            (:CastFailed
              (Transformation|AttachActorToActor _array_element_2 self "None" "KeepWorld" "KeepWorld" "KeepWorld" true)
              (Utilities|Array|Add (Variables|Default|GetManagedActors) _array_element_2))))))))

(fn GetCurrentOverlappedActors
  (bind _blockextent (Variables|Default|GetBlockExtent))
  (bind _outactors (Collision|ComponentOverlapActors _blockextent (Transformation|GetWorldTransform _blockextent) (Utilities|Array|MakeArray) 0 (Utilities|Array|MakeArray)))
  (return _outactors))

(fn OnPostActorUpdate
  (CallFunction|UpdateBoundsandManagedActors))

(fn AddOffsettoAttachedActors
  (params (Offset :type Vector))
  (bind _output_get (LocalVariables|SetL_AttachedActors (Actor|GetAttachedActors true false)))
  (for _array_element _output_get
    (Transformation|SetActorLocation _array_element (+ (Transformation|GetActorLocation _array_element) Offset) false false)))

(fn SpawnIOPortatCamera
  (bind (_bhit _hitlocation _cameratransform) (CallFunction|GetLineTracefromEditorCamera (Variables|Default|GetBlockExtent)))
  (if _bhit
    (LocalVariables|SetL_CameraTransform _cameratransform)
    (LocalVariables|SetL_SplineLocation _hitlocation)
    (Development|PrintString (Utilities|String|SelectString (Utilities|String|ToString(Vector) "0, 0, 0") "Miss" false))
    (if true
      (Class|CollabFunctionLibrary|TryAddandRegisterComponenttoActor self "/Game/CoLab/Modes/SurfRace/Blueprints/BPC_SurfBlockIOPort.BPC_SurfBlockIOPort_C" (Math|Transform|MakeTransform (LocalVariables|GetL_SplineLocation) (.rotation (LocalVariables|GetL_CameraTransform)))))))

(fn GetBlockComponent
  (return (Variables|Default|GetBlockExtent)))