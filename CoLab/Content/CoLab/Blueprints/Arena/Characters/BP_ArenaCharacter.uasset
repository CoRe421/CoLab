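; First-person arena character Blueprint that shows health and mana on an attribute widget; its ability-system binding code here is disconnected.
; Camera pitch goes to the server and returns through RepNotify.
; Collision-ignore actors are kept in local and replicated lists, merged onto the capsule in OnRep.
; TryFire passes weapon-interface components to an empty server event; death calls an empty client event, while a separate multicast timeline rolls the mesh.
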(event OnComponentHit(CapsuleComponent)
  (params (HitComponent :type Primitive%20Component%20Object%20Reference) (OtherActor :type Actor%20Object%20Reference) (OtherComp :type Primitive%20Component%20Object%20Reference) (NormalImpulse :type Vector :default "0, 0, 0") (Hit :type Hit%20Result%20Structure%20%28by%20ref%29))
  (bind _returnvalue (Class|PrimitiveComponent|CopyArrayOfMoveIgnoreActors (Variables|Default|GetCapsuleComponent)))
  (Development|PrintString (Utilities|String|ToString(Integer) (Utilities|Array|Length _returnvalue))))

(event Custom|SR_FireWeapon
  (params (Weapon :type Co%20Lab%20Weapon%20Interface%20Interface)))

(event Custom|CL_ControllerPlayerDeath
  ;[1 1 1] Will only fire on local client with a valid PlayerController
  (if (Pawn|IsLocallyControlled)
    _))

(event Custom|MUL_PlayDeathAnimation
  (Variables|Default|SetPreDeathRotation (Variables|/Script/Engine.SceneComponent|GetRelativeRotation (Variables|Default|GetMesh1P)))
  (bind _rotationpercent (Timeline|DeathTimeline PlayFromStart)
    (:Update
      (Transformation|SetRelativeRotation (Variables|Default|GetMesh1P) (Math|Rotator|Lerp(Rotator) (Math|Rotator|MakeRotator 0.0 (.Pitch (Math|Rotator|BreakRotator (Variables|Default|GetPreDeathRotation))) (.Yaw (Math|Rotator|BreakRotator (Variables|Default|GetPreDeathRotation)))) (Math|Rotator|MakeRotator 9e+01 (.Pitch (Math|Rotator|BreakRotator (Variables|Default|GetPreDeathRotation))) (.Yaw (Math|Rotator|BreakRotator (Variables|Default|GetPreDeathRotation)))) _rotationpercent) false false))))

(event Custom|SVR_SetPlayerCameraPitch
  (params (PlayerCameraPitch :type Float%20%28double-precision%29))
  (Variables|Default|SetPlayerCameraPitch PlayerCameraPitch))

(event Input|EnhancedActionEvents|EnhancedInputActionIA_CollabLookMouse
  (params (ActionValue :type Vector%202D%20Structure) (ElapsedSeconds :type Float%20%28double-precision%29) (TriggeredSeconds :type Float%20%28double-precision%29) (InputAction :type Input%20Action%20Object%20Reference :default "/Collab/Input/Actions/IA_CollabLookMouse.IA_CollabLookMouse"))
  (CallFunction|SVRSetPlayerCameraPitch (.Pitch (Math|Rotator|BreakRotator (Transformation|GetWorldRotation (Variables|Default|GetFirstPersonCameraComponent))))))

(event EventBeginPlay
  (Utilities|FlowControl|Sequence))

(event EventOnDestroyCharacter
  (CallFunction|OnCharacterDeath))

(event Input|KeyboardEvents|Q
  (params (Key :type Key%20Structure :default "None")))

(event Input|KeyboardEvents|F5
  (params (Key :type Key%20Structure :default "None")))

(event Input|KeyboardEvents|CapsLock
  (params (Key :type Key%20Structure :default "None")))

(fn ConstructionScript)

(fn TryFire
  (params (Value :type Input%20Action%20Value%20Structure%20%28by%20ref%29))
  (bind _output_get (LocalVariables|SetL_WeaponComponents (Class|Actor|GetComponentsbyInterface "/Script/CoLab.CoLabWeaponInterface")))
  (for _array_element _output_get
    (bind _asco_lab_weapon_interface (Utilities|Casting|CastToCoLabWeaponInterface _array_element))
    (CallFunction|SRFireWeapon _asco_lab_weapon_interface)))

(fn OnHealthChanged
  (params (NewHealth :type Float%20%28single-precision%29) (MaxHealth :type Float%20%28single-precision%29))
  (bind _aswb_character_attributes (Utilities|Casting|CastToWB_CharacterAttributes (UserInterface|GetWidget (Variables|Default|GetAttributeWidgetComponent))))
  (Default|SetHealth _aswb_character_attributes NewHealth MaxHealth))

(fn SetupAbilitySystemComponentBindings
  (|CallParentFunction))

(fn OnManaChanged
  (params (NewMana :type Float%20%28single-precision%29) (OldMana :type Float%20%28single-precision%29))
  (bind _aswb_character_attributes (Utilities|Casting|CastToWB_CharacterAttributes (UserInterface|GetWidget (Variables|Default|GetAttributeWidgetComponent))))
  (Default|SetMana _aswb_character_attributes NewMana OldMana))

(fn OnCharacterDeath
  (Utilities|FlowControl|Sequence
    (:then_0
      (CallFunction|CLControllerPlayerDeath))))

(fn DetachCamera
  (Transformation|DetachFromComponent (Variables|Default|GetFirstPersonCameraComponent) "KeepRelative" "KeepRelative" "KeepRelative" true))

(fn OnRepPlayerCameraPitch
  (bind _firstpersoncameracomponent (Variables|Default|GetFirstPersonCameraComponent))
  (bind _returnvalue (Transformation|GetWorldRotation _firstpersoncameracomponent))
  (bind (_roll _pitch _yaw) (Math|Rotator|BreakRotator _returnvalue))
  (Transformation|SetWorldRotation _firstpersoncameracomponent (Math|Rotator|MakeRotator _roll (Variables|Default|GetPlayerCameraPitch) _yaw) false false))

(fn SetIgnoreActorCollisions
  (params (Actor :type Actor%20Object%20Reference) (bShouldIgnore :type Boolean))
  (bind _repcollisionignoredactors (Variables|Default|GetRepCollisionIgnoredActors))
  (bind _localcollisionignoredactors (Variables|Default|GetLocalCollisionIgnoredActors))
  (Collision|IgnoreActorwhenMoving (Variables|Default|GetCapsuleComponent) Actor bShouldIgnore)
  (if bShouldIgnore
    (Utilities|Array|AddUnique _localcollisionignoredactors Actor)
    (Utilities|Array|AddUnique _repcollisionignoredactors Actor)
    (else
      (Utilities|Array|RemoveItem _localcollisionignoredactors Actor)
      (Utilities|Array|RemoveItem _repcollisionignoredactors Actor))))

(fn OnRepRepCollisionIgnoredActors
  (bind _capsulecomponent (Variables|Default|GetCapsuleComponent))
  (Collision|ClearMoveIgnoreActors (Variables|Default|GetCapsuleComponent))
  (for _array_element (Variables|Default|GetRepCollisionIgnoredActors)
    (Collision|IgnoreActorwhenMoving _capsulecomponent _array_element true))
  (for _array_element_2 (Variables|Default|GetLocalCollisionIgnoredActors)
    (Collision|IgnoreActorwhenMoving _capsulecomponent _array_element_2 true)))

(fn GetProjectileSpawnComponent
  (return (Variables|Default|GetProjectileSpawnLocation)))

(fn GetProjectileSpawnLocation
  (bind _projectilespawnlocation (Variables|Default|GetProjectileSpawnLocation))
  (bind _returnvalue (Transformation|GetWorldTransform _projectilespawnlocation))
  (bind (_location _rotation) (Math|Transform|BreakTransform _returnvalue))
  (return _location _rotation))