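; Base projectile actor for Arena ability-spawned projectiles, built around a sphere collision component.
; The construction script applies the collision radius and whether the sphere ignores its owner while moving, and a setter maintains a list of other ignored actors.
; RepNotify functions reapply the owner setting and rebuild the sphere's move-ignore list from that list.
; Hits only print the other actor's name.
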(event OnComponentHit(SphereCollision)
  (params (HitComponent :type Primitive%20Component%20Object%20Reference) (OtherActor :type Actor%20Object%20Reference) (OtherComp :type Primitive%20Component%20Object%20Reference) (NormalImpulse :type Vector :default "0, 0, 0") (Hit :type Hit%20Result%20Structure%20%28by%20ref%29))
  (Development|PrintString (Utilities|GetDisplayName OtherActor)))

(event EventBeginPlay)

(event Collision|EventActorBeginOverlap
  (params (OtherActor :type Actor%20Object%20Reference)))

(event EventTick
  (params (DeltaSeconds :type Float%20%28single-precision%29)))

(fn ConstructionScript
  (CallFunction|SetCollisionRadius (Variables|Default|GetSphereCollisionRadius))
  (CallFunction|SetIgnoreOwnerCollision (Variables|Default|GetbIgnoreOwnerCollision)))

(fn SetCollisionRadius
  (params (SphereCollisionRadius :type Float%20%28single-precision%29))
  (bind _output_get (Variables|Default|SetSphereCollisionRadius SphereCollisionRadius))
  (Components|Sphere|SetSphereRadius (Variables|Default|GetSphereCollision) _output_get true))

(fn SetIgnoreOwnerCollision
  (params (bIgnoreOwnerCollision :type Boolean))
  (bind _output_get (Variables|Default|SetbIgnoreOwnerCollision bIgnoreOwnerCollision))
  (Collision|IgnoreActorwhenMoving (Variables|Default|GetSphereCollision) (Components|GetOwner) _output_get))

(fn OnRepBIgnoreOwnerCollision
  (Collision|IgnoreActorwhenMoving (Variables|Default|GetSphereCollision) (Components|GetOwner) (Variables|Default|GetbIgnoreOwnerCollision)))

(fn SetIgnoreActorCollisions
  (params (Actor :type Actor%20Object%20Reference) (bShouldIgnore :type Boolean))
  (bind _collisionignoredactors (Variables|Default|GetCollisionIgnoredActors))
  (Collision|IgnoreActorwhenMoving (Variables|Default|GetSphereCollision) Actor bShouldIgnore)
  (if bShouldIgnore
    (Utilities|Array|AddUnique _collisionignoredactors Actor)
    (else
      (Utilities|Array|RemoveItem _collisionignoredactors Actor))))

(fn OnRepCollisionIgnoredActors
  (Collision|ClearMoveIgnoreActors (Variables|Default|GetSphereCollision))
  (for _array_element (Variables|Default|GetCollisionIgnoredActors)
    (Collision|IgnoreActorwhenMoving (Variables|Default|GetSphereCollision) _array_element true)))