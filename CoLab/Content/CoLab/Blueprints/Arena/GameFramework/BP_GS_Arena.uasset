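; Arena GameState that tracks per-player scores and caches the ruleset supplied by the arena GameMode.
; On authority, it syncs score entries with the player list and awards the instigator the ruleset's kill value on player death.
; Score changes and RepNotifies for scores and ruleset refresh tab menu widgets found through an interface.
; It exposes score and win-threshold getters, while the multicast win handler is an empty stub.
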(event Custom|SVR_UpdateCachedRuleset
  (bind _ruleset (Default|GetArenaRuleset (Variables|Default|GetCachedGameMode)))
  (Variables|Default|SetCachedRuleset _ruleset))

(event Custom|MUL_HandlePlayerWin
  (params (WinningPlayer :type Unique%20Net%20Id%20Repl%20Structure)))

(event Custom|OnPlayerScoreUpdate
  (params (PlayerID :type Integer%20%28by%20ref%29) (PlayerScore :type Integer%20%28by%20ref%29))
  (CallFunction|UpdateTabMenus))

(event EventBeginPlay
  (|CallParentFunction)
  (Utilities|FlowControl|Sequence
    (:then_0
      (EventDispatchers|BindEventtoOnPlayerListUpdated (EventDispatchers|CreateEvent :!event PlayerListUpdated)))
    (:then_1
      (Networking|SwitchHasAuthority
        (:Authority
          (bind _asbpi_gm_arena (Utilities|Casting|CastToBPI_GM_Arena (Game|GetGameMode)))
          (Variables|Default|SetCachedGameMode _asbpi_gm_arena)
          (CallFunction|SVRUpdateCachedRuleset)
          (EventDispatchers|BindEventtoOnPlayerScoreUpdated (delegate Custom|OnPlayerScoreUpdate)))
        (:Remote
          (CallFunction|SVRUpdateCachedRuleset))))))

(event EventTick
  (params (DeltaSeconds :type Float%20%28single-precision%29))
  (|CallParentFunction DeltaSeconds) ; This node is disabled and will not be called.\nDrag off pins to build functionality.
)

(event EventOnPlayerDeath
  (params (Instigator :type Actor%20Object%20Reference) (Target :type Actor%20Object%20Reference))
  (Networking|SwitchHasAuthority
    (:Authority
      (bind _asplayer_state (Utilities|Casting|CastToPlayerState Instigator))
      (CallFunction|AddPlayerScore (Variables|/Script/Engine.PlayerState|GetPlayerId _asplayer_state) (Default|GetPlayerKillScoreValue (Variables|Default|GetCachedRuleset))))))

(fn ConstructionScript
  (|CallParentFunction))

(fn AddPlayerScore
  (params (PlayerID :type Integer%20%28by%20ref%29) (ScoreToAdd :type Integer%20%28by%20ref%29))
  (bind (_playerscore _bfound) (CallFunction|TryFindPlayerScore PlayerID))
  (CallFunction|SetPlayerScore PlayerID (Math|Integer|SelectInt (+ (.Score (Utilities|Struct|BreakS_PlayerScore _playerscore)) ScoreToAdd) ScoreToAdd _bfound)))

(fn UpdateTabMenus
  (bind _foundwidgets (Class|WidgetBlueprintLibrary|GetAllWidgetswithInterface "/Collab/UI/Common/TabMenu/BPI_CollabPlayerListItem.BPI_CollabPlayerListItem_C" false))
  (for _array_element _foundwidgets
    (Class|BPICollabPlayerListItem|UpdateWidget(Message) _array_element)))

(fn UpdateRulesetProperties
  (params (PropertyName :type Name))
  (CallFunction|SVRUpdateCachedRuleset))

(fn OnRepCachedRuleset
  (CallFunction|UpdateTabMenus))

(fn TryFindPlayerScore
  (params (PlayerID :type Integer))
  (for _array_element (Variables|Default|GetPlayerScores)
    (if (== (.PlayerID (Utilities|Struct|BreakS_PlayerScore _array_element)) PlayerID)
      (return _array_element true)))
  (return "" false))

(fn SetPlayerScore
  (params (PlayerID :type Integer%20%28by%20ref%29) (NewScore :type Integer))
  (Networking|SwitchHasAuthority
    (:Authority
      (for _index (range 0 (Utilities|Array|LastIndex (Variables|Default|GetPlayerScores)))
        (if (== (.PlayerID (Utilities|Struct|BreakS_PlayerScore (Utilities|Array|Get(acopy) (Variables|Default|GetPlayerScores) _index))) PlayerID)
          (if (!= (.Score (Utilities|Struct|BreakS_PlayerScore (Utilities|Array|Get(acopy) (Variables|Default|GetPlayerScores) _index))) NewScore)
            (Utilities|Struct|SetmembersinS_PlayerScore (Utilities|Array|Get(acopy) (Variables|Default|GetPlayerScores) _index) NewScore)
            (Default|CallOnPlayerScoreUpdated PlayerID NewScore)
            (return)
            (else
              (return)))))
      ;[1 1 1] If player wasn't found, will add new player to array here
      (Utilities|Array|Add (Variables|Default|GetPlayerScores) (Utilities|Struct|MakeS_PlayerScore PlayerID NewScore))
      (return))))

(fn PlayerListUpdated
  (Networking|SwitchHasAuthority
    (:Authority
      (CallFunction|UpdateLocalPlayerScores))))

(fn UpdateLocalPlayerScores
  (for _array_element (Variables|Default|GetRepPlayerArray)
    (Utilities|Set|Add (LocalVariables|GetL_FoundPlayers) (Variables|/Script/Engine.PlayerState|GetPlayerId _array_element))
    (bind _bfound (CallFunction|TryFindPlayerScore (Variables|/Script/Engine.PlayerState|GetPlayerId _array_element)))
    (if (not _bfound)
      (CallFunction|SetPlayerScore (Variables|/Script/Engine.PlayerState|GetPlayerId _array_element))))
  (LocalVariables|SetL_CurrentIndex 0)
  (while (< (LocalVariables|GetL_CurrentIndex) (Utilities|Array|Length (Variables|Default|GetPlayerScores)))
    (if (Utilities|Set|Contains (LocalVariables|GetL_FoundPlayers) (.PlayerID (Utilities|Struct|BreakS_PlayerScore (Utilities|Array|Get(acopy) (Variables|Default|GetPlayerScores) (LocalVariables|GetL_CurrentIndex)))))
      (Math|Integer|IncrementInt (LocalVariables|GetL_CurrentIndex))
      (else
        (Utilities|Array|RemoveIndex (Variables|Default|GetPlayerScores) (LocalVariables|GetL_CurrentIndex))))))

(fn OnRepPlayerScores
  (CallFunction|OnPlayerScoreUpdate))

(fn GetMaxPlayerScore
  (bind _cachedruleset (Variables|Default|GetCachedRuleset)
    (:then
      (return (Default|GetPlayerWinScoreThreshold _cachedruleset)))
    (:else)))

(fn GetPlayerScore
  (params (PlayerID :type Integer))
  (bind (_playerscore _bfound) (CallFunction|TryFindPlayerScore PlayerID))
  (if _bfound
    (return (.Score (Utilities|Struct|BreakS_PlayerScore _playerscore)))
    (else
      (return -1))))