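; Gameplay Ability for a charged fireball that grows while input is held and launches along the character's aim on release.
; It spawns a replicated projectile on authority, otherwise a non-replicated one, and attaches it to the caster's spawn component.
; A looping timer charges growth cost and scales size, explosion radius and force by curve.
; A hit event triggers radius targeting, damage effects and radial impulse; hit or despawn ends the ability.
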(event Custom|FireballGrowTick
  ;[1 1 1] Growth
  (bind _output_get (Variables|Default|SetCurrentFireballGrowthTime (+ (Variables|Default|GetCurrentFireballGrowthTime) (Variables|Config|GetFireballGrowthRate))))
  (Variables|Default|SetCurrentScalar (Math|Float|Clamp(Float) (/ _output_get (Variables|Config|GetFireballGrowthMaxTime))))
  (Variables|Default|SetCost (Utilities|Struct|MakeScalableFloat (Math|Float|Lerp (Variables|Config|GetMinGrowthCost) (Variables|Config|GetMaxGrowthCost) (Math|Curves|GetFloatValue (Variables|Config|GetFireballGrowthCurve) (Variables|Default|GetCurrentScalar)))))
  (bind _returnvalue (Ability|CommitAbilityCost true))
  (if _returnvalue
    (CallFunction|ApplyScalartoFireball (Variables|Default|GetCurrentScalar))
    (if (>= (Variables|Default|GetCurrentScalar) 1.0)
      (Utilities|Time|ClearandInvalidateTimerbyHandle (Variables|Default|GetFireballGrowTickHandle)))
    (else
      (Utilities|Time|ClearandInvalidateTimerbyHandle (Variables|Default|GetFireballGrowTickHandle)))))

(event Custom|ApplyScalarToFireball
  (params (Scalar :type Float%20%28double-precision%29))
  (bind _fireball (Variables|Default|GetFireball))
  ;[1 1 1] Growth
  (Utilities|IsValid _fireball
    (:Is%20Valid
      (Transformation|SetWorldScale3D (Variables|/Game/CoLab/Blueprints/Arena/GameplayAbilitySystem/Abilities/Fireball/Blueprints/BP_Fireball.BP_Fireball_C|GetScaleComponent _fireball) (Math|Conversions|ToVector(Float) (Math|Float|Lerp (Variables|Config|GetFireballMinScale) (Variables|Config|GetFireballMaxScale) (Math|Curves|GetFloatValue (Variables|Config|GetFireballGrowthCurve) Scalar))))
      (Default|SetExplosionRadius (Variables|Default|GetFireball) (Math|Float|Lerp (Variables|Config|GetFireballMinExplosionRadius) (Variables|Config|GetFireballMaxExplosionRadius) (Math|Curves|GetFloatValue (Variables|Config|GetFireballGrowthCurve) Scalar)))
      (Default|SetExplosionStrength (Variables|Default|GetFireball) (Math|Float|Lerp (Variables|Config|GetFireballMinExplosionForce) (Variables|Config|GetFireballMaxExplosionForce) (Math|Curves|GetFloatValue (Variables|Config|GetFireballGrowthCurve) Scalar))))))

(event Ability|EventActivateAbility
  (Variables|Default|SetCost (Utilities|Struct|MakeScalableFloat (Variables|Config|GetPrimaryManaCost)))
  (bind _returnvalue (Ability|CommitAbilityCost true))
  (if _returnvalue
    (bind _returnvalue_2 (Class|CollabRuntimeConfigSubsystem|GetConfigData (Subsystems|GetCollabRuntimeConfigSubsystem) "/Game/CoLab/Blueprints/Arena/GameplayAbilitySystem/Abilities/Fireball/Config/PDA_FireballConfig.PDA_FireballConfig_C"))
    (Utilities|IsValid _returnvalue_2
      (:Is%20Valid
        (Variables|Default|SetFireballConfig _returnvalue_2)
        (bind _asbp_arena_character (Utilities|Casting|CastToBP_ArenaCharacter (Ability|GetAvatarActorfromActorInfo))
          (:then
            (bind _output_get (Variables|Default|SetCachedCharacter _asbp_arena_character))
            (Ability|GameplayEffect|AddLooseGameplayTags _output_get (GameplayTags|MakeGameplayTagContainerfromTag "(TagName=\"Gameplay.State.Casting\")"))
            (bind _asbpi_projectile_spawner (Utilities|Casting|CastToBPI_ProjectileSpawner _output_get)
              (:then
                (bind _projectilespawncomponent (Default|GetProjectileSpawnComponent _asbpi_projectile_spawner))
                (bind _returnvalue_3 (Game|SpawnActorfromClass (select (Utilities|Enum|Equal(Enum) (Utilities|Struct|BreakGameplayAbilityActivationInfo (Variables|Default|GetCurrentActivationInfo)) "Authority") "/Game/CoLab/Blueprints/Arena/GameplayAbilitySystem/Abilities/Fireball/Blueprints/BP_Fireball_Replicated.BP_Fireball_Replicated_C" "/Game/CoLab/Blueprints/Arena/GameplayAbilitySystem/Abilities/Fireball/Blueprints/BP_Fireball_NonReplicated.BP_Fireball_NonReplicated_C") (Transformation|GetWorldTransform _projectilespawncomponent) "AlwaysSpawn" "MultiplyWithRoot" (Variables|Default|GetCachedCharacter) 0))
                (bind _asbp_fireball (Utilities|Casting|CastToBP_Fireball _returnvalue_3)
                  (:then
                    (bind _output_get_2 (Variables|Default|SetFireball _asbp_fireball))
                    (Default|SetIgnoreActorCollisions (Variables|Default|GetCachedCharacter) _output_get_2 true)
                    (Default|SetIgnoreActorCollisions _output_get_2 (Variables|Default|GetCachedCharacter) true)
                    (Transformation|AttachComponentToComponent _output_get_2 _projectilespawncomponent "None" "KeepWorld" "KeepWorld" "KeepWorld" true)
                    (Variables|Default|SetCachedGravity (Variables|/Script/Engine.ProjectileMovementComponent|GetProjectileGravityScale (Variables|/Game/CoLab/Blueprints/Arena/GameplayAbilitySystem/Abilities/Fireball/Blueprints/BP_Fireball.BP_Fireball_C|GetProjectileMovement (Variables|Default|GetFireball))))
                    (Default|SetGravityScale (Variables|Default|GetFireball) 0.0)
                    (Ability|CommitAbilityCooldown true true)
                    (Utilities|FlowControl|Sequence
                      (:then_0
                        ;[1 1 1] On Hit
                        (bind _payload (Ability|Tasks|WaitGameplayEvent "(TagName=\"Gameplay.Event.Hit.Fireball\")" 0)
                          (:EventReceived
                            (bind _fireball (Variables|Default|GetFireball)
                              (:then
                                (if (== _fireball (.Instigator (Utilities|Struct|BreakGameplayEventData _payload)))
                                  (if (Variables|Default|GetbInputReleased)
                                    _
                                    (else
                                      (Ability|GameplayEffect|RemoveLooseGameplayTags (Variables|Default|GetCachedCharacter) (GameplayTags|MakeGameplayTagContainerfromTag "(TagName=\"Gameplay.State.Casting\")"))))
                                  (bind _data (|WaitTargetData :TaskInstanceName "FireballAOE" :ConfirmationType "Instant" :Class "/Script/GameplayAbilities.GameplayAbilityTargetActor_Radius" :Radius (Default|GetExplosionRadius (Variables|Default|GetFireball)) :StartLocation (Utilities|Struct|MakeGameplayAbilityTargetingLocationInfo "LiteralTransform" (Class|AbilitySystemBlueprintLibrary|GetTargetDataOrigin (.TargetData (Utilities|Struct|BreakGameplayEventData _payload)))) :ReticleClass 0)
                                    (:ValidData
                                      (bind _output_get_3 (Variables|Default|SetHitCharacters (Ability|TargetData|GetAllActorsfromTargetData _data)))
                                      (for _array_element _output_get_3
                                        (if (or (!= _array_element (Variables|Default|GetCachedCharacter)) (Variables|Config|GetbAllowSelfDamage))
                                          (GameplayEffects|ApplyGameplayEffectToTarget (Ability|TargetData|AbilityTargetDatafromActor _array_element) "/Game/CoLab/Blueprints/Arena/GameplayAbilitySystem/Abilities/Fireball/GE_FireballExplosionDamage.GE_FireballExplosionDamage_C" 1 1)))
                                      (Class|RadialForceComponent|FireImpulse (Variables|/Game/CoLab/Blueprints/Arena/GameplayAbilitySystem/Abilities/Fireball/Blueprints/BP_Fireball.BP_Fireball_C|GetRadialForce (Variables|Default|GetFireball)))
                                      (Ability|EndAbility))
                                    (:Cancelled
                                      (Ability|EndAbility)))))
                              (:else
                                (Ability|EndAbility))))))
                      (:then_1
                        ;[1 1 1] Despawn
                        (bind _payload_2 (Ability|Tasks|WaitGameplayEvent "(TagName=\"Gameplay.Event.Despawn.Fireball\")" 0)
                          (:EventReceived
                            (if (or (not (Utilities|IsValid (Variables|Default|GetFireball))) (== (Variables|Default|GetFireball) (.Instigator (Utilities|Struct|BreakGameplayEventData _payload_2))))
                              (Ability|EndAbility)))))
                      (:then_2
                        ;[1 1 1] On Release
                        (Variables|Default|SetbInputReleased false)
                        (Ability|Tasks|WaitInputRelease false
                          (:OnRelease
                            (Variables|Default|SetbInputReleased true)
                            (Ability|GameplayEffect|RemoveLooseGameplayTags (Variables|Default|GetCachedCharacter) (GameplayTags|MakeGameplayTagContainerfromTag "(TagName=\"Gameplay.State.Casting\")"))
                            (Ability|CommitAbilityCooldown true true)
                            (Ability|GameplayEffect|RemoveLooseGameplayTags (Variables|Default|GetCachedCharacter) (GameplayTags|MakeGameplayTagContainerfromTag "(TagName=\"Gameplay.State.Casting\")"))
                            (Utilities|Time|ClearandInvalidateTimerbyHandle (Variables|Default|GetFireballGrowTickHandle))
                            (Transformation|DetachFromActor (Variables|Default|GetFireball) "KeepWorld" "KeepWorld" "KeepWorld")
                            (Actor|SetLifeSpan (Variables|Default|GetFireball) (Variables|Config|GetDespawnTimer))
                            (Default|SetGravityScale (Variables|Default|GetFireball) (Variables|Default|GetCachedGravity))
                            (Variables|/Script/Engine.MovementComponent|SetVelocity (Variables|/Game/CoLab/Blueprints/Arena/GameplayAbilitySystem/Abilities/Fireball/Blueprints/BP_Fireball.BP_Fireball_C|GetProjectileMovement (Variables|Default|GetFireball)) (* (Math|Vector|GetForwardVector (Math|Rotator|MakeRotator (.Roll (Math|Rotator|BreakRotator (Transformation|GetActorRotation (Variables|Default|GetCachedCharacter)))) (Variables|/Game/CoLab/Blueprints/Arena/Characters/BP_ArenaCharacter.BP_ArenaCharacter_C|GetPlayerCameraPitch (Variables|Default|GetCachedCharacter)) (.Yaw (Math|Rotator|BreakRotator (Transformation|GetActorRotation (Variables|Default|GetCachedCharacter)))))) (Math|Conversions|ToVector(Float) (Variables|Config|GetFireballSpeed)))))))
                      (:then_3
                        ;[1 1 1] Growth
                        (CallFunction|ApplyScalartoFireball 0.0)
                        (Variables|Default|SetCurrentFireballGrowthTime 0.0)
                        (bind _returnvalue_4 (Utilities|Time|SetTimerbyEvent (delegate Custom|FireballGrowTick) (Variables|Config|GetFireballGrowthRate) true false (Variables|Config|GetFireballGrowthDelay)))
                        (Variables|Default|SetFireballGrowTickHandle _returnvalue_4))))
                  (:CastFailed
                    (Ability|EndAbility))))
              (:CastFailed
                (Development|PrintString "ERROR: Can't find spawn location")
                (Ability|EndAbility))))
          (:CastFailed
            (Ability|EndAbility))))
      (:Is%20Not%20Valid
        (Ability|EndAbility)))
    (else
      (Ability|EndAbility))))

(event Ability|EventOnEndAbility
  (params (bWasCancelled :type Boolean))
  (|CallParentFunction bWasCancelled)
  (CallFunction|Cleanup))

(fn Cleanup
  (Utilities|Time|ClearandInvalidateTimerbyHandle (Variables|Default|GetFireballGrowTickHandle))
  (if (Utilities|Enum|NotEqual(Enum) (Utilities|Struct|BreakGameplayAbilityActivationInfo (Variables|Default|GetCurrentActivationInfo)) "Confirmed")
    (Actor|DestroyActor (Variables|Default|GetFireball))))