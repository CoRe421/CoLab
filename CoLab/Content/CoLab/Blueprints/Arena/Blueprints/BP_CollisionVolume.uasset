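; Arena trigger box that cancels or damps the velocity of any actor that begins overlapping it.
; A per-axis VelocityResetComponents vector, clamped to 0–1 in the construction script, sets how much velocity is removed on each axis.
; The velocity is scaled through the actor's movement component if it has one, otherwise through its physics-simulating root primitive.
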(event OnComponentBeginOverlap(Box)
  (params (OverlappedComponent :type Primitive%20Component%20Object%20Reference) (OtherActor :type Actor%20Object%20Reference) (OtherComp :type Primitive%20Component%20Object%20Reference) (OtherBodyIndex :type Integer) (bFromSweep :type Boolean) (SweepResult :type Hit%20Result%20Structure%20%28by%20ref%29))
  (CallFunction|ResetActorVelocity OtherActor))

(event EventBeginPlay)

(event Collision|EventActorBeginOverlap
  (params (OtherActor :type Actor%20Object%20Reference)))

(event EventTick
  (params (DeltaSeconds :type Float%20%28single-precision%29)))

(fn ConstructionScript
  (Variables|Default|SetVelocityResetComponents (Math|Vector|MakeVector (Math|Float|Clamp(Float) (.X (Math|Vector|BreakVector (Variables|Default|GetVelocityResetComponents)))) (Math|Float|Clamp(Float) (.Y (Math|Vector|BreakVector (Variables|Default|GetVelocityResetComponents)))) (Math|Float|Clamp(Float) (.Z (Math|Vector|BreakVector (Variables|Default|GetVelocityResetComponents)))))))

(fn ResetActorVelocity
  (params (Actor :type Actor%20Object%20Reference))
  (bind _rootcomponent (Variables|/Script/Engine.Actor|GetRootComponent Actor))
  (bind _output_get (LocalVariables|SetL_MovementComponent (Actor|GetComponentbyClass Actor "/Script/Engine.MovementComponent")))
  (Utilities|IsValid _output_get
    (:Is%20Valid
      (Variables|/Script/Engine.MovementComponent|SetVelocity (LocalVariables|GetL_MovementComponent) (CallFunction|ApplyVelocityReset (Variables|/Script/Engine.MovementComponent|GetVelocity (LocalVariables|GetL_MovementComponent)))))
    (:Is%20Not%20Valid
      (if (Class|SceneComponent|IsAnySimulatingPhysics _rootcomponent)
        (bind _asprimitive_component (Utilities|Casting|CastToPrimitiveComponent _rootcomponent))
        (bind _returnvalue (Physics|GetPhysicsLinearVelocity _asprimitive_component "None"))
        (Class|PrimitiveComponent|SetAllPhysicsLinearVelocity _asprimitive_component (CallFunction|ApplyVelocityReset _returnvalue) false)))))

(fn ApplyVelocityReset
  (params (Velocity :type Vector))
  (bind _returnvalue (Class|KismetMathLibrary|VectorOne))
  (bind _velocityresetcomponents (Variables|Default|GetVelocityResetComponents))
  (bind _returnvalue_2 (- _returnvalue _velocityresetcomponents))
  (bind (_x _y _z) (Math|Vector|BreakVector _returnvalue_2))
  (return (* Velocity (Math|Vector|MakeVector (Math|Float|Absolute(Float) _x) (Math|Float|Absolute(Float) _y) (Math|Float|Absolute(Float) _z)))))