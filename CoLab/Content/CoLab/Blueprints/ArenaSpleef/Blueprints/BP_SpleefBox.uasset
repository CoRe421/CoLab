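; Spleef arena tile that holds a box child actor above a platform child actor and drops it once it is hit.
; Construction stacks and sizes the parts from component bounds, keeping the box static and unreplicated.
; The first hit enables replication and physics and disables the collision box, deferring that cost until needed.
; Hits at high velocity make the box ignore WorldStatic and flag it Fallen, as does its destruction.
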(event Custom|OnBoxHit
  (params (SelfActor :type Actor%20Object%20Reference) (OtherActor :type Actor%20Object%20Reference) (NormalImpulse :type Vector) (Hit :type Hit%20Result%20Structure%20%28by%20ref%29))
  (CallFunction|OnTouched))

(event Custom|OnBoxDestroyed
  (params (DestroyedActor :type Actor%20Object%20Reference))
  (Variables|Default|SetbFallen true))

(event EventBeginPlay
  (bind _boxphysicscomponent (Variables|Default|GetBoxPhysicsComponent)
    (:then
      (Collision|BindEventtoOnActorHit (Components|GetOwner _boxphysicscomponent) (delegate Custom|OnBoxHit))
      (Game|BindEventtoOnDestroyed (Components|GetOwner _boxphysicscomponent) (delegate Custom|OnBoxDestroyed)))
    (:else)))

(event Collision|EventActorBeginOverlap
  (params (OtherActor :type Actor%20Object%20Reference)))

(event EventOnTouched
  (params (TouchedComponents :type Array%20of%20Primitive%20Component%20Object%20References))
  (bind _box (Variables|Default|GetBox))
  (bind _childactor (Variables|/Script/Engine.ChildActorComponent|GetChildActor _box))
  (Utilities|FlowControl|Sequence
    (:then_0
      (Utilities|FlowControl|DoOnce false
        (:Completed
          (Class|ActorComponent|SetIsReplicated _box true)
          (Class|Actor|SetReplicateMovement _childactor true)
          (Networking|SetReplicates _childactor true)
          (Physics|SetSimulatePhysics (Variables|Default|GetBoxPhysicsComponent) true)
          (Collision|SetCollisionEnabled (Variables|Default|GetCollisionBox) "NoCollision"))))
    (:then_1
      (if (> (Math|Vector|VectorLength (Transformation|GetComponentVelocity (Variables|Default|GetBoxPhysicsComponent))) 4e+02)
        (Collision|SetCollisionResponsetoChannel (Variables|Default|GetBoxPhysicsComponent) "ECC_WorldStatic" "ECR_Ignore")
        (Variables|Default|SetbFallen true)))))

(fn ConstructionScript
  (bind _box (Variables|Default|GetBox))
  (bind _platform (Variables|Default|GetPlatform))
  (bind _childactor (Variables|/Script/Engine.ChildActorComponent|GetChildActor _box))
  (bind _childactor_2 (Variables|/Script/Engine.ChildActorComponent|GetChildActor _platform))
  (bind _boxextent (CallFunction|GetComponentSize (Variables|Default|GetPlatform)))
  (LocalVariables|SetL_PlatformSize _boxextent)
  (ChildActorComponent|SetChildActorClass (Variables|Default|GetBox) (Variables|Default|GetBoxClass))
  (bind _boxextent_2 (CallFunction|GetComponentSize (Variables|Default|GetBox)))
  (LocalVariables|SetL_BoxSize _boxextent_2)
  (Transformation|SetRelativeLocation (Variables|Default|GetBox) (Math|Vector|MakeVector 0.0 0.0 (+ (.Z (Math|Vector|BreakVector _boxextent_2)) (.Z (Math|Vector|BreakVector (LocalVariables|GetL_PlatformSize))))) false false)
  (Components|Box|SetBoxExtent (Variables|Default|GetCollisionBox) (LocalVariables|GetL_BoxSize) false)
  (bind _output_get (Variables|Default|SetBoxPhysicsComponent (Actor|GetComponentbyClass (Variables|/Script/Engine.ChildActorComponent|GetChildActor (Variables|Default|GetBox)) "/Script/Engine.PrimitiveComponent")))
  (Collision|SetCollisionResponsetoChannel _output_get "ECC_PhysicsBody" "ECR_Ignore")
  (Rendering|SetCastShadow (Actor|GetComponentbyClass (Variables|/Script/Engine.ChildActorComponent|GetChildActor (Variables|Default|GetPlatform)) "/Script/Engine.PrimitiveComponent") false)
  (Physics|SetSimulatePhysics _output_get false)
  (Class|ActorComponent|SetIsReplicated (Variables|Default|GetBox) false)
  (Components|Tick|SetComponentTickEnabled _box false)
  (Class|Actor|SetReplicateMovement _childactor false)
  (Networking|SetReplicates _childactor false)
  (Variables|/Script/Engine.Actor|SetbNetUseOwnerRelevancy _childactor true)
  (Actor|SetOwner _childactor self)
  (Variables|/Script/Engine.Actor|SetbNetUseOwnerRelevancy _childactor_2 true)
  (Actor|SetOwner _childactor_2 self))

(fn GetComponentSize
  (params (Component :type Scene%20Component%20Object%20Reference))
  (bind _output_get (LocalVariables|SetL_Components (Components|GetChildrenComponents Component true)))
  (Utilities|Array|Add _output_get Component)
  (for _array_element (LocalVariables|GetL_Components)
    (if (not (Math|Vector|VectorIsNearlyZero (.BoxExtent (Collision|GetComponentBounds _array_element))))
      (return (.BoxExtent (Collision|GetComponentBounds _array_element))))))