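; Gameplay ability that launches a fireball from the character along the camera direction, dealing area damage on hit.
; After committing, it spawns a replicated fireball on authority or a non-replicated one otherwise, then waits for hit or despawn gameplay events.
; On hit, the authority runs instant radius targeting at the impact and applies explosion damage to found actors.
; Despawn ends the ability; ending destroys the fireball unless activation mode is Confirmed.
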(event Ability|EventActivateAbility
  (bind _returnvalue (Ability|CommitAbility))
  (if _returnvalue
    (bind _ascharacter (Utilities|Casting|CastToCharacter (Ability|GetAvatarActorfromActorInfo))
      (:then
        (bind _output_get (Variables|Default|SetCachedCharacter _ascharacter))
        (bind _returnvalue_2 (Game|SpawnActorfromClass (select (Utilities|Enum|Equal(Enum) (Utilities|Struct|BreakGameplayAbilityActivationInfo (Variables|Default|GetCurrentActivationInfo)) "Authority") "/Game/CoLab/Blueprints/Gameplay/GameplayAbilitySystem/Abilities/Fireball/Blueprints/BP_Fireball_Replicated.BP_Fireball_Replicated_C" "/Game/CoLab/Blueprints/Gameplay/GameplayAbilitySystem/Abilities/Fireball/Blueprints/BP_Fireball_NonReplicated.BP_Fireball_NonReplicated_C") (Math|Transform|MakeTransform (+ (Transformation|GetActorLocation (Variables|Default|GetCachedCharacter)) (* (Math|Vector|GetForwardVector (Camera|GetCameraRotation (Variables|/Script/Engine.PlayerController|GetPlayerCameraManager (.AsPlayer%20Controller (Utilities|Casting|CastToPlayerController (Pawn|GetController (Variables|Default|GetCachedCharacter))))))) 1e+02)) (Camera|GetCameraRotation (Variables|/Script/Engine.PlayerController|GetPlayerCameraManager (.AsPlayer%20Controller (Utilities|Casting|CastToPlayerController (Pawn|GetController (Variables|Default|GetCachedCharacter))))))) "AlwaysSpawn" "MultiplyWithRoot" _output_get 0))
        (bind _asbp_fireball (Utilities|Casting|CastToBP_Fireball _returnvalue_2))
        (Variables|Default|SetFireball _asbp_fireball)
        (bind _payload (Ability|Tasks|WaitGameplayEvent "(TagName=\"Gameplay.Event.Hit.Fireball\")" 0 true)
          (:then
            (Ability|Tasks|WaitGameplayEvent "(TagName=\"Gameplay.Event.Despawn.Fireball\")" 0 true
              (:EventReceived
                (Ability|EndAbility))))
          (:EventReceived
            (Ability|HasAuthority
              (:True
                (Development|PrintString (Utilities|String|Append "Authority?: " (Utilities|String|ToString(Boolean) (Ability|HasAuthority (Variables|Default|GetCachedCharacter)))))
                (bind _data (|WaitTargetData :TaskInstanceName "FireballAOE" :ConfirmationType "Instant" :Class "/Script/GameplayAbilities.GameplayAbilityTargetActor_Radius" :Radius (Variables|Default|GetFireballExplosionRadius) :StartLocation (Utilities|Struct|MakeGameplayAbilityTargetingLocationInfo "LiteralTransform" (Class|AbilitySystemBlueprintLibrary|GetTargetDataOrigin (.TargetData (Utilities|Struct|BreakGameplayEventData _payload)))) :ReticleClass 0)
                  (:ValidData
                    (bind _output_get_2 (Variables|Default|SetHitCharacters (Ability|TargetData|GetActorsfromTargetData _data)))
                    (for _array_element _output_get_2
                      (GameplayEffects|ApplyGameplayEffectToTarget (Ability|TargetData|AbilityTargetDatafromActor _array_element) "/Game/CoLab/Blueprints/Gameplay/GameplayAbilitySystem/Abilities/Fireball/GE_FireballExplosionDamage.GE_FireballExplosionDamage_C" 1 1))
                    (Ability|EndAbility))
                  (:Cancelled
                    (Ability|EndAbility))))))))
      (:CastFailed
        (Ability|EndAbility)))
    (else
      (Ability|EndAbility))))

(event Ability|EventOnEndAbility
  (params (bWasCancelled :type Boolean))
  (if (Utilities|Enum|NotEqual(Enum) (Utilities|Struct|BreakGameplayAbilityActivationInfo (Variables|Default|GetCurrentActivationInfo)) "Confirmed")
    (Actor|DestroyActor (Variables|Default|GetFireball))))