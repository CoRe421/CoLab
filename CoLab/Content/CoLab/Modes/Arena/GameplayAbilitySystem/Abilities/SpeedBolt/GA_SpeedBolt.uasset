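; Arena gameplay ability for Speed Bolt, a hold-and-release shot that trades the character's speed for damage.
; While held, a looping timer lowers replicated time dilation and updates charge displays, reversing if velocity falls below half its initial value and cancelling at normal speed.
; Release runs an instant line trace, plays a gameplay cue and applies set-by-caller damage scaled by initial speed and dilation lost.
; Ending restores dilation and clears the UI.
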(event Custom|TryFireBolt
  (params (InitialSpeed :type Float%20%28double-precision%29) (SpeedDifferenceRatio :type Float%20%28double-precision%29))
  (bind _returnvalue (Math|Float|Lerp 1.0 0.0 SpeedDifferenceRatio))
  (bind _cachedcharacter (Variables|Default|GetCachedCharacter))
  (bind _cachedspeedpercentdamage (Variables|Default|GetCachedSpeedPercentDamage))
  (bind _returnvalue_2 (* InitialSpeed _cachedspeedpercentdamage))
  (bind _returnvalue_3 (* _returnvalue_2 _returnvalue))
  (bind _data (|WaitTargetData :TaskInstanceName "SpeedBoltTrace" :ConfirmationType "Instant" :Class "/Script/GameplayAbilities.GameplayAbilityTargetActor_SingleLineTrace" :MaxRange 99999.0 :TraceProfile "(Name=\"Projectile\")" :StartLocation (Utilities|Struct|MakeGameplayAbilityTargetingLocationInfo "LiteralTransform" (Transformation|GetWorldTransform (Variables|/Script/CoLab.CoLabCharacter|GetFirstPersonCameraComponent _cachedcharacter)) _cachedcharacter) :ReticleClass "/Script/GameplayAbilities.GameplayAbilityWorldReticle")
    (:ValidData
      (Utilities|FlowControl|Sequence
        (:then_0
          (bind _asbpi_projectile_spawner (Utilities|Casting|CastToBPI_ProjectileSpawner (Variables|Default|GetCachedCharacter))
            (:then
              (bind _projectilespawncomponent (Default|GetProjectileSpawnComponent _asbpi_projectile_spawner))
              (Class|GameplayAbility|ExecuteGameplayCuewithParams "(TagName=\"GameplayCue.Shot.SpeedBolt\")" (Ability|GameplayCue|MakeGameplayCueParameters :RawMagnitude _returnvalue_3 :EffectContext (Ability|GetContextfromOwner (Ability|TargetData|AbilityTargetDatafromHitResult (Ability|TargetData|GetHitResultfromTargetData _data))) :Location (.Location (Math|Transform|BreakTransform (Transformation|GetWorldTransform _projectilespawncomponent)))))
              (bind _output_get (Variables|Default|SetHitActor (Utilities|Array|Get(acopy) (Ability|TargetData|GetActorsfromTargetData _data))))
              (bind _returnvalue_4 (Ability|GameplayEffect|AssignTagSetbyCallerMagnitude (Ability|MakeOutgoingGameplayEffectSpec "/Game/CoLab/Modes/Arena/GameplayAbilitySystem/Abilities/SpeedBolt/GE_SpeedBoltDamage.GE_SpeedBoltDamage_C") "(TagName=\"Gameplay.Effect.Damage\")" (Math|Float|Max(Float) _returnvalue_3 1.0)))
              (GameplayEffects|ApplyGameplayEffectSpecToTarget _returnvalue_4 (Ability|TargetData|AbilityTargetDatafromActor _output_get)))
            (:CastFailed
              (Ability|EndAbility :!label _label))))
        (:then_1
          (goto _label))))
    (:Cancelled
      (goto _label))))

(event Custom|CustomEvent
  (Development|PrintString "Hello"))

(event Custom|OnHoldCancelled
  ;[1 1 1] Fired when speed is returned to normal without firing
  (Ability|GameplayEffect|RemoveLooseGameplayTags (Variables|Default|GetCachedCharacter) (GameplayTags|MakeLiteralGameplayTagContainer "(GameplayTags=((TagName=\"Gameplay.State.Casting\")))"))
  (Ability|CommitAbilityCooldown true true)
  (Ability|HasAuthority
    (:True
      (Ability|EndAbility))))

(event Ability|EventActivateAbility
  (bind _returnvalue (Class|CollabRuntimeConfigSubsystem|GetConfigData (Subsystems|GetCollabRuntimeConfigSubsystem) (Variables|Default|GetConfigClass)))
  (bind _aspda_speed_bolt_config (Utilities|Casting|CastToPDA_SpeedBoltConfig _returnvalue)
    (:then
      (Variables|Default|SetCachedConfigData _aspda_speed_bolt_config)
      (bind _asbp_arena_character (Utilities|Casting|CastToBP_ArenaCharacter (Ability|GetAvatarActorfromActorInfo))
        (:then
          (bind _output_get (Variables|Default|SetCachedCharacter _asbp_arena_character))
          (bind _output_get_2 (Variables|Default|SetCachedMovementComponent (Actor|GetComponentbyClass _output_get "/Script/Collab.CollabMovementComponent")))
          (Utilities|IsValid _output_get_2
            (:Is%20Valid
              (bind _returnvalue_2 (Ability|CommitAbilityCost true))
              (if _returnvalue_2
                (bind _returnvalue_3 (Ability|CommitAbilityCooldown true true))
                (if _returnvalue_3
                  (Variables|Default|SetCachedInitialVelocity (Variables|/Script/Engine.MovementComponent|GetVelocity (Variables|Default|GetCachedMovementComponent)))
                  (Ability|GameplayEffect|AddLooseGameplayTags (Variables|Default|GetCachedCharacter) (GameplayTags|MakeGameplayTagContainerfromTag "(TagName=\"Gameplay.State.Casting\")"))
                  (Variables|Default|SetCachedPrevTimeDilation (Variables|/Game/CoLab/Modes/Arena/Characters/BP_ArenaCharacter.BP_ArenaCharacter_C|GetRep_TimeDilation (Variables|Default|GetCachedCharacter)))
                  (Utilities|FlowControl|Sequence
                    (:then_0
                      ;[1 1 1] On Release
                      (Ability|Tasks|WaitInputRelease false
                        (:OnRelease
                          (Ability|GameplayEffect|RemoveLooseGameplayTags (Variables|Default|GetCachedCharacter) (GameplayTags|MakeLiteralGameplayTagContainer "(GameplayTags=((TagName=\"Gameplay.State.Casting\")))"))
                          (Ability|CommitAbilityCooldown true true)
                          (CallFunction|TryFireBolt (Math|Vector|VectorLength (Variables|Default|GetCachedInitialVelocity)) (/ (Variables|/Game/CoLab/Modes/Arena/Characters/BP_ArenaCharacter.BP_ArenaCharacter_C|GetRep_TimeDilation (Variables|Default|GetCachedCharacter)) (Variables|Default|GetCachedPrevTimeDilation))))))
                    (:then_1
                      (bind _output_get_3 (Variables|Default|SetCachedBoltGrowthRate (Variables|/Game/CoLab/Modes/Arena/GameplayAbilitySystem/Abilities/SpeedBolt/Config/PDA_SpeedBoltConfig.PDA_SpeedBoltConfig_C|GetSpeedBoltGrowthRate (Variables|Default|GetCachedConfigData))))
                      (Variables|Default|SetCachedMinTickReduction (/ _output_get_3 (Variables|/Game/CoLab/Modes/Arena/GameplayAbilitySystem/Abilities/SpeedBolt/Config/PDA_SpeedBoltConfig.PDA_SpeedBoltConfig_C|GetMinHoldTime (Variables|Default|GetCachedConfigData))))
                      (Variables|Default|SetCachedSpeedPercentDamage (Variables|/Game/CoLab/Modes/Arena/GameplayAbilitySystem/Abilities/SpeedBolt/Config/PDA_SpeedBoltConfig.PDA_SpeedBoltConfig_C|GetSpeedPercentDamage (Variables|Default|GetCachedConfigData)))
                      (Variables|Default|SetCachedMinHoldSpeedPercent (Variables|/Game/CoLab/Modes/Arena/GameplayAbilitySystem/Abilities/SpeedBolt/Config/PDA_SpeedBoltConfig.PDA_SpeedBoltConfig_C|GetMinHoldSpeedPercent (Variables|Default|GetCachedConfigData)))
                      (bind _output_get_4 (Variables|Default|SetbCachedScaleHoldTimeWithSpeed (Variables|/Game/CoLab/Modes/Arena/GameplayAbilitySystem/Abilities/SpeedBolt/Config/PDA_SpeedBoltConfig.PDA_SpeedBoltConfig_C|GetbScaleHoldTimeWithSpeed (Variables|Default|GetCachedConfigData))))
                      (if _output_get_4
                        (Variables|Default|SetCachedScaledSpeedTickReduction (/ (Variables|/Game/CoLab/Modes/Arena/GameplayAbilitySystem/Abilities/SpeedBolt/Config/PDA_SpeedBoltConfig.PDA_SpeedBoltConfig_C|GetScaledSpeedTickReduction (Variables|Default|GetCachedConfigData)) (Math|Float|Max(Float) (Math|Vector|VectorLength (Variables|Default|GetCachedInitialVelocity)) 1.0)))
                        (else
                          (Variables|Default|SetCachedStaticTickReduction (/ (Variables|Default|GetCachedBoltGrowthRate) (Variables|/Game/CoLab/Modes/Arena/GameplayAbilitySystem/Abilities/SpeedBolt/Config/PDA_SpeedBoltConfig.PDA_SpeedBoltConfig_C|GetStaticHoldTime (Variables|Default|GetCachedConfigData))))))
                      (Variables|Default|SetCurrentBoltGrowthTime 0.0)
                      (bind _widget (Class|BPIPCCollab|PushWidgettoStack(Message) (Pawn|GetLocalViewingPlayerController (Variables|Default|GetCachedCharacter)) "(TagName=\"UI.Layer.Game\")" "/Game/CoLab/Modes/Arena/GameplayAbilitySystem/Abilities/SpeedBolt/UI/WB_SpeedBoltUI.WB_SpeedBoltUI_C" true))
                      (bind _aswb_speed_bolt_ui (Utilities|Casting|CastToWB_SpeedBoltUI _widget)
                        (:then
                          (bind _output_get_5 (Variables|Default|SetCachedUI _aswb_speed_bolt_ui))
                          (Default|SetChargePercent _output_get_5 0.0))
                        (:CastFailed
                          _))
                      (bind _returnvalue_4 (Utilities|Time|SetTimerbyEvent (EventDispatchers|CreateEvent :!event TickBoltGrowth) (Variables|Default|GetCachedBoltGrowthRate) true))
                      (Variables|Default|SetBoltGrowthTickHandle _returnvalue_4)))
                  (else
                    (Ability|EndAbility)))
                (else
                  (Ability|EndAbility))))
            (:Is%20Not%20Valid
              (Ability|EndAbility))))
        (:CastFailed
          (Ability|EndAbility))))
    (:CastFailed
      (Ability|EndAbility))))

(event Ability|EventOnEndAbility
  (params (bWasCancelled :type Boolean)))

(event EventOnEndAbility
  (params (bWasCancelled :type Boolean))
  (bind _cachedcharacter (Variables|Default|GetCachedCharacter))
  (Default|SetReplicatedTimeDilation (Variables|Default|GetCachedCharacter) (Variables|Default|GetCachedPrevTimeDilation))
  (Utilities|Time|ClearandInvalidateTimerbyHandle (Variables|Default|GetBoltGrowthTickHandle))
  (Class|BPIPCCollab|RemoveWidgetfromStack(Message) (Pawn|GetLocalViewingPlayerController _cachedcharacter) "(TagName=\"UI.Layer.Game\")" (Variables|Default|GetCachedUI) true)
  (bind _asbpi_speed_bolt_charge (Utilities|Casting|CastToBPI_SpeedBoltCharge _cachedcharacter))
  (Default|SetChargePercent _asbpi_speed_bolt_charge 0.0))

(fn TickBoltGrowth
  (bind _cachedui (Variables|Default|GetCachedUI))
  (bind _cachedcharacter (Variables|Default|GetCachedCharacter))
  (bind _rep_timedilation (Variables|/Game/CoLab/Modes/Arena/Characters/BP_ArenaCharacter.BP_ArenaCharacter_C|GetRep_TimeDilation _cachedcharacter))
  (Variables|Default|SetCurrentBoltGrowthTime (+ (Variables|Default|GetCachedBoltGrowthRate) (Variables|Default|GetCurrentBoltGrowthTime)))
  (LocalVariables|SetL_DilationAdjustment (Math|Float|Min(Float) (Math|Float|SelectFloat (Variables|Default|GetCachedScaledSpeedTickReduction) (Variables|Default|GetCachedStaticTickReduction) (Variables|Default|GetbCachedScaleHoldTimeWithSpeed)) (Variables|Default|GetCachedMinTickReduction)))
  (LocalVariables|SetL_NewTimeDilation (Math|Float|Clamp(Float) (Math|Float|SelectFloat (+ _rep_timedilation (LocalVariables|GetL_DilationAdjustment)) (- _rep_timedilation (LocalVariables|GetL_DilationAdjustment)) (< (Math|Vector|VectorLength (Variables|/Script/Engine.MovementComponent|GetVelocity (Variables|/Script/Engine.Character|GetCharacterMovement (Variables|Default|GetCachedCharacter)))) (/ (Math|Vector|VectorLength (Variables|Default|GetCachedInitialVelocity)) 2.0))) (Variables|Default|GetCachedMinHoldSpeedPercent) (Variables|Default|GetCachedPrevTimeDilation)))
  (Utilities|IsValid _cachedui
    (:Is%20Valid
      (Default|SetChargePercent _cachedui (Math|Float|Lerp 1.0 0.0 (/ (- (LocalVariables|GetL_NewTimeDilation) (Variables|Default|GetCachedMinHoldSpeedPercent)) (Variables|Default|GetCachedPrevTimeDilation)))))
    (:Is%20Not%20Valid
      _))
  (bind _asbpi_speed_bolt_charge (Utilities|Casting|CastToBPI_SpeedBoltCharge (Variables|Default|GetCachedCharacter))
    (:then
      (Default|SetChargePercent _asbpi_speed_bolt_charge (Math|Float|Lerp 1.0 0.0 (/ (- (LocalVariables|GetL_NewTimeDilation) (Variables|Default|GetCachedMinHoldSpeedPercent)) (Variables|Default|GetCachedPrevTimeDilation)))))
    (:CastFailed
      _))
  (Default|SetReplicatedTimeDilation (Variables|Default|GetCachedCharacter) (LocalVariables|GetL_NewTimeDilation))
  (if (Math|Float|NearlyEqual(Float) (LocalVariables|GetL_NewTimeDilation) (Variables|Default|GetCachedPrevTimeDilation) 1e-06)
    (CallFunction|OnHoldCancelled)
    (Utilities|Time|ClearandInvalidateTimerbyHandle (Variables|Default|GetBoltGrowthTickHandle))))