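; Arena-mode player volume that teleports each newly entering player to a randomly chosen, tag-matched teleport target.
; On BeginPlay it collects every BP_PlayerTeleportTarget in the level whose TeleportTargetTag matches its own.
; OnNewPlayerEnter, overridden from the parent class, stops the player's character movement, then teleports them to the chosen target's location and rotation.
; If no matching targets were found, entering players are not moved.
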(event EventBeginPlay
  (|CallParentFunction)
  (bind _outactors (Actor|GetAllActorsOfClass "/Game/CoLab/Modes/Arena/Blueprints/TeleportVolume/BP_PlayerTeleportTarget.BP_PlayerTeleportTarget_C"))
  (for _array_element _outactors
    (if (== (Variables|Default|GetTeleport%20Target%20Tag) (Variables|/Game/CoLab/Modes/Arena/Blueprints/TeleportVolume/BP_PlayerTeleportTarget.BP_PlayerTeleportTarget_C|GetTeleportTargetTag _array_element))
      (Utilities|Array|Add (Variables|Default|GetFoundTeleportTargets) _array_element))))

(event Collision|EventActorBeginOverlap
  (params (OtherActor :type Actor%20Object%20Reference))
  (|CallParentFunction OtherActor) ; This node is disabled and will not be called.\nDrag off pins to build functionality.
)

(event EventTick
  (params (DeltaSeconds :type Float%20%28single-precision%29))
  (|CallParentFunction DeltaSeconds) ; This node is disabled and will not be called.\nDrag off pins to build functionality.
)

(fn ConstructionScript
  (|CallParentFunction))

(fn OnNewPlayerEnter
  (params (Player :type Collab%20Player%20Character%20Object%20Reference))
  (|CallParentFunction Player)
  (if (Utilities|Array|IsNotEmpty (Variables|Default|GetFoundTeleportTargets))
    (bind _output_get (LocalVariables|SetL_ChosenTarget (.OutItem (Utilities|Array|Random (Variables|Default|GetFoundTeleportTargets)))))
    (Components|Movement|StopMovementImmediately (Variables|/Script/Engine.Character|GetCharacterMovement Player))
    (Transformation|Teleport Player (.Location (Math|Transform|BreakTransform (Transformation|GetActorTransform _output_get))) (.Rotation (Math|Transform|BreakTransform (Transformation|GetActorTransform _output_get))))))