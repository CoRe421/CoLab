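; BP_PointsVolume is an Arena-mode volume that awards score when a new player enters it.
; On BeginPlay it caches the Arena game state and the Arena config data asset from the Collab runtime config subsystem.
; The OnNewPlayerEnter override adds the configured zone score to that player's net ID through the game state, then fires an OnPlayerScore event.
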(event EventBeginPlay
  (|CallParentFunction)
  (Utilities|FlowControl|Sequence
    (:then_0
      (bind _asbp_gs_arena (Utilities|Casting|CastToBP_GS_Arena (Game|GetGameState))
        (:then
          (Variables|Default|SetCachedGameState _asbp_gs_arena))
        (:CastFailed
          _))
      (bind _returnvalue (Class|CollabRuntimeConfigSubsystem|GetConfigData (Subsystems|GetCollabRuntimeConfigSubsystem) "/Game/CoLab/Modes/Arena/GameFramework/Config/PDA_ArenaConfig.PDA_ArenaConfig_C"))
      (Variables|Default|SetCachedArenaConfig _returnvalue))))

(event Collision|EventActorBeginOverlap
  (params (OtherActor :type Actor%20Object%20Reference)))

(event EventTick
  (params (DeltaSeconds :type Float%20%28single-precision%29)))

(fn ConstructionScript
  (|CallParentFunction))

(fn OnNewPlayerEnter
  (params (Player :type Collab%20Player%20Character%20Object%20Reference))
  (bind _playerstate (Variables|/Script/Engine.Pawn|GetPlayerState Player))
  (bind _cachedgamestate (Variables|Default|GetCachedGameState))
  (bind _cachedarenaconfig (Variables|Default|GetCachedArenaConfig))
  (|CallParentFunction Player)
  (if (Math|Boolean|ANDBoolean (Utilities|IsValid _cachedgamestate) (Utilities|IsValid _playerstate) (Utilities|IsValid _cachedarenaconfig))
    (Default|AddPlayerScore _cachedgamestate (PlayerState|GetUniqueID _playerstate) (Variables|/Game/CoLab/Modes/Arena/GameFramework/Config/PDA_ArenaConfig.PDA_ArenaConfig_C|GetPlayerZoneScoreValue _cachedarenaconfig))
    (Default|CallOnPlayerScore self)))